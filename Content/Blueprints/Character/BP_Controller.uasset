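; Controller Blueprint that switches the level between past and future on the T key via a dissolve effect.
; BeginPlay sorts StaticMeshActors into past and future arrays by their slot 0 dissolve material.
; Tick steps the shared material parameter collection's Dissolve value by a fixed per-frame amount toward the other era.
; When the fade completes, it flips the era flag and swaps collision between the two arrays.
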(event EventTick
  (params (DeltaSeconds :type Float%20%28single-precision%29))
  (if (Variables|Default|GettimeWalk)
    (if (Variables|DissolveVariables|GetCurrentTime)
      (if (> (Variables|DissolveVariables|GetDissolve) 0.0)
        (bind _output_get (Variables|DissolveVariables|SetDissolve (- (Variables|DissolveVariables|GetDissolve) 0.01)))
        (Rendering|Material|SetScalarParameterValue "/Game/Art/Meshes/M_Dissolve_Parameter.M_Dissolve_Parameter" "Dissolve" _output_get :!class /Script/Engine.KismetMaterialLibrary)
        (else
          (Variables|Default|SettimeWalk false)
          (Variables|DissolveVariables|SetCurrentTime false)
          (for _array_element (Variables|DissolveVariables|GetPastActor)
            (Collision|SetCollisionEnabled (Variables|/Script/Engine.StaticMeshActor|GetStaticMeshComponent _array_element) "QueryAndPhysics"))
          (for _array_element_2 (Variables|DissolveVariables|GetFutureActor)
            (Collision|SetCollisionEnabled (Variables|/Script/Engine.StaticMeshActor|GetStaticMeshComponent _array_element_2) "NoCollision"))))
      (elif (< (Variables|DissolveVariables|GetDissolve) 1.0)
        (bind _output_get_2 (Variables|DissolveVariables|SetDissolve (+ (Variables|DissolveVariables|GetDissolve) 0.01)))
        (Rendering|Material|SetScalarParameterValue "/Game/Art/Meshes/M_Dissolve_Parameter.M_Dissolve_Parameter" "Dissolve" _output_get_2 :!class /Script/Engine.KismetMaterialLibrary)
        (else
          (Variables|Default|SettimeWalk false)
          (Variables|DissolveVariables|SetCurrentTime true)
          (for _array_element_3 (Variables|DissolveVariables|GetPastActor)
            (Collision|SetCollisionEnabled (Variables|/Script/Engine.StaticMeshActor|GetStaticMeshComponent _array_element_3) "NoCollision"))
          (for _array_element_4 (Variables|DissolveVariables|GetFutureActor)
            (Collision|SetCollisionEnabled (Variables|/Script/Engine.StaticMeshActor|GetStaticMeshComponent _array_element_4) "QueryAndPhysics")))))))

(event EventBeginPlay
  (bind _outactors (Actor|GetAllActorsOfClass "/Script/Engine.StaticMeshActor"))
  (for _array_element _outactors
    (Math|Integer|IncrementInt (Variables|DissolveVariables|GetCounted)
      (:%20%20
        (if (== (Rendering|Material|GetMaterial (Variables|/Script/Engine.StaticMeshActor|GetStaticMeshComponent _array_element) 0) "/Game/Art/Meshes/M_Dissolve_Future.M_Dissolve_Future")
          (Utilities|Array|Add (Variables|DissolveVariables|GetFutureActor) _array_element)
          (elif (== (Rendering|Material|GetMaterial (Variables|/Script/Engine.StaticMeshActor|GetStaticMeshComponent _array_element) 0) "/Game/Art/Meshes/M_Dissolve_Past.M_Dissolve_Past")
            (Utilities|Array|Add (Variables|DissolveVariables|GetPastActor) _array_element))))))
  (Development|PrintString (Utilities|String|Append "Checked " (Utilities|String|ToString(Integer) (Variables|DissolveVariables|GetCounted)) " Objects")))

(event Input|KeyboardEvents|T
  (params (Key :type Key%20Structure :default "AnyKey"))
  (:Pressed
    (if (not (Variables|DissolveVariables|GetTimeWalk))
      (Variables|DissolveVariables|SetTimeWalk true))))

(fn ConstructionScript)
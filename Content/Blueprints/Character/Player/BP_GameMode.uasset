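; Game mode Blueprint that controls audio volume for Master, Ambient and SFX sound classes.
; Each Set function stores a volume, then calls its Load function to apply it through SetSoundClassVolume.
; Ambient and SFX inputs are scaled by master volume on storage.
; Changing master multiplies those already-scaled values again, so repeated master changes compound, then reapplies all three classes.
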(event EventBeginPlay)

(event EventTick
  (params (DeltaSeconds :type Float%20%28single-precision%29)))

(fn ConstructionScript)

(fn SetMasterVolume
  (params (Volume :type Float%20%28single-precision%29))
  (Variables|Default|Setm_MasterVolume Volume)
  (Variables|Default|Setm_AmbientVolume (* (Variables|Default|Getm_MasterVolume) (Variables|Default|Getm_AmbientVolume)))
  (Variables|Default|Setm_SFXVolume (* (Variables|Default|Getm_MasterVolume) (Variables|Default|Getm_SFXVolume)))
  (CallFunction|LoadMasterVolume))

(fn SetAmbientVolume
  (params (Volume :type Float%20%28single-precision%29))
  (Variables|Default|Setm_AmbientVolume (* (Variables|Default|Getm_MasterVolume) Volume))
  (CallFunction|LoadAmbientVolume))

(fn SetSFXVolume
  (params (Volume :type Float%20%28single-precision%29))
  (Variables|Default|Setm_SFXVolume (* (Variables|Default|Getm_MasterVolume) Volume))
  (CallFunction|LoadSFXVolume))

(fn LoadMasterVolume
  (Class|MGameMode|SetSoundClassVolume "/Game/Blueprints/Options/MasterSoundClass.MasterSoundClass" (Variables|Default|Getm_MasterVolume))
  (Class|MGameMode|SetSoundClassVolume "/Game/Blueprints/Options/MasterSoundClass.SFX_Sounds" (Variables|Default|Getm_SFXVolume))
  (Class|MGameMode|SetSoundClassVolume "/Game/Blueprints/Options/MasterSoundClass.Ambient_Sounds" (Variables|Default|Getm_AmbientVolume)))

(fn LoadAmbientVolume
  (Class|MGameMode|SetSoundClassVolume "/Game/Blueprints/Options/MasterSoundClass.Ambient_Sounds" (Variables|Default|Getm_AmbientVolume)))

(fn LoadSFXVolume
  (Class|MGameMode|SetSoundClassVolume "/Game/Blueprints/Options/MasterSoundClass.SFX_Sounds" (Variables|Default|Getm_SFXVolume)))
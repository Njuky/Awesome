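; Player controller that runs the time-walk mechanic, switching the level between past and future when T is pressed.
; BeginPlay sorts static meshes into past and future sets by dissolve material or component tag, and collects BP_BaseObject actors.
; Tick steps a dissolve value in a material parameter collection, then swaps collision on both sets and calls ChangeTexture on the objects.
; Returning to the past also spawns an AI_Follower near each BP_Character, gated by a DoOnce.
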(event EventTick
  (params (DeltaSeconds :type Float%20%28single-precision%29))
  (if (Variables|Default|GettimeWalk)
    (if (Variables|DissolveVariables|GetCurrentTime)
      (if (> (Variables|DissolveVariables|GetDissolve) 0.0)
        (bind _output_get (Variables|DissolveVariables|SetDissolve (- (Variables|DissolveVariables|GetDissolve) 0.01)))
        (Rendering|Material|SetScalarParameterValue "/Game/Art/Meshes/M_Dissolve_Parameter.M_Dissolve_Parameter" "Dissolve" _output_get :!class /Script/Engine.KismetMaterialLibrary)
        (Utilities|FlowControl|DoOnce false :!label _label
          (:Completed
            (bind _outactors (Actor|GetAllActorsOfClass "/Game/Blueprints/Character/Player/BP_Character.BP_Character_C"))
            (for _array_element _outactors
              (bind _returnvalue (Game|SpawnActorfromClass "/Game/Blueprints/Character/NPC/AI_Follower.AI_Follower_C" (Math|Transform|MakeTransform (+ (Transformation|GetActorLocation _array_element) (Math|Vector|MakeVector -2.5e+02 -2.5e+02 0.0)) "0, 0, 0" "1,1,1.000000") "AlwaysSpawn" 0 0))
              (Variables|/Script/Engine.Pawn|SetAIControllerClass _returnvalue "/Script/AIModule.AIController"))))
        (else
          (Variables|Default|SettimeWalk false)
          (Variables|DissolveVariables|SetCurrentTime false)
          (for _array_element_2 (Variables|DissolveVariables|GetPastDissolveObject)
            (Collision|SetCollisionEnabled (Variables|/Script/Engine.StaticMeshActor|GetStaticMeshComponent _array_element_2) "QueryAndPhysics")
            (goto _label Reset))
          (for _array_element_3 (Variables|DissolveVariables|GetFutureDissolveObject)
            (Collision|SetCollisionEnabled (Variables|/Script/Engine.StaticMeshActor|GetStaticMeshComponent _array_element_3) "NoCollision")
            (for _array_element_4 (Variables|DissolveVariables|GetTextureChangeActor)
              (Default|ChangeTexture _array_element_4 false)))))
      (elif (< (Variables|DissolveVariables|GetDissolve) 1.0)
        (bind _output_get_2 (Variables|DissolveVariables|SetDissolve (+ (Variables|DissolveVariables|GetDissolve) 0.01)))
        (Rendering|Material|SetScalarParameterValue "/Game/Art/Meshes/M_Dissolve_Parameter.M_Dissolve_Parameter" "Dissolve" _output_get_2 :!class /Script/Engine.KismetMaterialLibrary)
        (else
          (Variables|Default|SettimeWalk false)
          (Variables|DissolveVariables|SetCurrentTime true)
          (for _array_element_5 (Variables|DissolveVariables|GetPastDissolveObject)
            (Collision|SetCollisionEnabled (Variables|/Script/Engine.StaticMeshActor|GetStaticMeshComponent _array_element_5) "NoCollision"))
          (for _array_element_6 (Variables|DissolveVariables|GetFutureDissolveObject)
            (Collision|SetCollisionEnabled (Variables|/Script/Engine.StaticMeshActor|GetStaticMeshComponent _array_element_6) "QueryAndPhysics")
            (for _array_element_7 (Variables|DissolveVariables|GetTextureChangeActor)
              (Default|ChangeTexture _array_element_7 true))))))))

(event EventBeginPlay
  (Utilities|FlowControl|Sequence
    (:then_0
      (bind _outactors (Actor|GetAllActorsOfClass "/Script/Engine.StaticMeshActor"))
      (for _array_element _outactors
        (if (or (== (Rendering|Material|GetMaterial (Variables|/Script/Engine.StaticMeshActor|GetStaticMeshComponent _array_element) 0) "/Game/Art/Meshes/M_Dissolve_Future.M_Dissolve_Future") (Components|ComponentHasTag (Variables|/Script/Engine.StaticMeshActor|GetStaticMeshComponent _array_element) "Future"))
          (Utilities|Array|Add (Variables|DissolveVariables|GetFutureDissolveObject) _array_element)
          (elif (or (== (Rendering|Material|GetMaterial (Variables|/Script/Engine.StaticMeshActor|GetStaticMeshComponent _array_element) 0) "/Game/Art/Meshes/M_Dissolve_Past.M_Dissolve_Past") (Components|ComponentHasTag (Variables|/Script/Engine.StaticMeshActor|GetStaticMeshComponent _array_element) "Past"))
            (Utilities|Array|Add (Variables|DissolveVariables|GetPastDissolveObject) _array_element)))))
    (:then_1
      (bind _outactors_2 (Actor|GetAllActorsOfClass "/Game/Blueprints/Objects/BP_BaseObject.BP_BaseObject_C"))
      (for _array_element_2 _outactors_2
        (Utilities|Array|Add (Variables|DissolveVariables|GetTextureChangeActor) _array_element_2)))))

(event Input|KeyboardEvents|T
  (params (Key :type Key%20Structure :default "AnyKey"))
  (:Pressed
    (if (not (Variables|DissolveVariables|GetTimeWalk))
      (Variables|DissolveVariables|SetTimeWalk true))))

(fn ConstructionScript)
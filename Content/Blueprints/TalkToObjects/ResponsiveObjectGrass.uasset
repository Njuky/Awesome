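; Talk-to-object actor for grass that shows a text box when the player interacts with it nearby.
; Overlapping the Box enables input and talking only if the controller's CurrentTime is true, and leaving it disables both.
; While talking is allowed, entering the Sphere shows a B-button prompt, which pressing gamepad B or F swaps for the grass textbox widget.
; Gamepad X or leaving the Sphere removes all widgets.
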(event OnComponentEndOverlap(Box)
  (params (OtherActor :type Actor%20Object%20Reference) (OtherComp :type Primitive%20Component%20Object%20Reference) (OtherBodyIndex :type Integer))
  ;[0.9082 1 0.06893] Enable/Disable Input wenn in CollisonBox
  (Input|DisableInput (Game|GetPlayerController 0))
  (Variables|Default|SetCanTalk false))

(event OnComponentBeginOverlap(Sphere)
  (params (OtherActor :type Actor%20Object%20Reference) (OtherComp :type Primitive%20Component%20Object%20Reference) (OtherBodyIndex :type Integer) (bFromSweep :type Boolean) (SweepResult :type Hit%20Result%20Structure%20%28by%20ref%29))
  ;[0.3254 0.2845 1] B to interact Widget
  (if (Variables|Default|GetCanTalk)
    (bind _returnvalue (UserInterface|CreateWidget "/Game/Blueprints/TalkToObjects/BButtonWidget.BButtonWidget_C"))
    (UserInterface|Viewport|AddtoViewport _returnvalue 0)))

(event OnComponentEndOverlap(Sphere)
  (params (OtherActor :type Actor%20Object%20Reference) (OtherComp :type Primitive%20Component%20Object%20Reference) (OtherBodyIndex :type Integer))
  ;[0.9367 0.342 1] Remove Widget when out of sphere
  (Viewport|RemoveAllWidgets))

(event OnComponentBeginOverlap(Box)
  (params (OtherActor :type Actor%20Object%20Reference) (OtherComp :type Primitive%20Component%20Object%20Reference) (OtherBodyIndex :type Integer) (bFromSweep :type Boolean) (SweepResult :type Hit%20Result%20Structure%20%28by%20ref%29))
  (bind _returnvalue (Game|GetPlayerController 0))
  ;[0.9082 1 0.06893] Enable/Disable Input wenn in CollisonBox
  (bind _asbp_controller (Utilities|Casting|CastToBP_Controller _returnvalue))
  (if (Variables|/Game/Blueprints/Character/Player/BP_Controller.BP_Controller_C|GetCurrentTime _asbp_controller)
    (Variables|Default|SetCanTalk true)
    (Input|EnableInput _returnvalue)))

(event Input|KeyboardEvents|F
  (params (Key :type Key%20Structure :default "AnyKey"))
  (:Pressed
    ;[1 0.1381 0.1095] TextboxWidget
    (if (Variables|Default|GetCanTalk)
      (bind _returnvalue (UserInterface|CreateWidget "/Game/Blueprints/TalkToObjects/ResponsiveObjectWidgetGrass.ResponsiveObjectWidgetGrass_C"))
      (bind _output_get (Variables|Default|SetResponsiveObjectWidget _returnvalue))
      (if (not (UserInterface|Viewport|IsinViewport _output_get))
        (UserInterface|Viewport|AddtoViewport _returnvalue 0)
        (Widget|RemovefromParent (stale OnComponentBeginOverlap(Sphere) _returnvalue))))))

(event Input|GamepadEvents|GamepadFaceButtonRight
  (params (Key :type Key%20Structure :default "AnyKey"))
  (:Pressed
    ;[1 0.1381 0.1095] TextboxWidget
    (if (Variables|Default|GetCanTalk)
      (bind _returnvalue (UserInterface|CreateWidget "/Game/Blueprints/TalkToObjects/ResponsiveObjectWidgetGrass.ResponsiveObjectWidgetGrass_C"))
      (bind _output_get (Variables|Default|SetResponsiveObjectWidget _returnvalue))
      (if (not (UserInterface|Viewport|IsinViewport _output_get))
        (UserInterface|Viewport|AddtoViewport _returnvalue 0)
        (Widget|RemovefromParent (stale OnComponentBeginOverlap(Sphere) _returnvalue))))))

(event Input|GamepadEvents|GamepadFaceButtonLeft
  (params (Key :type Key%20Structure :default "AnyKey"))
  ;[0.388 1 0.3735] Close Textbox with X
  (:Pressed
    (Viewport|RemoveAllWidgets)))

(fn ConstructionScript)
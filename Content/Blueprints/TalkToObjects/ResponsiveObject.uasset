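; Interactable world object that shows a text box when the player talks to it.
; Box overlap enables and disables the player's input on the actor, while Sphere overlap shows a B-button prompt widget.
; Pressing B swaps the prompt for the responsive-object textbox widget.
; Pressing X or leaving the sphere removes all widgets from the viewport.
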(event OnComponentEndOverlap(Box)
  (params (OtherActor :type Actor%20Object%20Reference) (OtherComp :type Primitive%20Component%20Object%20Reference) (OtherBodyIndex :type Integer))
  ;[0.9082 1 0.06893] Enable/Disable Input wenn in CollisonBox
  (Input|DisableInput (Game|GetPlayerController 0)))

(event OnComponentBeginOverlap(Sphere)
  (params (OtherActor :type Actor%20Object%20Reference) (OtherComp :type Primitive%20Component%20Object%20Reference) (OtherBodyIndex :type Integer) (bFromSweep :type Boolean) (SweepResult :type Hit%20Result%20Structure%20%28by%20ref%29))
  ;[0.3254 0.2845 1] B to interact Widget
  (bind _returnvalue (UserInterface|CreateWidget "/Game/Blueprints/TalkToObjects/BButtonWidget.BButtonWidget_C"))
  (UserInterface|Viewport|AddtoViewport _returnvalue 0))

(event OnComponentEndOverlap(Sphere)
  (params (OtherActor :type Actor%20Object%20Reference) (OtherComp :type Primitive%20Component%20Object%20Reference) (OtherBodyIndex :type Integer))
  ;[0.9367 0.342 1] Remove Widget when out of sphere
  (Viewport|RemoveAllWidgets))

(event OnComponentBeginOverlap(Box)
  (params (OtherActor :type Actor%20Object%20Reference) (OtherComp :type Primitive%20Component%20Object%20Reference) (OtherBodyIndex :type Integer) (bFromSweep :type Boolean) (SweepResult :type Hit%20Result%20Structure%20%28by%20ref%29))
  ;[0.9082 1 0.06893] Enable/Disable Input wenn in CollisonBox
  (Input|EnableInput (Game|GetPlayerController 0)))

(event Input|KeyboardEvents|B
  (params (Key :type Key%20Structure :default "AnyKey"))
  ;[1 0.1381 0.1095] TextboxWidget
  (:Pressed
    (bind _returnvalue (UserInterface|CreateWidget "/Game/Blueprints/TalkToObjects/ResponsiveObjectWidget.ResponsiveObjectWidget_C"))
    (UserInterface|Viewport|AddtoViewport _returnvalue 0)
    (Widget|RemovefromParent (stale OnComponentBeginOverlap(Sphere) _returnvalue))))

(event Input|KeyboardEvents|X
  (params (Key :type Key%20Structure :default "AnyKey"))
  ;[0.388 1 0.3735] Close Textbox with X
  (:Pressed
    (Viewport|RemoveAllWidgets)))

(fn ConstructionScript)
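; BP_AIPath is a trigger-driven path actor that hands itself to AI when a BP_Character enters its box.
; The first such overlap marks it used, calls SetNewPath on every BP_AI in the level and sets AI Enabled.
; PathLogic is a stub returning defaults, and IncreaseStep advances CurrentStep when a point is reached, suggesting child paths supply the movement logic.
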(event OnComponentBeginOverlap(Box)
  (params (OverlappedComponent :type Primitive%20Component%20Object%20Reference) (OtherActor :type Actor%20Object%20Reference) (OtherComp :type Primitive%20Component%20Object%20Reference) (OtherBodyIndex :type Integer) (bFromSweep :type Boolean) (SweepResult :type Hit%20Result%20Structure%20%28by%20ref%29))
  (if (not (Variables|Default|Getused))
    (Utilities|Casting|CastToBP_Character OtherActor)
    (Variables|Default|Setused true)
    (bind _outactors (Actor|GetAllActorsOfClass "/Game/Blueprints/AI/BP_AI.BP_AI_C"))
    (for _array_element _outactors
      (Default|SetNewPath _array_element self)
      (Variables|/Game/Blueprints/AI/BP_AI.BP_AI_C|Setenabled (Variables|Default|GetAI) true))))

(fn ConstructionScript)

(fn PathLogic
  (return false 0))

(fn IncreaseStep
  (params (ReachedPoint :type Boolean))
  (if ReachedPoint
    (Math|Integer|IncrementInt (Variables|Default|GetCurrentStep))))
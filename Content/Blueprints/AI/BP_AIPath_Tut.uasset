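; Tutorial AI path that tracks the player through a ball-and-bowl puzzle with a time switch.
; PathLogic switches on CurrentStep, checking bowl slots, solved flags, and the player controller's inventory and time state.
; It returns whether the step's goal is met plus a point to move to, advancing through IncreaseStep except on the final step.
; The time-switch step unlocks timewalk on BP_Controller once.
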(fn ConstructionScript
  (|CallParentFunction))

(fn PathLogic
  (switch int (Variables|Default|GetCurrentStep)
    (:0
      ;[1 1 1] Take red Ball of green Bowl
      (Variables|Default|SetoutputBool (== (Variables|/Script/Project2016.C_Bowl|Getc_slot (Variables|Default|GetBowlGreen)) 0))
      (Variables|Default|SetoutputInt 2)
      (CallFunction|IncreaseStep (Variables|Default|GetoutputBool) :!label _label)
      (return (Variables|Default|GetoutputBool) (Variables|Default|GetoutputInt)))
    (:1
      ;[1 1 1] Place red ball in red bowl
      (Variables|Default|SetoutputBool (Variables|/Script/Project2016.C_Bowl|Getc_solved (Variables|Default|GetBowlRed)))
      (Variables|Default|SetoutputInt 6)
      (goto _label))
    (:2
      ;[1 1 1] Switch time
      (Utilities|FlowControl|Sequence
        (:then_0
          (Utilities|FlowControl|DoOnce false
            (:Completed
              (bind _asbp_controller (Utilities|Casting|CastToBP_Controller (Game|GetPlayerController 0)))
              (Variables|/Script/Project2016.C_PlayerController|SetcanTimewalk _asbp_controller true))))
        (:then_1
          (bind _asbp_controller_2 (Utilities|Casting|CastToBP_Controller (Game|GetPlayerController 0))
            (:then
              (Variables|Default|SetoutputBool (not (Variables|/Script/Project2016.C_PlayerController|GetcurrentTime _asbp_controller_2)))
              (goto _label))
            (:CastFailed
              (goto _label))))))
    (:3
      ;[1 1 1] Take green ball
      (bind _asbp_controller_3 (Utilities|Casting|CastToBP_Controller (Game|GetPlayerController 0))
        (:then
          (CallFunction|IncreaseStep (== (Variables|/Script/Project2016.C_PlayerController|Getc_Inventory _asbp_controller_3) (Variables|Default|GetGreenBall)))
          (Variables|Default|SetoutputBool (== (Variables|/Script/Project2016.C_PlayerController|Getc_Inventory _asbp_controller_3) (Variables|Default|GetGreenBall)))
          (Variables|Default|SetoutputInt 11)
          (return (Variables|Default|GetoutputBool) (Variables|Default|GetoutputInt)))
        (:CastFailed
          (goto _label))))
    (:4
      ;[1 1 1] Place green ball in green bowl
      (Variables|Default|SetoutputBool (Variables|/Script/Project2016.C_Bowl|Getc_solved (Variables|Default|GetBowlGreen)))
      (Variables|Default|SetoutputInt 99)
      (return (Variables|Default|GetoutputBool) (Variables|Default|GetoutputInt)))))
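; AI path script for the third puzzle, deciding how a companion AI animates and where it moves as the player progresses.
; PathLogic switches on CurrentStep: it first waits for the player to come near, then waves by the bowl until the controller's inventory holds a Berry.
; Each step returns a reached flag and target point index, passing the flag to IncreaseStep.
; A separate MyDelay event sets Execute after a delay.
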(event Custom|MyDelay
  (params (Time :type Float%20%28single-precision%29))
  (Utilities|FlowControl|Delay Time)
  (Variables|Default|SetExecute true))

(fn ConstructionScript
  (|CallParentFunction))

(fn PathLogic
  (bind _returnvalue (Game|GetPlayerCharacter 0))
  (bind _ai (Variables|Default|GetAI))
  (bind _returnvalue_2 (Transformation|GetDistanceTo _ai _returnvalue))
  (bind _returnvalue_3 (<= _returnvalue_2 8e+02))
  (switch int (Variables|Default|GetCurrentStep)
    (:0
      ;[1 1 1] Wait for player to be close
      (if _returnvalue_3
        _
        (else
          (Variables|/Game/Blueprints/AI/BP_AI.BP_AI_C|SetAnimationEnum (Variables|Default|GetAI) "NewEnumerator3")))
      (Variables|Default|SetoutputBool _returnvalue_3)
      (Variables|Default|SetoutputInt 5))
    (:1
      ;[1 1 1] Wave between bowl
      (bind _asbp_controller (Utilities|Casting|CastToBP_Controller (Game|GetPlayerController 0)))
      (if (== (Variables|/Script/Project2016.C_PlayerController|Getc_Inventory _asbp_controller) (Variables|Default|GetBerry))
        (Variables|Default|SetoutputInt 99)
        (else
          (Variables|/Game/Blueprints/AI/BP_AI.BP_AI_C|SetAnimationEnum (Variables|Default|GetAI) "NewEnumerator2")
          (Variables|Default|SetoutputInt 0)))
      (Variables|Default|SetoutputBool (== (Variables|/Script/Project2016.C_PlayerController|Getc_Inventory _asbp_controller) (Variables|Default|GetBerry)))))
  (CallFunction|IncreaseStep (Variables|Default|GetoutputBool))
  (return (Variables|Default|GetoutputBool) (Variables|Default|GetoutputInt)))
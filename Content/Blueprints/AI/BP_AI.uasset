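; AI companion that follows the player when it has no path and travels assigned spline paths between task points.
; SetNewPath navigates it to the spline start, then Tick steps it along the spline by a fixed per-frame distance.
; At each point it faces the player and waits until the path's PathLogic supplies the next point; index 99 releases the path.
; MoveToPlayer's far-distance teleport is unreachable behind the follow check.
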(event Custom|Wave
  ;[1 1 1] AI Waiting for Task
  (Utilities|FlowControl|Sequence
    (:then_0
      (Utilities|FlowControl|Delay (Math|Random|RandomFloatinRange 8.0 15.0))
      (Variables|Default|SetAnimationEnum "NewEnumerator2"))
    (:then_1
      ;[1 1 1] Face player character
      (Transformation|SetActorRotation (Math|Conversions|RotationFromXVector (Math|Vector|RotateVector (Math|Vector|Normalize (* (- (Transformation|GetActorLocation (Game|Player|GetPlayerPawn 0)) (Transformation|GetActorLocation)) "1.000000,1.000000, 0")) "0, 0, 0"))))))

(event EventBeginPlay
  (Variables|Default|SetMaxWalkSpeed (Class|MovementComponent|GetMaxSpeed (Variables|Character|GetCharacterMovement))))

(event EventTick
  (params (DeltaSeconds :type Float%20%28single-precision%29))
  (if (Variables|Default|Getenabled)
    (if (Variables|Default|GetNewPath)
      ;[1 1 1] Move to new Spline
      (CallFunction|CheckReachedNewPath)
      (elif (== (Variables|Default|GetPath) 0)
        (CallFunction|MovetoPlayer)
        (Rendering|SetVisibility (Variables|Default|GetParticleSystem) false false)
        (elif (Variables|Default|GetInAction)
          ;[1 1 1] Task in action
          (if (!= (Variables|Default|GetPointToMove) 99)
            (CallFunction|SetParticleSystem)
            (bind _reached (CallFunction|MoveAIAlongSpline (Variables|Default|GetPointToMove)))
            (Variables|Default|SetInAction (not _reached))
            (Rendering|SetVisibility (Variables|Default|GetMoveParticle) (not _reached) false)
            (else
              (Variables|Default|SetInAction false)
              (Variables|Default|SetPath 0)))
          (else
            ;[1 1 1] Waiting for task
            (CallFunction|Wave)
            (Rendering|SetVisibility (Variables|Default|GetMoveParticle) (>= (Transformation|GetDistanceTo (Game|GetPlayerCharacter 0)) 4e+02) false)
            (if (Utilities|IsValid (Variables|Default|GetPath))
              (bind (_reachedpoint _pointtomove) (Default|PathLogic (Variables|Default|GetPath)))
              (if _reachedpoint
                (Variables|Default|SetPointToMove _pointtomove)
                (Variables|Default|SetInAction _reachedpoint)))))))))

(fn ConstructionScript)

(fn SetNewPath
  (params (Path :type BP%20AI%20Path%20Object%20Reference))
  (Variables|Default|SetPath Path)
  (Variables|Default|SetPathDistance 0.0)
  (AI|Navigation|SimpleMovetoLocation (Pawn|GetController) (Spline|GetLocationatSplinePoint (Variables|/Game/Blueprints/AI/BP_AIPath.BP_AIPath_C|GetSpline (Variables|Default|GetPath)) 0 "World"))
  (Variables|Default|SetNewPath true)
  (Rendering|SetVisibility (Variables|Default|GetMoveParticle) true false)
  (Variables|Default|Setenabled true))

(fn CheckReachedNewPath
  (Utilities|IsValid (Variables|Default|GetPath)
    (:Is%20Valid
      (if (Math|Vector|Equal(Vector) (Transformation|GetActorLocation) (Spline|GetLocationatSplinePoint (Variables|/Game/Blueprints/AI/BP_AIPath.BP_AIPath_C|GetSpline (Variables|Default|GetPath)) 0 "World") 2e+02)
        (Variables|Default|SetNewPath false)))))

(fn MoveAIAlongSpline
  (params (PointToMove :type Integer))
  ;[1 1 1] Set Location
  (Transformation|SetActorLocationAndRotation (Spline|GetLocationatDistanceAlongSpline (Variables|/Game/Blueprints/AI/BP_AIPath.BP_AIPath_C|GetSpline (Variables|Default|GetPath)) (Variables|Default|GetPathDistance) "World") (Spline|GetRotationatDistanceAlongSpline (Variables|/Game/Blueprints/AI/BP_AIPath.BP_AIPath_C|GetSpline (Variables|Default|GetPath)) (Variables|Default|GetPathDistance) "World"))
  (if (Math|Float|NearlyEqual(Float) (Spline|GetDistanceAlongSplineatSplinePoint (Variables|/Game/Blueprints/AI/BP_AIPath.BP_AIPath_C|GetSpline (Variables|Default|GetPath)) PointToMove) (+ (Variables|Default|GetPathDistance) 12.0) 11.9)
    (Variables|Default|SetAnimationEnum "NewEnumerator2")
    (else
      ;[1 1 1] Move to Point
      (Variables|Default|SetPathDistance (+ (Variables|Default|GetPathDistance) 12.0))
      (if (Utilities|Enum|NotEqual(Enum) (Variables|Default|GetAnimationEnum) "NewEnumerator1")
        _
        (else
          (Variables|Default|SetAnimationEnum "NewEnumerator1")))))
  (return (Math|Float|NearlyEqual(Float) (Spline|GetDistanceAlongSplineatSplinePoint (Variables|/Game/Blueprints/AI/BP_AIPath.BP_AIPath_C|GetSpline (Variables|Default|GetPath)) PointToMove) (+ (Variables|Default|GetPathDistance) 12.0) 11.9)))

(fn MovetoPlayer
  (bind _returnvalue (Game|GetPlayerCharacter 0))
  (if (<= (Transformation|GetDistanceTo (Game|GetPlayerCharacter 0)) 2.5e+02)
    (Components|Movement|StopMovementImmediately (Variables|Character|GetCharacterMovement))
    (elif (>= (Transformation|GetDistanceTo (Game|GetPlayerCharacter 0)) 801.0)
      (AI|Navigation|SimpleMovetoActor (Pawn|GetController) (Game|GetPlayerCharacter 0))
      (elif (>= (Transformation|GetDistanceTo (Game|GetPlayerCharacter 0)) 3e+03)
        (Transformation|SetActorLocationAndRotation (- (Transformation|GetActorForwardVector _returnvalue) "-500.000000, 0, 0") (Transformation|GetActorRotation _returnvalue) false true)))))

(fn SetParticleSystem
  (params (Particle :type Particle%20System%20Object%20Reference))
  (bind _particlesystem (Variables|Default|GetParticleSystem))
  (Effects|Components|ParticleSystem|SetTemplate _particlesystem Particle)
  (Rendering|SetVisibility _particlesystem (Utilities|IsValid Particle) false))

(fn GetParticleSystem
  (return (!= (Variables|/Script/Engine.ParticleSystemComponent|GetTemplate (Variables|Default|GetParticleSystem)) 0)))
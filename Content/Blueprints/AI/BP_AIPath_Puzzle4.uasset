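; BP_AIPath_Puzzle4 is the path logic that guides an AI companion through the fourth puzzle.
; PathLogic switches on CurrentStep, gating each step on player proximity and returning a reached flag and target point index.
; The steps fly around or wave at puzzle props, setting the AI's animation enum for waves, then pass the flag to IncreaseStep.
; A separate MyDelay event sets Execute after a timed delay.
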(event Custom|MyDelay
  (params (Time :type Float%20%28single-precision%29))
  (Utilities|FlowControl|Delay Time)
  (Variables|Default|SetExecute true))

(fn ConstructionScript
  (|CallParentFunction))

(fn PathLogic
  (bind _returnvalue (Game|GetPlayerCharacter 0))
  (bind _ai (Variables|Default|GetAI))
  (bind _returnvalue_2 (Transformation|GetDistanceTo _ai _returnvalue))
  (bind _returnvalue_3 (<= _returnvalue_2 4e+02))
  (switch int (Variables|Default|GetCurrentStep)
    (:0
      ;[1 1 1] Fly around WM
      (Variables|Default|SetoutputBool (<= (Transformation|GetDistanceTo (Variables|Default|GetAI) (Game|GetPlayerCharacter 0)) 8e+02))
      (Variables|Default|SetoutputInt 4))
    (:1
      ;[1 1 1] Fly Around blue ball
      (Variables|Default|SetoutputBool (<= (Transformation|GetDistanceTo (Variables|Default|GetAI) (Game|GetPlayerCharacter 0)) 8e+02))
      (Variables|Default|SetoutputInt 7))
    (:2
      ;[1 1 1] Wave at bowl
      (Variables|Default|SetoutputBool (<= (Transformation|GetDistanceTo (Variables|Default|GetAI) (Game|GetPlayerCharacter 0)) 8e+02))
      (Variables|Default|SetoutputInt 8)
      (Variables|/Game/Blueprints/AI/BP_AI.BP_AI_C|SetAnimationEnum (Variables|Default|GetAI) "NewEnumerator2"))
    (:3
      ;[1 1 1] Wave at plant
      (if _returnvalue_3
        (Variables|Default|SetoutputInt 99)
        (else
          (Variables|/Game/Blueprints/AI/BP_AI.BP_AI_C|SetAnimationEnum (Variables|Default|GetAI) "NewEnumerator2")
          (Variables|Default|SetoutputInt 0)))
      (Variables|Default|SetoutputBool _returnvalue_3)))
  (CallFunction|IncreaseStep (Variables|Default|GetoutputBool))
  (return (Variables|Default|GetoutputBool) (Variables|Default|GetoutputInt)))
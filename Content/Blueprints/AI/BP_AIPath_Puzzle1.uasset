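; AI path Blueprint for the first puzzle, scripting an AI that waits for the player, visits the right and left flowers, then waves by a bowl.
; An overridden PathLogic switches on the current step, returns whether the point is reached and the next move point, and advances via IncreaseStep.
; Proximity gates the first step; later steps poll an Execute flag set by a Delay-based custom event to time their pauses.
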(event Custom|MyDelay
  (params (Time :type Float%20%28single-precision%29))
  (Utilities|FlowControl|Delay Time)
  (Variables|Default|SetExecute true))

(fn ConstructionScript
  (|CallParentFunction))

(fn PathLogic
  (bind _returnvalue (Game|GetPlayerCharacter 0))
  (bind _ai (Variables|Default|GetAI))
  (bind _returnvalue_2 (Transformation|GetDistanceTo _ai _returnvalue))
  (bind _returnvalue_3 (<= _returnvalue_2 8e+02))
  (switch int (Variables|Default|GetCurrentStep)
    (:0
      ;[1 1 1] Wait for player to be close
      (if _returnvalue_3
        _
        (else
          (Variables|/Game/Blueprints/AI/BP_AI.BP_AI_C|SetAnimationEnum (Variables|Default|GetAI) "NewEnumerator3")))
      (Variables|Default|SetoutputBool _returnvalue_3)
      (Variables|Default|SetoutputInt 1))
    (:1
      ;[1 1 1] Move to right flower and wait
      (CallFunction|MyDelay 2.0)
      (if (Variables|Default|GetExecute)
        (Variables|Default|SetoutputBool true)
        (Variables|Default|SetoutputInt 2)
        (Variables|Default|SetExecute false)
        (else
          (Variables|Default|SetoutputBool false))))
    (:2
      ;[1 1 1] Move to left flower and wait
      (CallFunction|MyDelay 2.0)
      (if (Variables|Default|GetExecute)
        (Variables|Default|SetoutputBool true)
        (Variables|Default|SetoutputInt 3)
        (Variables|Default|SetExecute false)
        (else
          (Variables|Default|SetoutputBool false))))
    (:3
      ;[1 1 1] Wave between bowl
      (CallFunction|MyDelay 2.0)
      (Variables|/Game/Blueprints/AI/BP_AI.BP_AI_C|SetAnimationEnum (Variables|Default|GetAI) "NewEnumerator2")
      (if (Variables|Default|GetExecute)
        (Variables|Default|SetoutputInt 99)
        (else
          (Variables|Default|SetoutputInt 0)))
      (Variables|Default|SetoutputBool (Variables|Default|GetExecute))))
  (CallFunction|IncreaseStep (Variables|Default|GetoutputBool))
  (return (Variables|Default|GetoutputBool) (Variables|Default|GetoutputInt)))
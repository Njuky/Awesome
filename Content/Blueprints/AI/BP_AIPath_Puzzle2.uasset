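; AI path script for the second puzzle, driving an AI's steps based on player proximity.
; PathLogic switches on CurrentStep, setting an animation while the player is out of range and choosing the point to move to.
; The distance check is returned as ReachedPoint and passed to IncreaseStep.
; A separate MyDelay event sets an Execute flag after a given time.
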(event Custom|MyDelay
  (params (Time :type Float%20%28single-precision%29))
  (Utilities|FlowControl|Delay Time)
  (Variables|Default|SetExecute true))

(fn ConstructionScript
  (|CallParentFunction))

(fn PathLogic
  (bind _returnvalue (Game|GetPlayerCharacter 0))
  (bind _returnvalue_2 (Game|GetPlayerCharacter 0))
  (bind _ai (Variables|Default|GetAI))
  (bind _ai_2 (Variables|Default|GetAI))
  (bind _returnvalue_3 (Transformation|GetDistanceTo _ai _returnvalue))
  (bind _returnvalue_4 (Transformation|GetDistanceTo _ai_2 _returnvalue_2))
  (bind _returnvalue_5 (<= _returnvalue_3 8e+02))
  (bind _returnvalue_6 (<= _returnvalue_4 8e+02))
  (switch int (Variables|Default|GetCurrentStep)
    (:0
      ;[1 1 1] Wait for player to be close
      (if _returnvalue_5
        _
        (else
          (Variables|/Game/Blueprints/AI/BP_AI.BP_AI_C|SetAnimationEnum (Variables|Default|GetAI) "NewEnumerator3")))
      (Variables|Default|SetoutputBool _returnvalue_5)
      (Variables|Default|SetoutputInt 1))
    (:1
      ;[1 1 1] Wave between bowl
      (if _returnvalue_6
        (Variables|Default|SetoutputInt 99)
        (else
          (Variables|/Game/Blueprints/AI/BP_AI.BP_AI_C|SetAnimationEnum (Variables|Default|GetAI) "NewEnumerator2")
          (Variables|Default|SetoutputInt 0)))
      (Variables|Default|SetoutputBool _returnvalue_6)))
  (CallFunction|IncreaseStep (Variables|Default|GetoutputBool))
  (return (Variables|Default|GetoutputBool) (Variables|Default|GetoutputInt)))
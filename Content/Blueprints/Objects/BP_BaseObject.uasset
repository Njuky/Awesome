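; BP_BaseObject is a base object whose static mesh switches between past and future looks.
; On BeginPlay it caches the mesh's material slot count.
; ChangeTexture takes a Time flag and sets every slot to the matching entry in the MaterialFuture array when true, or MaterialPast when false.
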(event EventBeginPlay
  (Variables|Default|SetMaterialAmount (Utilities|Array|Length (Rendering|Material|GetMaterials (Variables|Default|GetStaticMesh)))))

(fn ConstructionScript)

(fn ChangeTexture
  (params (Time :type Boolean))
  (if Time
    (for _index (range 0 (- (Variables|Default|GetMaterialAmount) 1))
      (Rendering|Material|SetMaterial (Variables|Default|GetStaticMesh) _index (Utilities|Array|Get(acopy) (Variables|Default|GetMaterial_Future) _index)))
    (else
      (for _index_2 (range 0 (- (Variables|Default|GetMaterialAmount) 1))
        (Rendering|Material|SetMaterial (Variables|Default|GetStaticMesh) _index_2 (Utilities|Array|Get(acopy) (Variables|Default|GetMaterial_Past) _index_2))))))
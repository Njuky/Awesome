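; Base collectible item that the player picks up into a single Inventory slot on BP_Controller and can drop again.
; Overlapping the Box with BP_Character enables input, so F or gamepad face-right runs CollectObject, which hides and disables the item; DropItem reverses this.
; Time-relevant items are visible, collidable and interactable only while the controller's CurrentTime matches SupposedTime.
; Tick polls Enabled and the time to update collision and visibility.
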(event OnComponentBeginOverlap(Box)
  (params (OtherActor :type Actor%20Object%20Reference) (OtherComp :type Primitive%20Component%20Object%20Reference) (OtherBodyIndex :type Integer) (bFromSweep :type Boolean) (SweepResult :type Hit%20Result%20Structure%20%28by%20ref%29))
  ;[0.3254 0.2845 1] B to interact Widget
  (Utilities|Casting|CastToBP_Character OtherActor)
  (if (Variables|Default|GetTimeRelevant)
    (Utilities|CheckTime
      (:True
        _)))
  (Variables|Default|SetShowBtn true)
  (Input|EnableInput (Game|GetPlayerController 0)))

(event OnComponentEndOverlap(Box)
  (params (OtherActor :type Actor%20Object%20Reference) (OtherComp :type Primitive%20Component%20Object%20Reference) (OtherBodyIndex :type Integer))
  ;[0.9367 0.342 1] Remove Widget when out of sphere
  (Utilities|Casting|CastToBP_Character OtherActor)
  (if (Variables|Default|GetTimeRelevant)
    (Utilities|CheckTime
      (:True
        _)))
  (Input|DisableInput (Game|GetPlayerController 0)))

(event EventTick
  (params (DeltaSeconds :type Float%20%28single-precision%29))
  (bind _box (Variables|Default|GetBox))
  (Utilities|FlowControl|Sequence
    (:then_0
      (if (Variables|Default|GetEnabled)
        (Collision|SetActorEnableCollision true)
        (else
          (Collision|SetActorEnableCollision false))))
    (:then_1
      (if (and (Variables|Default|GetTimeRelevant) (Variables|Default|GetEnabled))
        (bind _asbp_controller (Utilities|Casting|CastToBP_Controller (Game|GetPlayerController 0)))
        (if (Math|Boolean|Equal(Boolean) (Variables|/Game/Blueprints/Character/Player/BP_Controller.BP_Controller_C|GetCurrentTime _asbp_controller) (Variables|Default|GetSupposedTime))
          (Rendering|SetVisibility (Variables|Default|GetObject_Mesh) true false)
          (Collision|SetActorEnableCollision true)
          (Variables|/Script/Engine.PrimitiveComponent|SetbGenerateOverlapEvents _box true)
          (else
            (Rendering|SetVisibility (Variables|Default|GetObject_Mesh) false false)
            (Collision|SetActorEnableCollision false)
            (Variables|/Script/Engine.PrimitiveComponent|SetbGenerateOverlapEvents _box false)))))))

(event Input|KeyboardEvents|F
  (params (Key :type Key%20Structure :default "AnyKey"))
  (:Pressed
    (if (Variables|Default|GetTimeRelevant)
      (Utilities|CheckTime
        (:True
          _)))
    (CallFunction|CollectObject)
    (Audio|PlaySoundatLocation "/Game/Audio/Sound/Platzhalter_Itemaufheben.Platzhalter_Itemaufheben" "0, 0, 0")))

(event Input|GamepadEvents|GamepadFaceButtonRight
  (params (Key :type Key%20Structure :default "AnyKey"))
  (:Pressed
    (if (Variables|Default|GetTimeRelevant)
      (Utilities|CheckTime
        (:True
          _)))
    (CallFunction|CollectObject)
    (Audio|PlaySoundatLocation "/Game/Audio/Sound/Platzhalter_Itemaufheben.Platzhalter_Itemaufheben" "0, 0, 0")))

(fn ConstructionScript)

(fn CollectObject
  (bind _asbp_controller (Utilities|Casting|CastToBP_Controller (Game|GetPlayerController 0)))
  (if (== (Variables|/Game/Blueprints/Character/Player/BP_Controller.BP_Controller_C|GetInventory _asbp_controller) 0)
    (Rendering|SetVisibility (Variables|Default|GetDefaultSceneRoot) false true)
    (Collision|SetActorEnableCollision false)
    (Variables|/Game/Blueprints/Character/Player/BP_Controller.BP_Controller_C|SetInventory _asbp_controller self)
    (Variables|Default|SetEnabled false)))

(fn DropItem
  (bind _returnvalue (Game|GetPlayerController 0))
  (Rendering|SetVisibility (Variables|Default|GetDefaultSceneRoot) true true)
  (Variables|Default|SetEnabled true)
  (bind _asbp_controller (Utilities|Casting|CastToBP_Controller _returnvalue))
  (Variables|/Game/Blueprints/Character/Player/BP_Controller.BP_Controller_C|SetInventory _asbp_controller 0)
  (Input|DisableInput _returnvalue)
  (Collision|SetActorEnableCollision true))
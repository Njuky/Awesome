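; BP_MainMenu is a Blueprint that creates and displays the main menu widget.
; On BeginPlay, after a short delay, it creates MainMenu, stores the reference, sets itself as the widget's Owner, adds it to the viewport and gives the PLAY button keyboard focus.
; The RunMainMenu event jumps into the same creation chain without the delay.
; A closing validity check leads to a loop over PLAY, CREDITS and QUIT that performs no action.
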(event Custom|Run%20Main%20Menu
  (bind _returnvalue (UserInterface|CreateWidget "/Game/Blueprints/Widgets/MainMenu.MainMenu_C"))
  (bind _output_get (Variables|Default|SetMainMenu%20Reference _returnvalue))
  (Variables|/Game/Blueprints/Widgets/MainMenu.MainMenu_C|SetOwner (Variables|Default|GetMainMenu%20Reference) self)
  (UserInterface|Viewport|AddtoViewport _output_get 0)
  (Widget|SetKeyboardFocus (Variables|/Game/Blueprints/Widgets/MainMenu.MainMenu_C|GetPLAY (Variables|Default|GetMainMenu%20Reference)))
  (if (Utilities|IsValid (Variables|Default|GetMainMenu%20Reference))
    (for _array_element (Utilities|Array|MakeArray (Variables|/Game/Blueprints/Widgets/MainMenu.MainMenu_C|GetPLAY (Variables|Default|GetMainMenu%20Reference)) (Variables|/Game/Blueprints/Widgets/MainMenu.MainMenu_C|GetCREDITS (Variables|Default|GetMainMenu%20Reference)) (Variables|/Game/Blueprints/Widgets/MainMenu.MainMenu_C|GetQUIT (Variables|Default|GetMainMenu%20Reference)))
      _)))

(event EventBeginPlay
  (Utilities|FlowControl|Delay 0.2)
  (bind _returnvalue (UserInterface|CreateWidget "/Game/Blueprints/Widgets/MainMenu.MainMenu_C"))
  (bind _output_get (Variables|Default|SetMainMenu%20Reference _returnvalue))
  (Variables|/Game/Blueprints/Widgets/MainMenu.MainMenu_C|SetOwner (Variables|Default|GetMainMenu%20Reference) self)
  (UserInterface|Viewport|AddtoViewport _output_get 0)
  (Widget|SetKeyboardFocus (Variables|/Game/Blueprints/Widgets/MainMenu.MainMenu_C|GetPLAY (Variables|Default|GetMainMenu%20Reference)))
  (if (Utilities|IsValid (Variables|Default|GetMainMenu%20Reference))
    (for _array_element (Utilities|Array|MakeArray (Variables|/Game/Blueprints/Widgets/MainMenu.MainMenu_C|GetPLAY (Variables|Default|GetMainMenu%20Reference)) (Variables|/Game/Blueprints/Widgets/MainMenu.MainMenu_C|GetCREDITS (Variables|Default|GetMainMenu%20Reference)) (Variables|/Game/Blueprints/Widgets/MainMenu.MainMenu_C|GetQUIT (Variables|Default|GetMainMenu%20Reference)))
      _)))

(fn ConstructionScript)
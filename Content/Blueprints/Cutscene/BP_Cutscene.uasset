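; BP_Cutscene is a proximity-triggered actor that ends the current level and returns the game to the main menu.
; Each tick it checks whether the player character is within range and, guarded by a one-shot Done flag, fades the camera out and holds it.
; After a short delay that outlasts the fade, it opens the MainMenu level.
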(event EventTick
  (params (DeltaSeconds :type Float%20%28single-precision%29))
  (if (<= (Transformation|GetDistanceTo (Game|GetPlayerCharacter 0)) 1e+03)
    (if (not (Variables|Default|GetDone))
      (Variables|Default|SetDone true)
      (CameraFades|StartCameraFade :self (Game|GetPlayerCameraManager 0) :ToAlpha 1.0 :Duration 3.0 :bHoldWhenFinished true)
      (Utilities|FlowControl|Delay 3.5)
      (Game|OpenLevel(byName) "MainMenu"))))

(fn ConstructionScript)
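; Quest 4 watering machine puzzle where the player places carried objects into four color-coded slots to turn a small plant into a giant one.
; Box overlaps enable input and mark the active slot, so interact swaps items between controller inventory and slot, mirroring the item's mesh and material.
; Matching color tags set Solved flags, and Tick swaps plant visibility when all are set and the controller's CurrentTime is false.
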(event OnComponentBeginOverlap(BoxOrange)
  (params (OverlappedComponent :type Primitive%20Component%20Object%20Reference) (OtherActor :type Actor%20Object%20Reference) (OtherComp :type Primitive%20Component%20Object%20Reference) (OtherBodyIndex :type Integer) (bFromSweep :type Boolean) (SweepResult :type Hit%20Result%20Structure%20%28by%20ref%29))
  (CallFunction|Enable OtherActor)
  (Variables|Default|Setplace1 true))

(event OnComponentEndOverlap(BoxOrange)
  (params (OverlappedComponent :type Primitive%20Component%20Object%20Reference) (OtherActor :type Actor%20Object%20Reference) (OtherComp :type Primitive%20Component%20Object%20Reference) (OtherBodyIndex :type Integer))
  (CallFunction|Disable OtherActor)
  (Variables|Default|Setplace1 false))

(event OnComponentBeginOverlap(BoxYellow)
  (params (OverlappedComponent :type Primitive%20Component%20Object%20Reference) (OtherActor :type Actor%20Object%20Reference) (OtherComp :type Primitive%20Component%20Object%20Reference) (OtherBodyIndex :type Integer) (bFromSweep :type Boolean) (SweepResult :type Hit%20Result%20Structure%20%28by%20ref%29))
  (CallFunction|Enable OtherActor)
  (Variables|Default|Setplace2 true))

(event OnComponentEndOverlap(BoxYellow)
  (params (OverlappedComponent :type Primitive%20Component%20Object%20Reference) (OtherActor :type Actor%20Object%20Reference) (OtherComp :type Primitive%20Component%20Object%20Reference) (OtherBodyIndex :type Integer))
  (CallFunction|Disable OtherActor)
  (Variables|Default|Setplace2 false))

(event OnComponentBeginOverlap(BoxGreen)
  (params (OverlappedComponent :type Primitive%20Component%20Object%20Reference) (OtherActor :type Actor%20Object%20Reference) (OtherComp :type Primitive%20Component%20Object%20Reference) (OtherBodyIndex :type Integer) (bFromSweep :type Boolean) (SweepResult :type Hit%20Result%20Structure%20%28by%20ref%29))
  (CallFunction|Enable OtherActor)
  (Variables|Default|Setplace3 true))

(event OnComponentEndOverlap(BoxGreen)
  (params (OverlappedComponent :type Primitive%20Component%20Object%20Reference) (OtherActor :type Actor%20Object%20Reference) (OtherComp :type Primitive%20Component%20Object%20Reference) (OtherBodyIndex :type Integer))
  (CallFunction|Disable OtherActor)
  (Variables|Default|Setplace3 false))

(event OnComponentBeginOverlap(BoxBlue)
  (params (OverlappedComponent :type Primitive%20Component%20Object%20Reference) (OtherActor :type Actor%20Object%20Reference) (OtherComp :type Primitive%20Component%20Object%20Reference) (OtherBodyIndex :type Integer) (bFromSweep :type Boolean) (SweepResult :type Hit%20Result%20Structure%20%28by%20ref%29))
  (CallFunction|Enable OtherActor)
  (Variables|Default|Setplace4 true))

(event OnComponentEndOverlap(BoxBlue)
  (params (OverlappedComponent :type Primitive%20Component%20Object%20Reference) (OtherActor :type Actor%20Object%20Reference) (OtherComp :type Primitive%20Component%20Object%20Reference) (OtherBodyIndex :type Integer))
  (CallFunction|Disable OtherActor)
  (Variables|Default|Setplace4 false))

(event EventTick
  (params (DeltaSeconds :type Float%20%28single-precision%29))
  (if (Math|Boolean|ANDBoolean (Utilities|Array|Get(acopy) (Variables|Default|Getsolved)) (Utilities|Array|Get(acopy) (Variables|Default|Getsolved) 1) (Utilities|Array|Get(acopy) (Variables|Default|Getsolved) 2) (Utilities|Array|Get(acopy) (Variables|Default|Getsolved) 3) (not (Variables|/Script/Project2016.C_PlayerController|GetcurrentTime (Variables|Default|GetPlayerControllerRef))))
    (Rendering|SetVisibility (Variables|Default|GetSmallPlant) false false)
    (Rendering|SetVisibility (Variables|Default|GetGiantPlant) true false)))

(event EventBeginPlay
  (bind _asbp_controller (Utilities|Casting|CastToBP_Controller (Game|GetPlayerController 0)))
  (Variables|Default|SetPlayerControllerRef _asbp_controller))

(event Input|KeyboardEvents|F
  (params (Key :type Key%20Structure :default "AnyKey"))
  (bind _playercontrollerref (Variables|Default|GetPlayerControllerRef))
  (bind _c_inventory (Variables|/Script/Project2016.C_PlayerController|Getc_Inventory _playercontrollerref))
  (:Pressed
    (Variables|/Script/Project2016.C_PlayerController|SetanimationType _playercontrollerref 2)
    (if (!= _c_inventory 0)
      (if (== (Utilities|GetClass _c_inventory) (Variables|Default|GetSupposedObject))
        (if (Variables|Default|Getplace1)
          (CallFunction|SetSlot (Variables|Default|GetSlot1))
          (elif (Variables|Default|Getplace2)
            (CallFunction|SetSlot (Variables|Default|GetSlot2))
            (elif (Variables|Default|Getplace3)
              (CallFunction|SetSlot (Variables|Default|GetSlot3))
              (elif (Variables|Default|Getplace4)
                (CallFunction|SetSlot (Variables|Default|GetSlot4)))))))
      (elif (Variables|Default|Getplace1)
        (CallFunction|GetSlot (Variables|Default|GetSlot1))
        (elif (Variables|Default|Getplace2)
          (CallFunction|GetSlot (Variables|Default|GetSlot2))
          (elif (Variables|Default|Getplace3)
            (CallFunction|GetSlot (Variables|Default|GetSlot3))
            (elif (Variables|Default|Getplace4)
              (CallFunction|GetSlot (Variables|Default|GetSlot4)))))))))

(event Input|GamepadEvents|GamepadFaceButtonRight
  (params (Key :type Key%20Structure :default "AnyKey"))
  (bind _playercontrollerref (Variables|Default|GetPlayerControllerRef))
  (bind _c_inventory (Variables|/Script/Project2016.C_PlayerController|Getc_Inventory _playercontrollerref))
  (:Pressed
    (Variables|/Script/Project2016.C_PlayerController|SetanimationType _playercontrollerref 2)
    (if (!= _c_inventory 0)
      (if (== (Utilities|GetClass _c_inventory) (Variables|Default|GetSupposedObject))
        (if (Variables|Default|Getplace1)
          (CallFunction|SetSlot (Variables|Default|GetSlot1))
          (elif (Variables|Default|Getplace2)
            (CallFunction|SetSlot (Variables|Default|GetSlot2))
            (elif (Variables|Default|Getplace3)
              (CallFunction|SetSlot (Variables|Default|GetSlot3))
              (elif (Variables|Default|Getplace4)
                (CallFunction|SetSlot (Variables|Default|GetSlot4)))))))
      (elif (Variables|Default|Getplace1)
        (CallFunction|GetSlot (Variables|Default|GetSlot1))
        (elif (Variables|Default|Getplace2)
          (CallFunction|GetSlot (Variables|Default|GetSlot2))
          (elif (Variables|Default|Getplace3)
            (CallFunction|GetSlot (Variables|Default|GetSlot3))
            (elif (Variables|Default|Getplace4)
              (CallFunction|GetSlot (Variables|Default|GetSlot4)))))))))

(fn ConstructionScript)

(fn Enable
  (params (Other%20Actor :type Actor%20Object%20Reference))
  (bind _returnvalue (Game|GetPlayerController 0))
  (Utilities|Casting|CastToBP_Character Other%20Actor)
  (Input|EnableInput _returnvalue)
  (bind _asbp_controller (Utilities|Casting|CastToBP_Controller _returnvalue))
  (Variables|/Script/Project2016.C_PlayerController|SetbCanInteract _asbp_controller false))

(fn Disable
  (params (Other%20Actor :type Actor%20Object%20Reference))
  (bind _returnvalue (Game|GetPlayerController 0))
  (Utilities|Casting|CastToBP_Character Other%20Actor)
  (Input|DisableInput _returnvalue)
  (bind _asbp_controller (Utilities|Casting|CastToBP_Controller _returnvalue))
  (Variables|/Script/Project2016.C_PlayerController|SetbCanInteract _asbp_controller true))

(fn SetSlot
  (params (Slot :type Base%20Collectable%20Object%20Reference))
  (if (== Slot 0)
    (if (Variables|Default|Getplace1)
      (bind _output_get (Variables|Default|SetSlot1 (Variables|/Script/Project2016.C_PlayerController|Getc_Inventory (Variables|Default|GetPlayerControllerRef))))
      (CallFunction|SetSM (Variables|Default|GetOrangeBall) true _output_get)
      (if (Utilities|Name|Equal(Name) (Variables|/Script/Project2016.BaseCollectable|GetsupposedBowlTag (Variables|Default|GetSlot1)) "Orange")
        (Utilities|Array|SetArrayElem (Variables|Default|Getsolved) 0 true))
      (Variables|/Script/Project2016.C_PlayerController|Setc_Inventory (Variables|Default|GetPlayerControllerRef) 0 :!label _label)
      (elif (Variables|Default|Getplace2)
        (bind _output_get_2 (Variables|Default|SetSlot2 (Variables|/Script/Project2016.C_PlayerController|Getc_Inventory (Variables|Default|GetPlayerControllerRef))))
        (CallFunction|SetSM (Variables|Default|GetYellowBall) true _output_get_2)
        (if (Utilities|Name|Equal(Name) (Variables|/Script/Project2016.BaseCollectable|GetsupposedBowlTag (Variables|Default|GetSlot2)) "Yellow")
          (Utilities|Array|SetArrayElem (Variables|Default|Getsolved) 1 true)
          (goto _label)
          (else
            (goto _label)))
        (elif (Variables|Default|Getplace3)
          (bind _output_get_3 (Variables|Default|SetSlot3 (Variables|/Script/Project2016.C_PlayerController|Getc_Inventory (Variables|Default|GetPlayerControllerRef))))
          (CallFunction|SetSM (Variables|Default|GetGreenBall) true _output_get_3)
          (if (Utilities|Name|Equal(Name) (Variables|/Script/Project2016.BaseCollectable|GetsupposedBowlTag (Variables|Default|GetSlot3)) "Green")
            (Utilities|Array|SetArrayElem (Variables|Default|Getsolved) 2 true)
            (goto _label)
            (else
              (goto _label)))
          (elif (Variables|Default|Getplace4)
            (bind _output_get_4 (Variables|Default|SetSlot4 (Variables|/Script/Project2016.C_PlayerController|Getc_Inventory (Variables|Default|GetPlayerControllerRef))))
            (CallFunction|SetSM (Variables|Default|GetBlueBall) true _output_get_4)
            (if (Utilities|Name|Equal(Name) (Variables|/Script/Project2016.BaseCollectable|GetsupposedBowlTag (Variables|Default|GetSlot4)) "Blue")
              (Utilities|Array|SetArrayElem (Variables|Default|Getsolved) 3 true)
              (goto _label)
              (else
                (goto _label)))))))))

(fn GetSlot
  (params (Slot :type Base%20Collectable%20Object%20Reference))
  (if (not (== Slot 0))
    (if (== Slot (Variables|Default|GetSlot1))
      (Variables|/Script/Project2016.C_PlayerController|Setc_Inventory (Variables|Default|GetPlayerControllerRef) (Variables|Default|GetSlot1))
      (bind _output_get (Variables|Default|SetSlot1 0))
      (CallFunction|SetSM (Variables|Default|GetOrangeBall) false _output_get)
      (Utilities|Array|SetArrayElem (Variables|Default|Getsolved) 0 false)
      (elif (== Slot (Variables|Default|GetSlot2))
        (Variables|/Script/Project2016.C_PlayerController|Setc_Inventory (Variables|Default|GetPlayerControllerRef) (Variables|Default|GetSlot2))
        (bind _output_get_2 (Variables|Default|SetSlot2 0))
        (CallFunction|SetSM (Variables|Default|GetYellowBall) false _output_get_2)
        (Utilities|Array|SetArrayElem (Variables|Default|Getsolved) 1 false)
        (elif (== Slot (Variables|Default|GetSlot3))
          (Variables|/Script/Project2016.C_PlayerController|Setc_Inventory (Variables|Default|GetPlayerControllerRef) (Variables|Default|GetSlot3))
          (bind _output_get_3 (Variables|Default|SetSlot3 0))
          (CallFunction|SetSM (Variables|Default|GetGreenBall) false _output_get_3)
          (Utilities|Array|SetArrayElem (Variables|Default|Getsolved) 2 false)
          (elif (== Slot (Variables|Default|GetSlot4))
            (Variables|/Script/Project2016.C_PlayerController|Setc_Inventory (Variables|Default|GetPlayerControllerRef) (Variables|Default|GetSlot4))
            (bind _output_get_4 (Variables|Default|SetSlot4 0))
            (CallFunction|SetSM (Variables|Default|GetBlueBall) false _output_get_4)
            (Utilities|Array|SetArrayElem (Variables|Default|Getsolved) 3 false)))))))

(fn SetSM
  (params (StaticMesh :type Static%20Mesh%20Component%20Object%20Reference) (visible :type Boolean) (Slot :type Base%20Collectable%20Object%20Reference))
  (bind _staticmeshcomponent (Variables|/Script/Project2016.BaseCollectable|GetStaticMeshComponent Slot))
  (if visible
    (Rendering|SetVisibility StaticMesh visible false)
    (Components|StaticMesh|SetStaticMesh StaticMesh (Variables|/Script/Engine.StaticMeshComponent|GetStaticMesh _staticmeshcomponent))
    (Rendering|Material|SetMaterial StaticMesh 0 (Rendering|Material|GetMaterial _staticmeshcomponent 0))
    (else
      (Rendering|SetVisibility StaticMesh visible false))))
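; Quest plant puzzle actor that grows from small to giant across the controller's two time states once every bowl is solved.
; Tick polls the controller's CurrentTime: when true, it hides Plant and checks all bowls, playing water sound and particles and setting LittlePlant if solved.
; When false, it shows Plant and uses that flag to display either the giant plant with collision or the small one.
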(event EventTick
  (params (DeltaSeconds :type Float%20%28single-precision%29))
  (bind _plant (Variables|Default|GetPlant))
  (bind _giantplant (Variables|Default|GetGiantPlant))
  (bind _giantplant_2 (Variables|Default|GetGiantPlant))
  (bind _solvedarray (Variables|Default|GetSolvedArray))
  (bind _smallplant (Variables|Default|GetSmallPlant))
  (bind _waterparticle (Variables|Default|GetWaterParticle))
  (bind _giantplant_3 (Variables|Default|GetGiantPlant))
  (if (Variables|/Script/Project2016.C_PlayerController|GetcurrentTime (Variables|Default|GetPlayerControllerRef))
    (Rendering|SetActorHiddenInGame _plant true)
    (bind (_array_element _array_index) (Utilities|Array|ForEachLoopwithBreak (Variables|Default|GetBowlArray) :!label _label)
      (:LoopBody
        (if (Variables|/Script/Project2016.C_Bowl|Getc_solved _array_element)
          (Utilities|Array|SetArrayElem _solvedarray _array_index true)
          (Math|Integer|IncrementInt (Variables|Default|GetDoneIndex))
          (else
            (Utilities|Array|SetArrayElem _solvedarray _array_index false)
            (Variables|Default|SetDoneIndex 0)
            (goto _label Break))))
      (:Completed
        (if (== (Variables|Default|GetDoneIndex) (Utilities|Array|Length (Variables|Default|GetSolvedArray)))
          (Audio|PlaySoundatLocation "/Game/Audio/Sound/Puzzel_Sounds/SoundCues/Wasseregluckern_Cue.Wasseregluckern_Cue" (Transformation|GetActorLocation))
          (Rendering|SetActorHiddenInGame _waterparticle false)
          (Variables|Default|SetLittlePlant true)
          (Variables|Default|SetDoneIndex 0)
          (else
            (Rendering|SetVisibility (Variables|Default|GetSmallPlant) true false)
            (Rendering|SetVisibility _giantplant_2 false false)
            (Rendering|SetActorHiddenInGame _waterparticle true)
            (Collision|SetCollisionEnabled _giantplant_2 "NoCollision")
            (Variables|Default|SetLittlePlant false)))))
    (else
      (Rendering|SetActorHiddenInGame _plant false)
      (if (Variables|Default|GetLittlePlant)
        (Rendering|SetVisibility _smallplant false false)
        (Rendering|SetVisibility _giantplant true false)
        (Collision|SetCollisionEnabled _giantplant "QueryAndPhysics")
        (else
          (Rendering|SetVisibility _smallplant true false)
          (Rendering|SetVisibility _giantplant_3 false false)
          (Collision|SetCollisionEnabled _giantplant_3 "NoCollision")))
      (Rendering|SetActorHiddenInGame (Variables|Default|GetWaterParticle) true))))

(event EventBeginPlay
  (bind _asbp_controller (Utilities|Casting|CastToBP_Controller (Game|GetPlayerController 0)))
  (Variables|Default|SetPlayerControllerRef _asbp_controller)
  (for _array_element (Variables|Default|GetBowlArray)
    (Utilities|Array|Add (Variables|Default|GetSolvedArray) false)))

(fn ConstructionScript)
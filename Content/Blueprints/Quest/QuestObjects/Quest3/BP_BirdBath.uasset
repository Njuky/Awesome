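; Quest 3 bird bath puzzle object that shows water or an empty bowl according to the controller's CurrentTime flag.
; Overlapping its sphere enables the interact key, which, while CurrentTime is true, moves accepted items between the controller's single inventory slot and the bath.
; Using the stone on a placed berry smashes it, and Tick then turns the liquid and any inserted item red, retagging that item "pRed".
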(event OnComponentBeginOverlap(Sphere)
  (params (OtherActor :type Actor%20Object%20Reference) (OtherComp :type Primitive%20Component%20Object%20Reference) (OtherBodyIndex :type Integer) (bFromSweep :type Boolean) (SweepResult :type Hit%20Result%20Structure%20%28by%20ref%29))
  (Utilities|Casting|CastToBP_Character OtherActor)
  (Input|EnableInput (Game|GetPlayerController 0))
  (bind _asbp_controller_2 (Utilities|Casting|CastToBP_Controller2 (Game|GetPlayerController 0)))
  (Variables|/Script/Project2016.C_PlayerController|SetbCanInteract _asbp_controller_2 false))

(event OnComponentEndOverlap(Sphere)
  (params (OtherActor :type Actor%20Object%20Reference) (OtherComp :type Primitive%20Component%20Object%20Reference) (OtherBodyIndex :type Integer))
  (Utilities|Casting|CastToBP_Character OtherActor)
  (Input|DisableInput (Game|GetPlayerController 0))
  (bind _asbp_controller_2 (Utilities|Casting|CastToBP_Controller2 (Game|GetPlayerController 0)))
  (Variables|/Script/Project2016.C_PlayerController|SetbCanInteract _asbp_controller_2 true))

(event EventBeginPlay
  (bind _asbp_controller_2 (Utilities|Casting|CastToBP_Controller2 (Game|GetPlayerController 0)))
  (Variables|Default|SetpController_Ref _asbp_controller_2))

(event EventTick
  (params (DeltaSeconds :type Float%20%28single-precision%29))
  (bind _c_slot (Variables|Default|Getc_slot))
  (if (Variables|/Script/Project2016.C_PlayerController|GetcurrentTime (Variables|Default|GetpController_Ref))
    (if (Variables|Default|Getsmashed)
      (Rendering|Material|SetMaterial (Variables|Default|GetBowlWater) 1 "/Game/Art/Materials/Balls/M_Red.M_Red")
      (if (!= (Variables|Default|Getc_slot) 0)
        (Rendering|Material|SetMaterial (Variables|/Script/Project2016.BaseCollectable|GetStaticMeshComponent _c_slot) 0 "/Game/Art/Materials/Balls/M_Red.M_Red")
        (Variables|/Script/Project2016.BaseCollectable|SetsupposedBowlTag _c_slot "pRed")
        (Rendering|Material|SetMaterial (Variables|Default|GetInsertedObject) 0 "/Game/Art/Materials/Balls/M_Red.M_Red"))
      (else
        (Rendering|SetVisibility (Variables|Default|GetBowl) true false)
        (Rendering|SetVisibility (Variables|Default|GetBowlWater) false false)))
    (else
      (Rendering|Material|SetMaterial (Variables|Default|GetBowlWater) 1 "/Game/Art/Puzzel_Assets/M_water.M_water")
      (Rendering|SetVisibility (Variables|Default|GetBowlWater) true false)
      (Rendering|SetVisibility (Variables|Default|GetBowl) false false))))

(event Input|KeyboardEvents|F
  (params (Key :type Key%20Structure :default "AnyKey"))
  (bind _pcontroller_ref (Variables|Default|GetpController_Ref))
  (bind _pcontroller_ref_2 (Variables|Default|GetpController_Ref))
  (bind _pcontroller_ref_3 (Variables|Default|GetpController_Ref))
  (:Pressed
    (Variables|/Script/Project2016.C_PlayerController|SetanimationType _pcontroller_ref 2)
    (if (Variables|/Script/Project2016.C_PlayerController|GetcurrentTime _pcontroller_ref)
      (if (!= (Variables|/Script/Project2016.C_PlayerController|Getc_Inventory (Variables|Default|GetpController_Ref)) 0)
        (if (and (== (Utilities|GetClass (Variables|/Script/Project2016.C_PlayerController|Getc_Inventory (Variables|Default|GetpController_Ref))) (Variables|Default|GetacceptedClass)) (== (Variables|Default|Getc_Slot_Berry) 0))
          (Rendering|SetVisibility (Variables|Default|GetInsertedObject) true false)
          (Variables|Default|Setc_Slot (Variables|/Script/Project2016.C_PlayerController|Getc_Inventory _pcontroller_ref_2))
          (Variables|/Script/Project2016.C_PlayerController|Setc_Inventory _pcontroller_ref_2 0)
          (elif (and (== (Utilities|GetClass (Variables|/Script/Project2016.C_PlayerController|Getc_Inventory (Variables|Default|GetpController_Ref))) (Variables|Default|GetacceptedClassBerry)) (== (Variables|Default|Getc_Slot) 0))
            (Rendering|SetVisibility (Variables|Default|GetBerry) true false)
            (Variables|Default|Setc_Slot_Berry (Variables|/Script/Project2016.C_PlayerController|Getc_Inventory _pcontroller_ref_3))
            (Variables|/Script/Project2016.C_PlayerController|Setc_Inventory _pcontroller_ref_3 0)
            (elif (and (== (Utilities|GetClass (Variables|/Script/Project2016.C_PlayerController|Getc_Inventory (Variables|Default|GetpController_Ref))) (Variables|Default|GetacceptedClassStone)) (!= (Variables|Default|Getc_Slot_Berry) 0))
              (Variables|Default|Setc_Slot_Berry 0)
              (Variables|/Script/Project2016.C_PlayerController|Setc_Inventory (Variables|Default|GetpController_Ref) 0)
              (Variables|Default|Setsmashed true)
              (Rendering|SetVisibility (Variables|Default|GetBowlWater) true false)
              (Rendering|SetVisibility (Variables|Default|GetBowl) false false))))
        (else
          (if (!= (Variables|Default|Getc_Slot) 0) :!label _label
            (Variables|/Script/Project2016.C_PlayerController|Setc_Inventory (Variables|Default|GetpController_Ref) (Variables|Default|Getc_Slot))
            (Variables|Default|Setc_Slot 0)
            (Rendering|SetVisibility (Variables|Default|GetInsertedObject) false false))))
      (elif (not (!= (Variables|Default|GetpController_Ref) 0))
        (goto _label)))))

(event Input|GamepadEvents|GamepadFaceButtonRight
  (params (Key :type Key%20Structure :default "AnyKey"))
  (bind _pcontroller_ref (Variables|Default|GetpController_Ref))
  (bind _pcontroller_ref_2 (Variables|Default|GetpController_Ref))
  (bind _pcontroller_ref_3 (Variables|Default|GetpController_Ref))
  (:Pressed
    (Variables|/Script/Project2016.C_PlayerController|SetanimationType _pcontroller_ref 2)
    (if (Variables|/Script/Project2016.C_PlayerController|GetcurrentTime _pcontroller_ref)
      (if (!= (Variables|/Script/Project2016.C_PlayerController|Getc_Inventory (Variables|Default|GetpController_Ref)) 0)
        (if (and (== (Utilities|GetClass (Variables|/Script/Project2016.C_PlayerController|Getc_Inventory (Variables|Default|GetpController_Ref))) (Variables|Default|GetacceptedClass)) (== (Variables|Default|Getc_Slot_Berry) 0))
          (Rendering|SetVisibility (Variables|Default|GetInsertedObject) true false)
          (Variables|Default|Setc_Slot (Variables|/Script/Project2016.C_PlayerController|Getc_Inventory _pcontroller_ref_2))
          (Variables|/Script/Project2016.C_PlayerController|Setc_Inventory _pcontroller_ref_2 0)
          (elif (and (== (Utilities|GetClass (Variables|/Script/Project2016.C_PlayerController|Getc_Inventory (Variables|Default|GetpController_Ref))) (Variables|Default|GetacceptedClassBerry)) (== (Variables|Default|Getc_Slot) 0))
            (Rendering|SetVisibility (Variables|Default|GetBerry) true false)
            (Variables|Default|Setc_Slot_Berry (Variables|/Script/Project2016.C_PlayerController|Getc_Inventory _pcontroller_ref_3))
            (Variables|/Script/Project2016.C_PlayerController|Setc_Inventory _pcontroller_ref_3 0)
            (elif (and (== (Utilities|GetClass (Variables|/Script/Project2016.C_PlayerController|Getc_Inventory (Variables|Default|GetpController_Ref))) (Variables|Default|GetacceptedClassStone)) (!= (Variables|Default|Getc_Slot_Berry) 0))
              (Variables|Default|Setc_Slot_Berry 0)
              (Variables|/Script/Project2016.C_PlayerController|Setc_Inventory (Variables|Default|GetpController_Ref) 0)
              (Variables|Default|Setsmashed true)
              (Rendering|SetVisibility (Variables|Default|GetBowlWater) true false)
              (Rendering|SetVisibility (Variables|Default|GetBowl) false false))))
        (else
          (if (!= (Variables|Default|Getc_Slot) 0) :!label _label
            (Variables|/Script/Project2016.C_PlayerController|Setc_Inventory (Variables|Default|GetpController_Ref) (Variables|Default|Getc_Slot))
            (Variables|Default|Setc_Slot 0)
            (Rendering|SetVisibility (Variables|Default|GetInsertedObject) false false))))
      (elif (not (!= (Variables|Default|GetpController_Ref) 0))
        (goto _label)))))

(fn ConstructionScript)
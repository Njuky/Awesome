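; Berry bush quest object for Quest 3 that registers itself as an interaction target when the player is near.
; Entering SphereComponent enables input and sets the bush as the controller's CTempInventory, and leaving reverses both.
; If TimeRelevant is set, both steps require the controller's CurrentTime to match SupposedTime.
; A separate SphereCollision, sized by TriggerRadius in the construction script, toggles custom depth highlighting on the bush meshes.
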(event OnComponentBeginOverlap(SphereComponent)
  (params (OtherActor :type Actor%20Object%20Reference) (OtherComp :type Primitive%20Component%20Object%20Reference) (OtherBodyIndex :type Integer) (bFromSweep :type Boolean) (SweepResult :type Hit%20Result%20Structure%20%28by%20ref%29))
  (bind _returnvalue (Game|GetPlayerController 0))
  ;[0.3254 0.2845 1] B to interact Widget
  (if (== OtherActor (Game|GetPlayerCharacter 0))
    (if (Variables|Default|GettimeRelevant)
      (bind _asbp_controller_2 (Utilities|Casting|CastToBP_Controller2 (Game|GetPlayerController 0)))
      (if (Math|Boolean|Equal(Boolean) (Variables|Default|GetsupposedTime) (Variables|/Script/Project2016.C_PlayerController|GetcurrentTime _asbp_controller_2))
        (Input|EnableInput _returnvalue :!label _label)
        (bind _asbp_controller_2_2 (Utilities|Casting|CastToBP_Controller2 _returnvalue))
        (Variables|/Script/Project2016.C_PlayerController|Setc_TempInventory _asbp_controller_2_2 self))
      (else
        (goto _label)))))

(event OnComponentEndOverlap(SphereComponent)
  (params (OtherActor :type Actor%20Object%20Reference) (OtherComp :type Primitive%20Component%20Object%20Reference) (OtherBodyIndex :type Integer))
  (bind _returnvalue (Game|GetPlayerController 0))
  ;[0.9367 0.342 1] Remove Widget when out of sphere
  (Utilities|Casting|CastToBP_Character OtherActor)
  (if (Variables|Default|GettimeRelevant)
    (bind _asbp_controller_2 (Utilities|Casting|CastToBP_Controller2 (Game|GetPlayerController 0)))
    (if (Math|Boolean|Equal(Boolean) (Variables|Default|GetsupposedTime) (Variables|/Script/Project2016.C_PlayerController|GetcurrentTime _asbp_controller_2))
      (Input|DisableInput _returnvalue :!label _label)
      (bind _asbp_controller_2_2 (Utilities|Casting|CastToBP_Controller2 _returnvalue))
      (Variables|/Script/Project2016.C_PlayerController|Setc_TempInventory _asbp_controller_2_2 0))
    (else
      (goto _label))))

(event OnComponentBeginOverlap(SphereCollision)
  (params (OtherActor :type Actor%20Object%20Reference) (OtherComp :type Primitive%20Component%20Object%20Reference) (OtherBodyIndex :type Integer) (bFromSweep :type Boolean) (SweepResult :type Hit%20Result%20Structure%20%28by%20ref%29))
  (Utilities|Casting|CastToBP_Character OtherActor)
  (Rendering|SetRenderCustomDepth (Variables|Default|GetBerry2) true))

(event OnComponentEndOverlap(SphereCollision)
  (params (OtherActor :type Actor%20Object%20Reference) (OtherComp :type Primitive%20Component%20Object%20Reference) (OtherBodyIndex :type Integer))
  (Utilities|Casting|CastToBP_Character OtherActor)
  (Rendering|SetRenderCustomDepth (Variables|Default|GetBerry2) false))

(fn ConstructionScript
  (Components|Sphere|SetSphereRadius (Variables|Default|GetSphereCollision) (Variables|Default|GetTriggerRadius) true))
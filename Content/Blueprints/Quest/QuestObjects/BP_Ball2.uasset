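; BP_Ball2 is a quest object the player can carry as an inventory item and drop.
; Its sphere overlap toggles input and registers or clears the ball as BP_Controller2's temporary inventory, unless TimeRelevant is set.
; DropItem forwards to every altar, the last flower or the last place according to its flags, otherwise makes the mesh visible, then normally clears the controller's inventory and restores collision.
; The construction script hides the mesh when not Enabled.
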(event OnComponentBeginOverlap(SphereComponent)
  (params (OtherActor :type Actor%20Object%20Reference) (OtherComp :type Primitive%20Component%20Object%20Reference) (OtherBodyIndex :type Integer) (bFromSweep :type Boolean) (SweepResult :type Hit%20Result%20Structure%20%28by%20ref%29))
  (bind _returnvalue (Game|GetPlayerController 0))
  ;[0.3254 0.2845 1] B to interact Widget
  (if (== OtherActor (Game|GetPlayerCharacter 0))
    (if (not (Variables|Default|GettimeRelevant))
      (Input|EnableInput _returnvalue)
      (bind _asbp_controller_2 (Utilities|Casting|CastToBP_Controller2 _returnvalue))
      (Variables|/Script/Project2016.C_PlayerController|Setc_TempInventory _asbp_controller_2 self))))

(event OnComponentEndOverlap(SphereComponent)
  (params (OtherActor :type Actor%20Object%20Reference) (OtherComp :type Primitive%20Component%20Object%20Reference) (OtherBodyIndex :type Integer))
  (bind _returnvalue (Game|GetPlayerController 0))
  ;[0.9367 0.342 1] Remove Widget when out of sphere
  (Utilities|Casting|CastToBP_Character OtherActor)
  (if (not (Variables|Default|GettimeRelevant))
    (Input|DisableInput _returnvalue)
    (bind _asbp_controller_2 (Utilities|Casting|CastToBP_Controller2 _returnvalue))
    (Variables|/Script/Project2016.C_PlayerController|Setc_TempInventory _asbp_controller_2 0)))

(event Custom|DropItem
  (bind _returnvalue (Game|GetPlayerController 0))
  (if (Variables|Default|Getaltar)
    (bind _outactors (Actor|GetAllActorsOfClass "/Game/Blueprints/Quest/QuestObjects/Quest2/BP_Altar.BP_Altar_C"))
    (for _array_element _outactors
      (Default|DropItem _array_element)
      (bind _asbp_controller_2 (Utilities|Casting|CastToBP_Controller2 _returnvalue))
      (Variables|/Script/Project2016.C_PlayerController|Setc_Inventory _asbp_controller_2 0)
      (Input|DisableInput _returnvalue)
      (Collision|SetActorEnableCollision true))
    (else
      (if (Variables|Default|GetFlower_0)
        (Default|DropItem (Variables|Default|GetlastFlower))
        (elif (Variables|Default|GetBowl)
          (Default|DropItem (Variables|Default|GetLastPlace))
          (else
            (Rendering|SetVisibility (Variables|Default|GetStaticMeshComponent) true true)
            (Variables|Default|SetEnabled true))))
      (bind _asbp_controller_2_2 (Utilities|Casting|CastToBP_Controller2 _returnvalue))
      (Variables|/Script/Project2016.C_PlayerController|Setc_Inventory _asbp_controller_2_2 0)
      (Input|DisableInput _returnvalue)
      (Collision|SetActorEnableCollision true))))

(fn ConstructionScript
  (if (not (Variables|Default|GetEnabled))
    (Rendering|SetVisibility (Variables|Default|GetStaticMeshComponent) false true)))
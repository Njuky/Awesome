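; BP_Basic_Tendrils is a quest obstacle with a configurable mesh that is removed once its linked bowls are solved.
; On Tick, only an instance flagged Master gathers each bowl's Solved state, optionally only while BP_Controller's CurrentTime matches SupposedTime.
; When every gathered state is true it destroys all actors in its Tendrils array, otherwise it resets the counter and tries to clear the results.
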(event EventTick
  (params (DeltaSeconds :type Float%20%28single-precision%29))
  (bind _allsolved (Variables|Default|GetAllSolved))
  (bind _allsolved_2 (Variables|Default|GetAllSolved))
  (if (Variables|Default|GetMaster)
    (if (Variables|Default|GetTimeRelevant)
      (if (Math|Boolean|Equal(Boolean) (Variables|Default|GetSupposedTime) (Variables|/Game/Blueprints/Character/Player/BP_Controller.BP_Controller_C|GetCurrentTime (Variables|Default|GetBP_controller)))
        (for (_array_element _array_index) (Variables|Default|GetBowl) :!label _label
          (Utilities|Array|Add (Variables|Default|GetAllSolved) true)
          (if (Variables|/Game/Blueprints/Quest/QuestObjects/BP_Basic_Bowl.BP_Basic_Bowl_C|GetSolved _array_element)
            (Utilities|Array|SetArrayElem _allsolved _array_index true)
            (else
              (Utilities|Array|SetArrayElem _allsolved _array_index false))))
        (for _array_element_2 (Variables|Default|GetAllSolved)
          (if _array_element_2
            (Math|Integer|IncrementInt (Variables|Default|GetDoneIndex))))
        (if (== (Variables|Default|GetDoneIndex) (Utilities|Array|Length (Variables|Default|GetAllSolved)))
          (for _array_element_3 (Variables|Default|GetTendrils)
            (Actor|DestroyActor _array_element_3))
          (else
            (Variables|Default|SetDoneIndex 0)
            (for _array_element_4 _allsolved_2
              (Utilities|Array|RemoveItem _allsolved_2 _array_element_4)))))
      (else
        (goto _label)))))

(event EventBeginPlay
  (bind _asbp_controller (Utilities|Casting|CastToBP_Controller (Game|GetPlayerController 0)))
  (Variables|Default|SetBP_controller _asbp_controller))

(fn ConstructionScript
  (Components|StaticMesh|SetStaticMesh (Variables|Default|GetStaticMesh) (Variables|Default|GetMesh)))
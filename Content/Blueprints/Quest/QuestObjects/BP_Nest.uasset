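; BP_Nest is a quest object that the player can interact with inside a sphere trigger, optionally only in a matching time state.
; Overlap enables its input and registers it as the controller's CTempInventory; leaving reverses both.
; When TimeRelevant is set, CheckTime gates both overlap events by comparing SupposedTime to the controller's CurrentTime.
; While Enabled, Tick sets mesh visibility directly from the boolean CurrentTime.
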(event OnComponentBeginOverlap(SphereComponent)
  (params (OtherActor :type Actor%20Object%20Reference) (OtherComp :type Primitive%20Component%20Object%20Reference) (OtherBodyIndex :type Integer) (bFromSweep :type Boolean) (SweepResult :type Hit%20Result%20Structure%20%28by%20ref%29))
  (bind _returnvalue (Game|GetPlayerController 0))
  ;[0.3254 0.2845 1] B to interact Widget
  (if (== OtherActor (Game|GetPlayerCharacter 0))
    (if (Variables|Default|GettimeRelevant)
      (Utilities|CheckTime
        (:True
          _)))
    (Input|EnableInput _returnvalue)
    (bind _asbp_controller_2 (Utilities|Casting|CastToBP_Controller2 _returnvalue))
    (Variables|/Script/Project2016.C_PlayerController|Setc_TempInventory _asbp_controller_2 self)))

(event OnComponentEndOverlap(SphereComponent)
  (params (OtherActor :type Actor%20Object%20Reference) (OtherComp :type Primitive%20Component%20Object%20Reference) (OtherBodyIndex :type Integer))
  (bind _returnvalue (Game|GetPlayerController 0))
  ;[0.9367 0.342 1] Remove Widget when out of sphere
  (Utilities|Casting|CastToBP_Character OtherActor)
  (if (Variables|Default|GettimeRelevant)
    (Utilities|CheckTime
      (:True
        _)))
  (Input|DisableInput _returnvalue)
  (bind _asbp_controller_2 (Utilities|Casting|CastToBP_Controller2 _returnvalue))
  (Variables|/Script/Project2016.C_PlayerController|Setc_TempInventory _asbp_controller_2 0))

(event EventBeginPlay
  (bind _asbp_controller_2 (Utilities|Casting|CastToBP_Controller2 (Game|GetPlayerController 0)))
  (Variables|Default|SetPController _asbp_controller_2))

(event EventTick
  (params (DeltaSeconds :type Float%20%28single-precision%29))
  (if (Variables|Default|Getenabled)
    (Rendering|SetVisibility (Variables|Default|GetStaticMeshComponent) (Variables|/Script/Project2016.C_PlayerController|GetcurrentTime (Variables|Default|GetPController)) false)))

(fn ConstructionScript)
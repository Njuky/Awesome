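; BP_Ball is a Quest2 pickup item that the player carries in the BP_Controller inventory and can place at altars or flowers.
; An overlap sphere enables interact input, which picks up an intact ball or repairs a broken "Verzweiflung" ball by consuming a held BP_Schnecke.
; A delayed Tick swaps intact and broken meshes, and toggles disabled "Hass" balls by CurrentTime and placement.
; DropItem forwards to altars or the last flower, otherwise reshows the ball.
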(event OnComponentBeginOverlap(Sphere1)
  (params (OtherActor :type Actor%20Object%20Reference) (OtherComp :type Primitive%20Component%20Object%20Reference) (OtherBodyIndex :type Integer) (bFromSweep :type Boolean) (SweepResult :type Hit%20Result%20Structure%20%28by%20ref%29))
  (Utilities|Casting|CastToBP_Character OtherActor)
  (Input|EnableInput (Game|GetPlayerController 0)))

(event OnComponentEndOverlap(Sphere1)
  (params (OtherActor :type Actor%20Object%20Reference) (OtherComp :type Primitive%20Component%20Object%20Reference) (OtherBodyIndex :type Integer))
  (Utilities|Casting|CastToBP_Character OtherActor)
  (Input|DisableInput (Game|GetPlayerController 0)))

(event EventTick
  (params (DeltaSeconds :type Float%20%28single-precision%29))
  (bind _brokenball (Variables|Default|GetBrokenBall))
  (bind _sphere (Variables|Default|GetSphere))
  (bind _defaultsceneroot (Variables|Default|GetDefaultSceneRoot))
  (Utilities|FlowControl|Delay 0.2)
  (if (Variables|Default|GetEnabled)
    (if (Variables|Default|GetBroken)
      (Rendering|SetVisibility _brokenball true false)
      (Rendering|SetVisibility _sphere false false)
      (else
        (Rendering|SetVisibility _brokenball false false)
        (Rendering|SetVisibility _sphere true false)))
    (elif (Actor|ActorHasTag "Hass")
      (bind _asbp_controller (Utilities|Casting|CastToBP_Controller (Game|GetPlayerController 0)))
      (if (!= (Variables|/Game/Blueprints/Character/Player/BP_Controller.BP_Controller_C|GetInventory _asbp_controller) 0)
        (if (not (Actor|ActorHasTag (Variables|/Game/Blueprints/Character/Player/BP_Controller.BP_Controller_C|GetInventory _asbp_controller) "Hass"))
          (if (Math|Boolean|ANDBoolean (not (Variables|Default|GetAltar)) (not (Variables|Default|GetFlower)) (Variables|/Game/Blueprints/Character/Player/BP_Controller.BP_Controller_C|GetCurrentTime _asbp_controller)) :!label _label
            (Rendering|SetVisibility _defaultsceneroot true true)
            (Variables|Default|SetEnabled true)
            (Collision|SetActorEnableCollision true)
            (else
              (Rendering|SetVisibility _defaultsceneroot false true)
              (Variables|Default|SetEnabled false)
              (Collision|SetActorEnableCollision false))))
        (else
          (goto _label))))))

(event EventDropItem
  (bind _returnvalue (Game|GetPlayerController 0))
  (if (Variables|Default|GetAltar)
    (bind _outactors (Actor|GetAllActorsOfClass "/Game/Blueprints/Quest/QuestObjects/Quest2/BP_Altar.BP_Altar_C"))
    (for _array_element _outactors
      (Default|DropItem _array_element)
      (bind _asbp_controller (Utilities|Casting|CastToBP_Controller _returnvalue))
      (Variables|/Game/Blueprints/Character/Player/BP_Controller.BP_Controller_C|SetInventory _asbp_controller 0)
      (Input|DisableInput _returnvalue)
      (Collision|SetActorEnableCollision true))
    (else
      (if (Variables|Default|GetFlower)
        (Default|DropItem (Variables|Default|GetlastFlower))
        (else
          (Rendering|SetVisibility (Variables|Default|GetDefaultSceneRoot) true true)
          (Variables|Default|SetEnabled true)))
      (bind _asbp_controller_2 (Utilities|Casting|CastToBP_Controller _returnvalue))
      (Variables|/Game/Blueprints/Character/Player/BP_Controller.BP_Controller_C|SetInventory _asbp_controller_2 0)
      (Input|DisableInput _returnvalue)
      (Collision|SetActorEnableCollision true))))

(event Input|KeyboardEvents|F
  (params (Key :type Key%20Structure :default "AnyKey"))
  (:Pressed
    (if (Variables|Default|GetEnabled)
      (bind _asbp_controller (Utilities|Casting|CastToBP_Controller (Game|GetPlayerController 0)))
      (if (Variables|Default|GetBroken)
        (if (and (== (Utilities|GetClass (Variables|/Game/Blueprints/Character/Player/BP_Controller.BP_Controller_C|GetInventory _asbp_controller)) "/Game/Blueprints/Quest/QuestObjects/Quest2/BP_Schnecke.BP_Schnecke_C") (Actor|ActorHasTag "Verzweiflung"))
          (Variables|Default|SetBroken false)
          (Actor|DestroyActor (Variables|/Game/Blueprints/Character/Player/BP_Controller.BP_Controller_C|GetInventory _asbp_controller))
          (Variables|/Game/Blueprints/Character/Player/BP_Controller.BP_Controller_C|SetInventory _asbp_controller 0))
        (elif (== (Variables|/Game/Blueprints/Character/Player/BP_Controller.BP_Controller_C|GetInventory _asbp_controller) 0)
          (Rendering|SetVisibility (Variables|Default|GetDefaultSceneRoot) false true)
          (Variables|/Game/Blueprints/Character/Player/BP_Controller.BP_Controller_C|SetInventory _asbp_controller self)
          (Variables|Default|SetEnabled false)
          (Collision|SetActorEnableCollision false))))))

(event Input|GamepadEvents|GamepadFaceButtonRight
  (params (Key :type Key%20Structure :default "AnyKey"))
  (:Pressed
    (if (Variables|Default|GetEnabled)
      (bind _asbp_controller (Utilities|Casting|CastToBP_Controller (Game|GetPlayerController 0)))
      (if (Variables|Default|GetBroken)
        (if (and (== (Utilities|GetClass (Variables|/Game/Blueprints/Character/Player/BP_Controller.BP_Controller_C|GetInventory _asbp_controller)) "/Game/Blueprints/Quest/QuestObjects/Quest2/BP_Schnecke.BP_Schnecke_C") (Actor|ActorHasTag "Verzweiflung"))
          (Variables|Default|SetBroken false)
          (Actor|DestroyActor (Variables|/Game/Blueprints/Character/Player/BP_Controller.BP_Controller_C|GetInventory _asbp_controller))
          (Variables|/Game/Blueprints/Character/Player/BP_Controller.BP_Controller_C|SetInventory _asbp_controller 0))
        (elif (== (Variables|/Game/Blueprints/Character/Player/BP_Controller.BP_Controller_C|GetInventory _asbp_controller) 0)
          (Rendering|SetVisibility (Variables|Default|GetDefaultSceneRoot) false true)
          (Variables|/Game/Blueprints/Character/Player/BP_Controller.BP_Controller_C|SetInventory _asbp_controller self)
          (Variables|Default|SetEnabled false)
          (Collision|SetActorEnableCollision false))))))

(fn ConstructionScript
  (Rendering|Components|TextRender|SetText (Variables|Default|GetTextRender) (Variables|Default|Gettext))
  (if (not (Variables|Default|GetEnabled))
    (Rendering|SetVisibility (Variables|Default|GetDefaultSceneRoot) false true)))
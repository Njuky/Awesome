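; BP_BranchRadius is a Quest 2 interaction zone where the player uses a branch from the inventory.
; Its sphere enables input while BP_Character overlaps it and disables input when the character leaves.
; Pressing F or the right gamepad face button checks that the controller's inventory item is a BP_Branch.
; It then destroys the "before" reference actor, enables the "after" one and clears the inventory.
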(event OnComponentBeginOverlap(Sphere)
  (params (OtherActor :type Actor%20Object%20Reference) (OtherComp :type Primitive%20Component%20Object%20Reference) (OtherBodyIndex :type Integer) (bFromSweep :type Boolean) (SweepResult :type Hit%20Result%20Structure%20%28by%20ref%29))
  (Utilities|Casting|CastToBP_Character OtherActor)
  (Input|EnableInput (Game|GetPlayerController 0)))

(event OnComponentEndOverlap(Sphere)
  (params (OtherActor :type Actor%20Object%20Reference) (OtherComp :type Primitive%20Component%20Object%20Reference) (OtherBodyIndex :type Integer))
  (Utilities|Casting|CastToBP_Character OtherActor)
  (Input|DisableInput (Game|GetPlayerController 0)))

(event EventBeginPlay
  (bind _asbp_controller_2 (Utilities|Casting|CastToBP_Controller2 (Game|GetPlayerController 0)))
  (Variables|Default|SetBP_ControllerRef _asbp_controller_2))

(event Input|KeyboardEvents|F
  (params (Key :type Key%20Structure :default "AnyKey"))
  (:Pressed
    (if (== (Utilities|GetClass (Variables|/Game/Blueprints/Character/Player/BP_Controller2.BP_Controller2_C|GetInventory (Variables|Default|GetBP_ControllerRef))) "/Game/Blueprints/Quest/QuestObjects/Quest2/BP_Branch.BP_Branch_C")
      (Actor|DestroyActor (Variables|Default|GetSupposedBallRef_Before))
      (Variables|/Script/Project2016.BaseCollectable|Setenabled (Variables|Default|GetSupposedBallRef_After) true)
      (Variables|/Game/Blueprints/Character/Player/BP_Controller2.BP_Controller2_C|SetInventory (Variables|Default|GetBP_ControllerRef) 0))))

(event Input|GamepadEvents|GamepadFaceButtonRight
  (params (Key :type Key%20Structure :default "AnyKey"))
  (:Pressed
    (if (== (Utilities|GetClass (Variables|/Game/Blueprints/Character/Player/BP_Controller2.BP_Controller2_C|GetInventory (Variables|Default|GetBP_ControllerRef))) "/Game/Blueprints/Quest/QuestObjects/Quest2/BP_Branch.BP_Branch_C")
      (Actor|DestroyActor (Variables|Default|GetSupposedBallRef_Before))
      (Variables|/Script/Project2016.BaseCollectable|Setenabled (Variables|Default|GetSupposedBallRef_After) true)
      (Variables|/Game/Blueprints/Character/Player/BP_Controller2.BP_Controller2_C|SetInventory (Variables|Default|GetBP_ControllerRef) 0))))

(fn ConstructionScript)
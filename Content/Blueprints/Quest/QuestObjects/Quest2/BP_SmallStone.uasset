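; BP_SmallStone is a Quest 2 object, a small stone the player can pick up.
; Its Box overlap enables input while a BP_Character is inside and disables it on exit.
; Pressing F or the gamepad right face button, when the BP_Controller2 Inventory slot is empty, hides the stone, turns off its collision, stores it in that slot and clears its Enabled flag.
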(event OnComponentBeginOverlap(Box)
  (params (OtherActor :type Actor%20Object%20Reference) (OtherComp :type Primitive%20Component%20Object%20Reference) (OtherBodyIndex :type Integer) (bFromSweep :type Boolean) (SweepResult :type Hit%20Result%20Structure%20%28by%20ref%29))
  (Utilities|Casting|CastToBP_Character OtherActor)
  (Input|EnableInput (Game|GetPlayerController 0)))

(event OnComponentEndOverlap(Box)
  (params (OtherActor :type Actor%20Object%20Reference) (OtherComp :type Primitive%20Component%20Object%20Reference) (OtherBodyIndex :type Integer))
  (Utilities|Casting|CastToBP_Character OtherActor)
  (Input|DisableInput (Game|GetPlayerController 0)))

(event Input|GamepadEvents|GamepadFaceButtonRight
  (params (Key :type Key%20Structure :default "AnyKey"))
  (:Pressed
    (bind _asbp_controller_2 (Utilities|Casting|CastToBP_Controller2 (Game|GetPlayerController 0)))
    (if (== (Variables|/Game/Blueprints/Character/Player/BP_Controller2.BP_Controller2_C|GetInventory _asbp_controller_2) 0)
      (Rendering|SetVisibility (Variables|Default|GetCapsuleComponent) false true)
      (Collision|SetActorEnableCollision false)
      (Variables|/Game/Blueprints/Character/Player/BP_Controller2.BP_Controller2_C|SetInventory _asbp_controller_2 self)
      (Variables|Default|Setenabled false))))

(event Input|KeyboardEvents|F
  (params (Key :type Key%20Structure :default "AnyKey"))
  (:Pressed
    (bind _asbp_controller_2 (Utilities|Casting|CastToBP_Controller2 (Game|GetPlayerController 0)))
    (if (== (Variables|/Game/Blueprints/Character/Player/BP_Controller2.BP_Controller2_C|GetInventory _asbp_controller_2) 0)
      (Rendering|SetVisibility (Variables|Default|GetCapsuleComponent) false true)
      (Collision|SetActorEnableCollision false)
      (Variables|/Game/Blueprints/Character/Player/BP_Controller2.BP_Controller2_C|SetInventory _asbp_controller_2 self)
      (Variables|Default|Setenabled false))))

(fn ConstructionScript
  (|CallParentFunction))
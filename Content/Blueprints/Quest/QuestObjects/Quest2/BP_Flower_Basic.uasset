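; Quest 2 flower bowl that stores one emotion ball, swapped with the controller's inventory on interact while the player overlaps its box.
; Tag-matched meshes show the held emotion; taken balls record their source flower.
; "Broken" variants poll the controller's time state, appearing broken until fixed with cloth, or intact and refilled with their designated ball if it is unplaced and uncarried.
; Bowl-less "Nest" variants accept a nest item to reveal the bowl mesh.
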(event OnComponentBeginOverlap(Box)
  (params (OtherActor :type Actor%20Object%20Reference) (OtherComp :type Primitive%20Component%20Object%20Reference) (OtherBodyIndex :type Integer) (bFromSweep :type Boolean) (SweepResult :type Hit%20Result%20Structure%20%28by%20ref%29))
  (Utilities|Casting|CastToBP_Character OtherActor)
  (Input|EnableInput (Game|GetPlayerController 0)))

(event OnComponentEndOverlap(Box)
  (params (OtherActor :type Actor%20Object%20Reference) (OtherComp :type Primitive%20Component%20Object%20Reference) (OtherBodyIndex :type Integer))
  (Utilities|Casting|CastToBP_Character OtherActor)
  (Input|DisableInput (Game|GetPlayerController 0)))

(event Custom|DropItem
  (bind _asbp_controller (Utilities|Casting|CastToBP_Controller (Game|GetPlayerController 0)))
  (if (Variables|Default|GetBowl)
    (if (== (Utilities|GetClass (Variables|/Game/Blueprints/Character/Player/BP_Controller.BP_Controller_C|GetInventory _asbp_controller)) "/Game/Blueprints/Quest/QuestObjects/Quest2/BP_Ball.BP_Ball_C")
      (if (== (Variables|Default|GetSlot) 0)
        (if (Actor|ActorHasTag "Broken")
          (if (Actor|ActorHasTag "Hass")
            (Rendering|SetVisibility (Variables|Default|GetHass) true false)
            (Variables|Default|SetSlot (Variables|/Game/Blueprints/Character/Player/BP_Controller.BP_Controller_C|GetInventory _asbp_controller))
            (Variables|/Game/Blueprints/Character/Player/BP_Controller.BP_Controller_C|SetInventory _asbp_controller 0))
          (elif (Actor|ActorHasTag (Variables|/Game/Blueprints/Character/Player/BP_Controller.BP_Controller_C|GetInventory _asbp_controller) "Angst")
            (Rendering|SetVisibility (Variables|Default|GetAngst) true false)
            (Variables|Default|SetSlot (Variables|/Game/Blueprints/Character/Player/BP_Controller.BP_Controller_C|GetInventory _asbp_controller))
            (Variables|/Game/Blueprints/Character/Player/BP_Controller.BP_Controller_C|SetInventory _asbp_controller 0 :!label _label)
            (elif (Actor|ActorHasTag (Variables|/Game/Blueprints/Character/Player/BP_Controller.BP_Controller_C|GetInventory _asbp_controller) "Hass")
              (Rendering|SetVisibility (Variables|Default|GetHass) true false)
              (Variables|Default|SetSlot (Variables|/Game/Blueprints/Character/Player/BP_Controller.BP_Controller_C|GetInventory _asbp_controller))
              (goto _label)
              (elif (Actor|ActorHasTag (Variables|/Game/Blueprints/Character/Player/BP_Controller.BP_Controller_C|GetInventory _asbp_controller) "Wut")
                (Rendering|SetVisibility (Variables|Default|GetWoot) true false)
                (Variables|Default|SetSlot (Variables|/Game/Blueprints/Character/Player/BP_Controller.BP_Controller_C|GetInventory _asbp_controller))
                (goto _label)
                (elif (Actor|ActorHasTag (Variables|/Game/Blueprints/Character/Player/BP_Controller.BP_Controller_C|GetInventory _asbp_controller) "Verzweiflung")
                  (Rendering|SetVisibility (Variables|Default|GetVerzweiflung) true false)
                  (Variables|Default|SetSlot (Variables|/Game/Blueprints/Character/Player/BP_Controller.BP_Controller_C|GetInventory _asbp_controller))
                  (goto _label)
                  (elif (Actor|ActorHasTag (Variables|/Game/Blueprints/Character/Player/BP_Controller.BP_Controller_C|GetInventory _asbp_controller) "Trauer")
                    (Rendering|SetVisibility (Variables|Default|GetTrauer) true false)
                    (Variables|Default|SetSlot (Variables|/Game/Blueprints/Character/Player/BP_Controller.BP_Controller_C|GetInventory _asbp_controller))
                    (goto _label))))))))
      (elif (== (Variables|/Game/Blueprints/Character/Player/BP_Controller.BP_Controller_C|GetInventory _asbp_controller) 0)
        (if (Variables|/Script/Engine.SceneComponent|GetbVisible (Variables|Default|GetAngst))
          (CallFunction|TakeBall (Variables|Default|GetAngst))
          (bind _asbp_ball (Utilities|Casting|CastToBP_Ball (Variables|/Game/Blueprints/Character/Player/BP_Controller.BP_Controller_C|GetInventory _asbp_controller) :!label _label_2))
          (Variables|/Game/Blueprints/Quest/QuestObjects/Quest2/BP_Ball.BP_Ball_C|SetFlower _asbp_ball true)
          (Variables|/Game/Blueprints/Quest/QuestObjects/Quest2/BP_Ball.BP_Ball_C|SetAltar _asbp_ball false)
          (Variables|/Game/Blueprints/Quest/QuestObjects/Quest2/BP_Ball.BP_Ball_C|SetlastFlower _asbp_ball self)
          (elif (Variables|/Script/Engine.SceneComponent|GetbVisible (Variables|Default|GetHass))
            (CallFunction|TakeBall (Variables|Default|GetHass))
            (goto _label_2)
            (elif (Variables|/Script/Engine.SceneComponent|GetbVisible (Variables|Default|GetWoot))
              (CallFunction|TakeBall (Variables|Default|GetWoot))
              (goto _label_2)
              (elif (Variables|/Script/Engine.SceneComponent|GetbVisible (Variables|Default|GetVerzweiflung))
                (CallFunction|TakeBall (Variables|Default|GetVerzweiflung))
                (goto _label_2)
                (elif (Variables|/Script/Engine.SceneComponent|GetbVisible (Variables|Default|GetTrauer))
                  (CallFunction|TakeBall (Variables|Default|GetTrauer))
                  (goto _label_2))))))))
    (elif (Actor|ActorHasTag "Nest")
      (if (== (Utilities|GetClass (Variables|/Game/Blueprints/Character/Player/BP_Controller.BP_Controller_C|GetInventory _asbp_controller)) "/Game/Blueprints/Quest/QuestObjects/Quest2/BP_Nest.BP_Nest_C")
        (Rendering|SetVisibility (Variables|Default|GetBowl_Mesh) true false)
        (Variables|/Game/Blueprints/Character/Player/BP_Controller.BP_Controller_C|SetInventory _asbp_controller 0))
      (elif (and (Actor|ActorHasTag "Broken") (Variables|/Game/Blueprints/Character/Player/BP_Controller.BP_Controller_C|GetCurrentTime _asbp_controller))
        (if (== (Utilities|GetClass (Variables|/Game/Blueprints/Character/Player/BP_Controller.BP_Controller_C|GetInventory _asbp_controller)) "/Game/Blueprints/Quest/QuestObjects/Quest2/BP_Cloth.BP_Cloth_C")
          (Rendering|SetVisibility (Variables|Default|GetBowl_Mesh) true false)
          (Variables|/Game/Blueprints/Character/Player/BP_Controller.BP_Controller_C|SetInventory _asbp_controller 0)
          (Variables|Default|SetFixed true)
          (Variables|Default|SetBowl true))))))

(event EventTick
  (params (DeltaSeconds :type Float%20%28single-precision%29))
  (bind _bowl_broken (Variables|Default|GetBowl_Broken))
  (bind _bowl_mesh (Variables|Default|GetBowl_Mesh))
  (bind _suposedball (Variables|Default|GetSuposedBall))
  (Utilities|FlowControl|Delay 0.2)
  (if (Actor|ActorHasTag "Broken")
    (bind _asbp_controller (Utilities|Casting|CastToBP_Controller (Game|GetPlayerController 0)))
    (if (and (Variables|/Game/Blueprints/Character/Player/BP_Controller.BP_Controller_C|GetCurrentTime _asbp_controller) (not (Variables|Default|GetFixed)))
      (Variables|Default|SetBowl false)
      (Rendering|SetVisibility _bowl_broken true false)
      (Rendering|SetVisibility _bowl_mesh false false)
      (else
        (Variables|Default|SetBowl true)
        (Rendering|SetVisibility _bowl_broken false false)
        (Rendering|SetVisibility _bowl_mesh true false)
        (if (Math|Boolean|ANDBoolean (== (Variables|Default|GetSlot) 0) (not (Variables|/Game/Blueprints/Quest/QuestObjects/Quest2/BP_Ball.BP_Ball_C|GetAltar _suposedball)) (not (Variables|/Game/Blueprints/Quest/QuestObjects/Quest2/BP_Ball.BP_Ball_C|GetFlower _suposedball)) (!= (Variables|/Game/Blueprints/Character/Player/BP_Controller.BP_Controller_C|GetInventory _asbp_controller) (Variables|Default|GetSuposedBall)))
          (Variables|Default|SetSlot (Variables|Default|GetSuposedBall))
          (Rendering|SetVisibility (Variables|Default|GetHass) true false)
          (Variables|/Game/Blueprints/Objects/Collectible/BP_BaseCollectable.BP_BaseCollectable_C|SetEnabled (Variables|Default|GetSuposedBall) false))))))

(event Input|GamepadEvents|GamepadFaceButtonBottom
  (params (Key :type Key%20Structure :default "AnyKey"))
  (:Pressed
    (bind _asbp_controller (Utilities|Casting|CastToBP_Controller (Game|GetPlayerController 0)))
    (if (Variables|Default|GetBowl)
      (if (== (Utilities|GetClass (Variables|/Game/Blueprints/Character/Player/BP_Controller.BP_Controller_C|GetInventory _asbp_controller)) "/Game/Blueprints/Quest/QuestObjects/Quest2/BP_Ball.BP_Ball_C")
        (if (== (Variables|Default|GetSlot) 0)
          (if (Actor|ActorHasTag "Broken")
            (if (Actor|ActorHasTag "Hass")
              (Rendering|SetVisibility (Variables|Default|GetHass) true false)
              (Variables|Default|SetSlot (Variables|/Game/Blueprints/Character/Player/BP_Controller.BP_Controller_C|GetInventory _asbp_controller))
              (Variables|/Game/Blueprints/Character/Player/BP_Controller.BP_Controller_C|SetInventory _asbp_controller 0))
            (elif (Actor|ActorHasTag (Variables|/Game/Blueprints/Character/Player/BP_Controller.BP_Controller_C|GetInventory _asbp_controller) "Angst")
              (Rendering|SetVisibility (Variables|Default|GetAngst) true false)
              (Variables|Default|SetSlot (Variables|/Game/Blueprints/Character/Player/BP_Controller.BP_Controller_C|GetInventory _asbp_controller))
              (Variables|/Game/Blueprints/Character/Player/BP_Controller.BP_Controller_C|SetInventory _asbp_controller 0 :!label _label)
              (elif (Actor|ActorHasTag (Variables|/Game/Blueprints/Character/Player/BP_Controller.BP_Controller_C|GetInventory _asbp_controller) "Hass")
                (Rendering|SetVisibility (Variables|Default|GetHass) true false)
                (Variables|Default|SetSlot (Variables|/Game/Blueprints/Character/Player/BP_Controller.BP_Controller_C|GetInventory _asbp_controller))
                (goto _label)
                (elif (Actor|ActorHasTag (Variables|/Game/Blueprints/Character/Player/BP_Controller.BP_Controller_C|GetInventory _asbp_controller) "Wut")
                  (Rendering|SetVisibility (Variables|Default|GetWoot) true false)
                  (Variables|Default|SetSlot (Variables|/Game/Blueprints/Character/Player/BP_Controller.BP_Controller_C|GetInventory _asbp_controller))
                  (goto _label)
                  (elif (Actor|ActorHasTag (Variables|/Game/Blueprints/Character/Player/BP_Controller.BP_Controller_C|GetInventory _asbp_controller) "Verzweiflung")
                    (Rendering|SetVisibility (Variables|Default|GetVerzweiflung) true false)
                    (Variables|Default|SetSlot (Variables|/Game/Blueprints/Character/Player/BP_Controller.BP_Controller_C|GetInventory _asbp_controller))
                    (goto _label)
                    (elif (Actor|ActorHasTag (Variables|/Game/Blueprints/Character/Player/BP_Controller.BP_Controller_C|GetInventory _asbp_controller) "Trauer")
                      (Rendering|SetVisibility (Variables|Default|GetTrauer) true false)
                      (Variables|Default|SetSlot (Variables|/Game/Blueprints/Character/Player/BP_Controller.BP_Controller_C|GetInventory _asbp_controller))
                      (goto _label))))))))
        (elif (== (Variables|/Game/Blueprints/Character/Player/BP_Controller.BP_Controller_C|GetInventory _asbp_controller) 0)
          (if (Variables|/Script/Engine.SceneComponent|GetbVisible (Variables|Default|GetAngst))
            (CallFunction|TakeBall (Variables|Default|GetAngst))
            (bind _asbp_ball (Utilities|Casting|CastToBP_Ball (Variables|/Game/Blueprints/Character/Player/BP_Controller.BP_Controller_C|GetInventory _asbp_controller) :!label _label_2))
            (Variables|/Game/Blueprints/Quest/QuestObjects/Quest2/BP_Ball.BP_Ball_C|SetFlower _asbp_ball true)
            (Variables|/Game/Blueprints/Quest/QuestObjects/Quest2/BP_Ball.BP_Ball_C|SetAltar _asbp_ball false)
            (Variables|/Game/Blueprints/Quest/QuestObjects/Quest2/BP_Ball.BP_Ball_C|SetlastFlower _asbp_ball self)
            (elif (Variables|/Script/Engine.SceneComponent|GetbVisible (Variables|Default|GetHass))
              (CallFunction|TakeBall (Variables|Default|GetHass))
              (goto _label_2)
              (elif (Variables|/Script/Engine.SceneComponent|GetbVisible (Variables|Default|GetWoot))
                (CallFunction|TakeBall (Variables|Default|GetWoot))
                (goto _label_2)
                (elif (Variables|/Script/Engine.SceneComponent|GetbVisible (Variables|Default|GetVerzweiflung))
                  (CallFunction|TakeBall (Variables|Default|GetVerzweiflung))
                  (goto _label_2)
                  (elif (Variables|/Script/Engine.SceneComponent|GetbVisible (Variables|Default|GetTrauer))
                    (CallFunction|TakeBall (Variables|Default|GetTrauer))
                    (goto _label_2))))))))
      (elif (Actor|ActorHasTag "Nest")
        (if (== (Utilities|GetClass (Variables|/Game/Blueprints/Character/Player/BP_Controller.BP_Controller_C|GetInventory _asbp_controller)) "/Game/Blueprints/Quest/QuestObjects/Quest2/BP_Nest.BP_Nest_C")
          (Rendering|SetVisibility (Variables|Default|GetBowl_Mesh) true false)
          (Variables|/Game/Blueprints/Character/Player/BP_Controller.BP_Controller_C|SetInventory _asbp_controller 0))
        (elif (and (Actor|ActorHasTag "Broken") (Variables|/Game/Blueprints/Character/Player/BP_Controller.BP_Controller_C|GetCurrentTime _asbp_controller))
          (if (== (Utilities|GetClass (Variables|/Game/Blueprints/Character/Player/BP_Controller.BP_Controller_C|GetInventory _asbp_controller)) "/Game/Blueprints/Quest/QuestObjects/Quest2/BP_Cloth.BP_Cloth_C")
            (Rendering|SetVisibility (Variables|Default|GetBowl_Mesh) true false)
            (Variables|/Game/Blueprints/Character/Player/BP_Controller.BP_Controller_C|SetInventory _asbp_controller 0)
            (Variables|Default|SetFixed true)
            (Variables|Default|SetBowl true)))))))

(event Input|KeyboardEvents|F
  (params (Key :type Key%20Structure :default "AnyKey"))
  (:Pressed
    (bind _asbp_controller (Utilities|Casting|CastToBP_Controller (Game|GetPlayerController 0)))
    (if (Variables|Default|GetBowl)
      (if (== (Utilities|GetClass (Variables|/Game/Blueprints/Character/Player/BP_Controller.BP_Controller_C|GetInventory _asbp_controller)) "/Game/Blueprints/Quest/QuestObjects/Quest2/BP_Ball.BP_Ball_C")
        (if (== (Variables|Default|GetSlot) 0)
          (if (Actor|ActorHasTag "Broken")
            (if (Actor|ActorHasTag "Hass")
              (Rendering|SetVisibility (Variables|Default|GetHass) true false)
              (Variables|Default|SetSlot (Variables|/Game/Blueprints/Character/Player/BP_Controller.BP_Controller_C|GetInventory _asbp_controller))
              (Variables|/Game/Blueprints/Character/Player/BP_Controller.BP_Controller_C|SetInventory _asbp_controller 0))
            (elif (Actor|ActorHasTag (Variables|/Game/Blueprints/Character/Player/BP_Controller.BP_Controller_C|GetInventory _asbp_controller) "Angst")
              (Rendering|SetVisibility (Variables|Default|GetAngst) true false)
              (Variables|Default|SetSlot (Variables|/Game/Blueprints/Character/Player/BP_Controller.BP_Controller_C|GetInventory _asbp_controller))
              (Variables|/Game/Blueprints/Character/Player/BP_Controller.BP_Controller_C|SetInventory _asbp_controller 0 :!label _label)
              (elif (Actor|ActorHasTag (Variables|/Game/Blueprints/Character/Player/BP_Controller.BP_Controller_C|GetInventory _asbp_controller) "Hass")
                (Rendering|SetVisibility (Variables|Default|GetHass) true false)
                (Variables|Default|SetSlot (Variables|/Game/Blueprints/Character/Player/BP_Controller.BP_Controller_C|GetInventory _asbp_controller))
                (goto _label)
                (elif (Actor|ActorHasTag (Variables|/Game/Blueprints/Character/Player/BP_Controller.BP_Controller_C|GetInventory _asbp_controller) "Wut")
                  (Rendering|SetVisibility (Variables|Default|GetWoot) true false)
                  (Variables|Default|SetSlot (Variables|/Game/Blueprints/Character/Player/BP_Controller.BP_Controller_C|GetInventory _asbp_controller))
                  (goto _label)
                  (elif (Actor|ActorHasTag (Variables|/Game/Blueprints/Character/Player/BP_Controller.BP_Controller_C|GetInventory _asbp_controller) "Verzweiflung")
                    (Rendering|SetVisibility (Variables|Default|GetVerzweiflung) true false)
                    (Variables|Default|SetSlot (Variables|/Game/Blueprints/Character/Player/BP_Controller.BP_Controller_C|GetInventory _asbp_controller))
                    (goto _label)
                    (elif (Actor|ActorHasTag (Variables|/Game/Blueprints/Character/Player/BP_Controller.BP_Controller_C|GetInventory _asbp_controller) "Trauer")
                      (Rendering|SetVisibility (Variables|Default|GetTrauer) true false)
                      (Variables|Default|SetSlot (Variables|/Game/Blueprints/Character/Player/BP_Controller.BP_Controller_C|GetInventory _asbp_controller))
                      (goto _label))))))))
        (elif (== (Variables|/Game/Blueprints/Character/Player/BP_Controller.BP_Controller_C|GetInventory _asbp_controller) 0)
          (if (Variables|/Script/Engine.SceneComponent|GetbVisible (Variables|Default|GetAngst))
            (CallFunction|TakeBall (Variables|Default|GetAngst))
            (bind _asbp_ball (Utilities|Casting|CastToBP_Ball (Variables|/Game/Blueprints/Character/Player/BP_Controller.BP_Controller_C|GetInventory _asbp_controller) :!label _label_2))
            (Variables|/Game/Blueprints/Quest/QuestObjects/Quest2/BP_Ball.BP_Ball_C|SetFlower _asbp_ball true)
            (Variables|/Game/Blueprints/Quest/QuestObjects/Quest2/BP_Ball.BP_Ball_C|SetAltar _asbp_ball false)
            (Variables|/Game/Blueprints/Quest/QuestObjects/Quest2/BP_Ball.BP_Ball_C|SetlastFlower _asbp_ball self)
            (elif (Variables|/Script/Engine.SceneComponent|GetbVisible (Variables|Default|GetHass))
              (CallFunction|TakeBall (Variables|Default|GetHass))
              (goto _label_2)
              (elif (Variables|/Script/Engine.SceneComponent|GetbVisible (Variables|Default|GetWoot))
                (CallFunction|TakeBall (Variables|Default|GetWoot))
                (goto _label_2)
                (elif (Variables|/Script/Engine.SceneComponent|GetbVisible (Variables|Default|GetVerzweiflung))
                  (CallFunction|TakeBall (Variables|Default|GetVerzweiflung))
                  (goto _label_2)
                  (elif (Variables|/Script/Engine.SceneComponent|GetbVisible (Variables|Default|GetTrauer))
                    (CallFunction|TakeBall (Variables|Default|GetTrauer))
                    (goto _label_2))))))))
      (elif (Actor|ActorHasTag "Nest")
        (if (== (Utilities|GetClass (Variables|/Game/Blueprints/Character/Player/BP_Controller.BP_Controller_C|GetInventory _asbp_controller)) "/Game/Blueprints/Quest/QuestObjects/Quest2/BP_Nest.BP_Nest_C")
          (Rendering|SetVisibility (Variables|Default|GetBowl_Mesh) true false)
          (Variables|/Game/Blueprints/Character/Player/BP_Controller.BP_Controller_C|SetInventory _asbp_controller 0))
        (elif (and (Actor|ActorHasTag "Broken") (Variables|/Game/Blueprints/Character/Player/BP_Controller.BP_Controller_C|GetCurrentTime _asbp_controller))
          (if (== (Utilities|GetClass (Variables|/Game/Blueprints/Character/Player/BP_Controller.BP_Controller_C|GetInventory _asbp_controller)) "/Game/Blueprints/Quest/QuestObjects/Quest2/BP_Cloth.BP_Cloth_C")
            (Rendering|SetVisibility (Variables|Default|GetBowl_Mesh) true false)
            (Variables|/Game/Blueprints/Character/Player/BP_Controller.BP_Controller_C|SetInventory _asbp_controller 0)
            (Variables|Default|SetFixed true)
            (Variables|Default|SetBowl true)))))))

(fn ConstructionScript
  (Rendering|Components|TextRender|SetText (Variables|Default|GetTextRender) (Variables|Default|GetNewVar_0))
  (Components|StaticMesh|SetStaticMesh (Variables|Default|GetBowl_Mesh) (Variables|Default|GetBowl_Ref))
  (Development|PrintString "BP_Flower_Basic ->Construction"))

(fn TakeBall
  (params (Ball :type Static%20Mesh%20Component%20Object%20Reference))
  (bind _asbp_controller (Utilities|Casting|CastToBP_Controller (Game|GetPlayerController 0)))
  (Variables|/Game/Blueprints/Character/Player/BP_Controller.BP_Controller_C|SetInventory _asbp_controller (Variables|Default|GetSlot))
  (Variables|Default|SetSlot 0)
  (Rendering|SetVisibility Ball false false))
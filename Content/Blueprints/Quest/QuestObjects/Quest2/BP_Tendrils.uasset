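; BP_Tendrils is a Quest 2 object that clears tendril actors once the flower puzzle is solved.
; Only the actor tagged Master runs the check, on a Tick throttled by a short Delay and gated by the player controller's CurrentTime flag.
; It copies each Flower's Solved state into an array, counts leading solved entries, and at five destroys every actor in Tendrils, with a debug print standing in for effects.
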(event EventTick
  (params (DeltaSeconds :type Float%20%28single-precision%29))
  (Utilities|FlowControl|Delay 0.2)
  (if (Actor|ActorHasTag "Master")
    (bind _asbp_controller (Utilities|Casting|CastToBP_Controller (Game|GetPlayerController 0)))
    (if (Variables|/Game/Blueprints/Character/Player/BP_Controller.BP_Controller_C|GetCurrentTime _asbp_controller)
      (for (_array_element _array_index) (Variables|Default|GetFlower)
        (if (Variables|/Game/Blueprints/Quest/QuestObjects/Quest2/BP_Flower_Basic.BP_Flower_Basic_C|GetSolved _array_element)
          (Utilities|Array|SetArrayElem (Variables|Default|GetSolved) _array_index true)
          (else
            (Utilities|Array|SetArrayElem (Variables|Default|GetSolved) _array_index false))))
      (bind _array_element_2 (Utilities|Array|ForEachLoopwithBreak (Variables|Default|GetSolved) :!label _label)
        (:LoopBody
          (if _array_element_2
            (Math|Integer|IncrementInt (Variables|Default|GetDoneIndex))
            (else
              (goto _label Break))))
        (:Completed
          (if (== (Variables|Default|GetDoneIndex) 5)
            (Variables|Default|SetDoneIndex 0)
            (for _array_element_3 (Variables|Default|GetTendrils)
              (Development|PrintString "Do fancy stuff")
              (Actor|DestroyActor _array_element_3))
            (else
              (Variables|Default|SetDoneIndex 0))))))))

(fn ConstructionScript)
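; BP_Tree is a quest tree whose nest and red ball change with the controller's CurrentTime state.
; Tick watches for time switches and toggles the ball's visibility.
; Inventory, bowl and altar checks select one of four nest/ball mesh variants and its animation.
; When CurrentTime is true, it plays any matching fall animation and hides the nest mesh after a delay; otherwise it shows the mesh.
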(event EventBeginPlay
  (bind _skm_nest (Variables|Default|GetSKM_Nest))
  (bind _skm_nest_2 (Variables|Default|GetSKM_Nest))
  (bind _asbp_controller (Utilities|Casting|CastToBP_Controller (Game|GetPlayerController 0)))
  (Variables|Default|SetPController _asbp_controller)
  (if (Variables|/Script/Project2016.C_PlayerController|GetcurrentTime (Variables|Default|GetPController))
    (CallFunction|CheckCondition)
    (switch int (Variables|Default|Getanimation)
      (:0
        (Components|Animation|PlayAnimation _skm_nest_2 "/Game/Art/Animation/Objects/A_Nest_Falling.A_Nest_Falling" false))
      (:1
        (Components|Animation|PlayAnimation _skm_nest_2 "/Game/Art/Animation/Objects/A_Nest_ohneKugel.A_Nest_ohneKugel" false))
      (:2
        (Components|Animation|PlayAnimation _skm_nest_2 "/Game/Art/Animation/Objects/A_Kugel_ohne_Nest.A_Kugel_ohne_Nest" false))
      (:3
        _))
    (Utilities|FlowControl|Delay 1.0)
    (Rendering|SetVisibility (Variables|Default|GetSKM_Nest) false false)
    (else
      (CallFunction|CheckCondition)
      (Components|Animation|PlayAnimation _skm_nest 0 false)
      (Rendering|SetVisibility _skm_nest true false))))

(event EventTick
  (params (DeltaSeconds :type Float%20%28single-precision%29))
  (bind _skm_nest (Variables|Default|GetSKM_Nest))
  (bind _redballref (Variables|Default|GetRedBallRef))
  (bind _skm_nest_2 (Variables|Default|GetSKM_Nest))
  (bind _returnvalue (VehicleSound|GetRootComponent _redballref))
  (if (not (Math|Boolean|Equal(Boolean) (Variables|/Script/Project2016.C_PlayerController|GetcurrentTime (Variables|Default|GetPController)) (Variables|Default|GetoldTime)))
    (Variables|Default|SetoldTime (Variables|/Script/Project2016.C_PlayerController|GetcurrentTime (Variables|Default|GetPController)))
    (bind _condition (CallFunction|CheckBallCondition))
    (if (Math|Boolean|ANDBoolean _condition (Variables|/Script/Project2016.BaseCollectable|Getm_enabled (Variables|Default|GetRedBallRef)) (Variables|/Script/Project2016.C_PlayerController|GetcurrentTime (Variables|Default|GetPController)))
      (Rendering|SetVisibility _returnvalue true true)
      (else
        (Rendering|SetVisibility _returnvalue false true)))
    (if (Variables|/Script/Project2016.C_PlayerController|GetcurrentTime (Variables|Default|GetPController))
      (CallFunction|CheckCondition)
      (switch int (Variables|Default|Getanimation)
        (:0
          (Components|Animation|PlayAnimation _skm_nest_2 "/Game/Art/Animation/Objects/A_Nest_Falling.A_Nest_Falling" false))
        (:1
          (Components|Animation|PlayAnimation _skm_nest_2 "/Game/Art/Animation/Objects/A_Nest_ohneKugel.A_Nest_ohneKugel" false))
        (:2
          (Components|Animation|PlayAnimation _skm_nest_2 "/Game/Art/Animation/Objects/A_Kugel_ohne_Nest.A_Kugel_ohne_Nest" false))
        (:3
          _))
      (Utilities|FlowControl|Delay 1.0)
      (Rendering|SetVisibility (Variables|Default|GetSKM_Nest) false false)
      (else
        (CallFunction|CheckCondition)
        (Components|Animation|PlayAnimation _skm_nest 0 false)
        (Rendering|SetVisibility _skm_nest true false)))))

(fn ConstructionScript)

(fn CheckNestCondition
  (return (and (not (Variables|/Script/Project2016.C_Bowl|GetbowlExist (Variables|Default|GetBowl))) (!= (Variables|/Script/Project2016.C_PlayerController|Getc_Inventory (Variables|Default|GetPController)) (Variables|Default|GetNestRef)))))

(fn CheckBallCondition
  (return (Math|Boolean|ANDBoolean (!= (Variables|/Script/Project2016.C_PlayerController|Getc_Inventory (Variables|Default|GetPController)) (Variables|Default|GetRedBallRef)) (!= (Variables|/Script/Project2016.C_Bowl|Getc_slot (Variables|Default|GetBowl1)) (Variables|Default|GetRedBallRef)) (!= (Variables|/Script/Project2016.C_Bowl|Getc_slot (Variables|Default|GetBowl3)) (Variables|Default|GetRedBallRef)) (!= (Variables|Default|GetAltar) (Variables|Default|GetRedBallRef)))))

(fn CheckCondition
  (bind _skm_nest (Variables|Default|GetSKM_Nest))
  (bind _condition (CallFunction|CheckNestCondition))
  (if _condition
    ;[1 1 1] Nest Exist
    (bind _condition_2 (CallFunction|CheckBallCondition))
    (if _condition_2
      (Class|SkinnedMeshComponent|SetSkeletalMesh _skm_nest "/Game/Art/Meshes/Skeletal/Tree/SKM_Tree_Nest.SKM_Tree_Nest" true)
      (Variables|Default|Setanimation 0)
      (else
        (Class|SkinnedMeshComponent|SetSkeletalMesh _skm_nest "/Game/Art/Meshes/Skeletal/Tree/SKM_Nest_ohneKugel.SKM_Nest_ohneKugel" true)
        (Variables|Default|Setanimation 1)))
    (else
      ;[1 1 1] Nest don't exist
      (bind _condition_3 (CallFunction|CheckBallCondition))
      (if _condition_3
        (Class|SkinnedMeshComponent|SetSkeletalMesh (Variables|Default|GetSKM_Nest) "/Game/Art/Meshes/Skeletal/Tree/SKM_Tree_ohne_Nest.SKM_Tree_ohne_Nest" true)
        (Variables|Default|Setanimation 2)
        (else
          (Class|SkinnedMeshComponent|SetSkeletalMesh (Variables|Default|GetSKM_Nest) 0 true)
          (Variables|Default|Setanimation 3))))))
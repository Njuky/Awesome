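; BP_Cloth is a cloth pickup for Quest 2 that the player collects by interacting.
; Its sphere overlap with BP_Character toggles input, so F or the right gamepad face button works only nearby.
; A press conditionally stores the cloth in BP_Controller2's CInventory slot, plays a pickup sound at world origin and clears Enabled.
; Tick polls Enabled and hides the capsule and its children when false, without destroying the actor.
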(event OnComponentBeginOverlap(Sphere1)
  (params (OtherActor :type Actor%20Object%20Reference) (OtherComp :type Primitive%20Component%20Object%20Reference) (OtherBodyIndex :type Integer) (bFromSweep :type Boolean) (SweepResult :type Hit%20Result%20Structure%20%28by%20ref%29))
  ;[0.3254 0.2845 1] B to interact Widget
  (Utilities|Casting|CastToBP_Character OtherActor)
  (Input|EnableInput (Game|GetPlayerController 0)))

(event OnComponentEndOverlap(Sphere1)
  (params (OtherActor :type Actor%20Object%20Reference) (OtherComp :type Primitive%20Component%20Object%20Reference) (OtherBodyIndex :type Integer))
  ;[0.9367 0.342 1] Remove Widget when out of sphere
  (Utilities|Casting|CastToBP_Character OtherActor)
  (Input|DisableInput (Game|GetPlayerController 0)))

(event EventTick
  (params (DeltaSeconds :type Float%20%28single-precision%29))
  (if (not (Variables|Default|Getenabled))
    (Rendering|SetVisibility (Variables|Default|GetCapsuleComponent) false true)))

(event Input|KeyboardEvents|F
  (params (Key :type Key%20Structure :default "AnyKey"))
  (:Pressed
    (bind _asbp_controller_2 (Utilities|Casting|CastToBP_Controller2 (Game|GetPlayerController 0)))
    (if (== (Variables|/Script/Project2016.C_PlayerController|Getc_Inventory _asbp_controller_2) 0)
      (Variables|/Script/Project2016.C_PlayerController|Setc_Inventory _asbp_controller_2 self)
      (Audio|PlaySoundatLocation "/Game/Audio/Sound/Platzhalter_Itemaufheben.Platzhalter_Itemaufheben" "0, 0, 0")
      (Variables|Default|Setenabled false))))

(event Input|GamepadEvents|GamepadFaceButtonRight
  (params (Key :type Key%20Structure :default "AnyKey"))
  (:Pressed
    (bind _asbp_controller_2 (Utilities|Casting|CastToBP_Controller2 (Game|GetPlayerController 0)))
    (if (== (Variables|/Script/Project2016.C_PlayerController|Getc_Inventory _asbp_controller_2) 0)
      (Variables|/Script/Project2016.C_PlayerController|Setc_Inventory _asbp_controller_2 self)
      (Audio|PlaySoundatLocation "/Game/Audio/Sound/Platzhalter_Itemaufheben.Platzhalter_Itemaufheben" "0, 0, 0")
      (Variables|Default|Setenabled false))))

(fn ConstructionScript
  (|CallParentFunction))
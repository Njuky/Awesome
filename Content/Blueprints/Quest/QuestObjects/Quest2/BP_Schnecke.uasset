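; BP_Schnecke is a pickup quest object (a snail, per its name) for Quest2.
; Overlapping its box with BP_Character enables player input on the actor, and leaving disables it.
; Pressing F or the gamepad right face button while enabled stores the actor in BP_Controller's single Inventory slot if empty, hiding it and turning off collision and overlaps.
; The construction script fills its text render from the Text variable.
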(event OnComponentBeginOverlap(Box)
  (params (OtherActor :type Actor%20Object%20Reference) (OtherComp :type Primitive%20Component%20Object%20Reference) (OtherBodyIndex :type Integer) (bFromSweep :type Boolean) (SweepResult :type Hit%20Result%20Structure%20%28by%20ref%29))
  (Utilities|Casting|CastToBP_Character OtherActor)
  (Input|EnableInput (Game|GetPlayerController 0)))

(event OnComponentEndOverlap(Box)
  (params (OtherActor :type Actor%20Object%20Reference) (OtherComp :type Primitive%20Component%20Object%20Reference) (OtherBodyIndex :type Integer))
  (Utilities|Casting|CastToBP_Character OtherActor)
  (Input|DisableInput (Game|GetPlayerController 0)))

(event Input|KeyboardEvents|F
  (params (Key :type Key%20Structure :default "AnyKey"))
  (:Pressed
    (if (Variables|Default|GetEnabled)
      (bind _asbp_controller (Utilities|Casting|CastToBP_Controller (Game|GetPlayerController 0)))
      (if (== (Variables|/Game/Blueprints/Character/Player/BP_Controller.BP_Controller_C|GetInventory _asbp_controller) 0)
        (Rendering|SetVisibility (Variables|Default|GetDefaultSceneRoot) false true)
        (Variables|/Game/Blueprints/Character/Player/BP_Controller.BP_Controller_C|SetInventory _asbp_controller self)
        (Variables|Default|SetEnabled false)
        (Rendering|SetVisibility (Variables|Default|GetObject_Mesh) false false)
        (Collision|SetActorEnableCollision false)
        (Variables|/Script/Engine.PrimitiveComponent|SetbGenerateOverlapEvents (Variables|Default|GetBox) false)))))

(event Input|GamepadEvents|GamepadFaceButtonRight
  (params (Key :type Key%20Structure :default "AnyKey"))
  (:Pressed
    (if (Variables|Default|GetEnabled)
      (bind _asbp_controller (Utilities|Casting|CastToBP_Controller (Game|GetPlayerController 0)))
      (if (== (Variables|/Game/Blueprints/Character/Player/BP_Controller.BP_Controller_C|GetInventory _asbp_controller) 0)
        (Rendering|SetVisibility (Variables|Default|GetDefaultSceneRoot) false true)
        (Variables|/Game/Blueprints/Character/Player/BP_Controller.BP_Controller_C|SetInventory _asbp_controller self)
        (Variables|Default|SetEnabled false)
        (Rendering|SetVisibility (Variables|Default|GetObject_Mesh) false false)
        (Collision|SetActorEnableCollision false)
        (Variables|/Script/Engine.PrimitiveComponent|SetbGenerateOverlapEvents (Variables|Default|GetBox) false)))))

(fn ConstructionScript
  (Rendering|Components|TextRender|SetText (Variables|Default|GetTextRender) (Variables|Default|Gettext)))
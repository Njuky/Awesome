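; Quest 2 altar actor where the player places and takes back LightBlue, Pink and Red balls.
; Per-color overlap boxes enable input for the character; F or gamepad right face button then moves balls between the controller's inventory and three slots, toggling display components.
; Placement follows the ball's tag; pickup requires standing in that color's box and sets the ball's origin flags.
; Tick also drives Nest egg visibility from CurrentTime and Dropped.
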(event OnComponentBeginOverlap(B_LightBlue)
  (params (OtherActor :type Actor%20Object%20Reference) (OtherComp :type Primitive%20Component%20Object%20Reference) (OtherBodyIndex :type Integer) (bFromSweep :type Boolean) (SweepResult :type Hit%20Result%20Structure%20%28by%20ref%29))
  ;[1 1 1] Enable/Disable input
  (CallFunction|Enable OtherActor)
  (Variables|Default|SetPlace1 true))

(event OnComponentEndOverlap(B_LightBlue)
  (params (OtherActor :type Actor%20Object%20Reference) (OtherComp :type Primitive%20Component%20Object%20Reference) (OtherBodyIndex :type Integer))
  ;[1 1 1] Enable/Disable input
  (CallFunction|Disable OtherActor)
  (Variables|Default|SetPlace1 false))

(event OnComponentBeginOverlap(B_Pink)
  (params (OtherActor :type Actor%20Object%20Reference) (OtherComp :type Primitive%20Component%20Object%20Reference) (OtherBodyIndex :type Integer) (bFromSweep :type Boolean) (SweepResult :type Hit%20Result%20Structure%20%28by%20ref%29))
  ;[1 1 1] Enable/Disable input
  (CallFunction|Enable OtherActor)
  (Variables|Default|SetPlace2 true))

(event OnComponentEndOverlap(B_Pink)
  (params (OtherActor :type Actor%20Object%20Reference) (OtherComp :type Primitive%20Component%20Object%20Reference) (OtherBodyIndex :type Integer))
  ;[1 1 1] Enable/Disable input
  (CallFunction|Disable OtherActor)
  (Variables|Default|SetPlace2 false))

(event OnComponentBeginOverlap(B_Red)
  (params (OtherActor :type Actor%20Object%20Reference) (OtherComp :type Primitive%20Component%20Object%20Reference) (OtherBodyIndex :type Integer) (bFromSweep :type Boolean) (SweepResult :type Hit%20Result%20Structure%20%28by%20ref%29))
  ;[1 1 1] Enable/Disable input
  (CallFunction|Enable OtherActor)
  (Variables|Default|SetPlace3 true))

(event OnComponentEndOverlap(B_Red)
  (params (OtherActor :type Actor%20Object%20Reference) (OtherComp :type Primitive%20Component%20Object%20Reference) (OtherBodyIndex :type Integer))
  ;[1 1 1] Enable/Disable input
  (CallFunction|Disable OtherActor)
  (Variables|Default|SetPlace3 false))

(event Custom|DropItem
  ;[1 1 1] Start Place/Take
  (if (== (Variables|/Game/Blueprints/Character/Player/BP_Controller2.BP_Controller2_C|GetInventory (Variables|Default|GetBP_Controller_Ref)) 0)
    ;[1 1 1] Take ball
    (if (== (Variables|/Game/Blueprints/Character/Player/BP_Controller2.BP_Controller2_C|GetInventory (Variables|Default|GetBP_Controller_Ref)) 0)
      (if (and (Variables|/Script/Engine.SceneComponent|GetbVisible (Variables|Default|GetLightBlue)) (Variables|Default|GetPlace1))
        (Variables|/Game/Blueprints/Character/Player/BP_Controller2.BP_Controller2_C|SetInventory (Variables|Default|GetBP_Controller_Ref) (Variables|Default|GetSlot1))
        (Variables|Default|SetSlot1 0)
        (Rendering|SetVisibility (Variables|Default|GetLightBlue) false false)
        (bind _asbp_ball (Utilities|Casting|CastToBP_Ball (Variables|/Game/Blueprints/Character/Player/BP_Controller2.BP_Controller2_C|GetInventory (Variables|Default|GetBP_Controller_Ref)) :!label _label))
        (Variables|/Script/Project2016.BaseCollectable|Setaltar _asbp_ball true)
        (Variables|/Game/Blueprints/Quest/QuestObjects/BP_Ball.BP_Ball_C|SetFlower_0 _asbp_ball false)
        (Variables|/Script/Project2016.BaseCollectable|Setbowl _asbp_ball false)
        (elif (and (Variables|/Script/Engine.SceneComponent|GetbVisible (Variables|Default|GetPink)) (Variables|Default|GetPlace2))
          (Variables|/Game/Blueprints/Character/Player/BP_Controller2.BP_Controller2_C|SetInventory (Variables|Default|GetBP_Controller_Ref) (Variables|Default|GetSlot2))
          (Variables|Default|SetSlot2 0)
          (Rendering|SetVisibility (Variables|Default|GetPink) false false)
          (goto _label)
          (elif (and (Variables|/Script/Engine.SceneComponent|GetbVisible (Variables|Default|GetRed)) (Variables|Default|GetPlace3))
            (Variables|/Game/Blueprints/Character/Player/BP_Controller2.BP_Controller2_C|SetInventory (Variables|Default|GetBP_Controller_Ref) (Variables|Default|GetSlot3))
            (Variables|Default|SetSlot3 0)
            (Rendering|SetVisibility (Variables|Default|GetRed) false false)
            (goto _label)))))
    (else
      ;[1 1 1] Place Ball
      (if (== (Utilities|GetClass (Variables|/Game/Blueprints/Character/Player/BP_Controller2.BP_Controller2_C|GetInventory (Variables|Default|GetBP_Controller_Ref))) "/Game/Blueprints/Quest/QuestObjects/BP_Ball.BP_Ball_C")
        (if (Actor|ActorHasTag (Variables|/Game/Blueprints/Character/Player/BP_Controller2.BP_Controller2_C|GetInventory (Variables|Default|GetBP_Controller_Ref)) "LightBlue")
          (Rendering|SetVisibility (Variables|Default|GetLightBlue) true false)
          (Variables|Default|SetSlot1 (Variables|/Game/Blueprints/Character/Player/BP_Controller2.BP_Controller2_C|GetInventory (Variables|Default|GetBP_Controller_Ref)))
          (Variables|/Game/Blueprints/Character/Player/BP_Controller2.BP_Controller2_C|SetInventory (Variables|Default|GetBP_Controller_Ref) 0 :!label _label_2)
          (elif (Actor|ActorHasTag (Variables|/Game/Blueprints/Character/Player/BP_Controller2.BP_Controller2_C|GetInventory (Variables|Default|GetBP_Controller_Ref)) "Pink")
            (Rendering|SetVisibility (Variables|Default|GetPink) true false)
            (Variables|Default|SetSlot2 (Variables|/Game/Blueprints/Character/Player/BP_Controller2.BP_Controller2_C|GetInventory (Variables|Default|GetBP_Controller_Ref)))
            (goto _label_2)
            (elif (Actor|ActorHasTag (Variables|/Game/Blueprints/Character/Player/BP_Controller2.BP_Controller2_C|GetInventory (Variables|Default|GetBP_Controller_Ref)) "Red")
              (Rendering|SetVisibility (Variables|Default|GetRed) true false)
              (Variables|Default|SetSlot3 (Variables|/Game/Blueprints/Character/Player/BP_Controller2.BP_Controller2_C|GetInventory (Variables|Default|GetBP_Controller_Ref)))
              (goto _label_2))))))))

(event EventTick
  (params (DeltaSeconds :type Float%20%28single-precision%29))
  (bind _nest (Variables|Default|GetNest))
  (bind _eier (Variables|/Game/Blueprints/Quest/QuestObjects/Quest2/BP_Nest.BP_Nest_C|GetEier _nest))
  (if (Variables|/Script/Project2016.C_PlayerController|GetcurrentTime (Variables|Default|GetBP_Controller_Ref))
    (Rendering|SetVisibility _eier false false :!label _label)
    (elif (Variables|/Game/Blueprints/Quest/QuestObjects/Quest2/BP_Nest.BP_Nest_C|GetDropped (Variables|Default|GetNest))
      (goto _label)
      (else
        (Rendering|SetVisibility _eier true false)))))

(event EventBeginPlay
  (bind _asbp_controller_2 (Utilities|Casting|CastToBP_Controller2 (Game|GetPlayerController 0)))
  (Variables|Default|SetBP_Controller_Ref _asbp_controller_2))

(event Input|GamepadEvents|GamepadFaceButtonRight
  (params (Key :type Key%20Structure :default "AnyKey"))
  ;[1 1 1] Start Place/Take
  (:Pressed
    (if (== (Variables|/Game/Blueprints/Character/Player/BP_Controller2.BP_Controller2_C|GetInventory (Variables|Default|GetBP_Controller_Ref)) 0)
      ;[1 1 1] Take ball
      (if (== (Variables|/Game/Blueprints/Character/Player/BP_Controller2.BP_Controller2_C|GetInventory (Variables|Default|GetBP_Controller_Ref)) 0)
        (if (and (Variables|/Script/Engine.SceneComponent|GetbVisible (Variables|Default|GetLightBlue)) (Variables|Default|GetPlace1))
          (Variables|/Game/Blueprints/Character/Player/BP_Controller2.BP_Controller2_C|SetInventory (Variables|Default|GetBP_Controller_Ref) (Variables|Default|GetSlot1))
          (Variables|Default|SetSlot1 0)
          (Rendering|SetVisibility (Variables|Default|GetLightBlue) false false)
          (bind _asbp_ball (Utilities|Casting|CastToBP_Ball (Variables|/Game/Blueprints/Character/Player/BP_Controller2.BP_Controller2_C|GetInventory (Variables|Default|GetBP_Controller_Ref)) :!label _label))
          (Variables|/Script/Project2016.BaseCollectable|Setaltar _asbp_ball true)
          (Variables|/Game/Blueprints/Quest/QuestObjects/BP_Ball.BP_Ball_C|SetFlower_0 _asbp_ball false)
          (Variables|/Script/Project2016.BaseCollectable|Setbowl _asbp_ball false)
          (elif (and (Variables|/Script/Engine.SceneComponent|GetbVisible (Variables|Default|GetPink)) (Variables|Default|GetPlace2))
            (Variables|/Game/Blueprints/Character/Player/BP_Controller2.BP_Controller2_C|SetInventory (Variables|Default|GetBP_Controller_Ref) (Variables|Default|GetSlot2))
            (Variables|Default|SetSlot2 0)
            (Rendering|SetVisibility (Variables|Default|GetPink) false false)
            (goto _label)
            (elif (and (Variables|/Script/Engine.SceneComponent|GetbVisible (Variables|Default|GetRed)) (Variables|Default|GetPlace3))
              (Variables|/Game/Blueprints/Character/Player/BP_Controller2.BP_Controller2_C|SetInventory (Variables|Default|GetBP_Controller_Ref) (Variables|Default|GetSlot3))
              (Variables|Default|SetSlot3 0)
              (Rendering|SetVisibility (Variables|Default|GetRed) false false)
              (goto _label)))))
      (else
        ;[1 1 1] Place Ball
        (if (== (Utilities|GetClass (Variables|/Game/Blueprints/Character/Player/BP_Controller2.BP_Controller2_C|GetInventory (Variables|Default|GetBP_Controller_Ref))) "/Game/Blueprints/Quest/QuestObjects/BP_Ball.BP_Ball_C")
          (if (Actor|ActorHasTag (Variables|/Game/Blueprints/Character/Player/BP_Controller2.BP_Controller2_C|GetInventory (Variables|Default|GetBP_Controller_Ref)) "LightBlue")
            (Rendering|SetVisibility (Variables|Default|GetLightBlue) true false)
            (Variables|Default|SetSlot1 (Variables|/Game/Blueprints/Character/Player/BP_Controller2.BP_Controller2_C|GetInventory (Variables|Default|GetBP_Controller_Ref)))
            (Variables|/Game/Blueprints/Character/Player/BP_Controller2.BP_Controller2_C|SetInventory (Variables|Default|GetBP_Controller_Ref) 0 :!label _label_2)
            (elif (Actor|ActorHasTag (Variables|/Game/Blueprints/Character/Player/BP_Controller2.BP_Controller2_C|GetInventory (Variables|Default|GetBP_Controller_Ref)) "Pink")
              (Rendering|SetVisibility (Variables|Default|GetPink) true false)
              (Variables|Default|SetSlot2 (Variables|/Game/Blueprints/Character/Player/BP_Controller2.BP_Controller2_C|GetInventory (Variables|Default|GetBP_Controller_Ref)))
              (goto _label_2)
              (elif (Actor|ActorHasTag (Variables|/Game/Blueprints/Character/Player/BP_Controller2.BP_Controller2_C|GetInventory (Variables|Default|GetBP_Controller_Ref)) "Red")
                (Rendering|SetVisibility (Variables|Default|GetRed) true false)
                (Variables|Default|SetSlot3 (Variables|/Game/Blueprints/Character/Player/BP_Controller2.BP_Controller2_C|GetInventory (Variables|Default|GetBP_Controller_Ref)))
                (goto _label_2)))))))))

(event Input|KeyboardEvents|F
  (params (Key :type Key%20Structure :default "AnyKey"))
  ;[1 1 1] Start Place/Take
  (:Pressed
    (if (== (Variables|/Game/Blueprints/Character/Player/BP_Controller2.BP_Controller2_C|GetInventory (Variables|Default|GetBP_Controller_Ref)) 0)
      ;[1 1 1] Take ball
      (if (== (Variables|/Game/Blueprints/Character/Player/BP_Controller2.BP_Controller2_C|GetInventory (Variables|Default|GetBP_Controller_Ref)) 0)
        (if (and (Variables|/Script/Engine.SceneComponent|GetbVisible (Variables|Default|GetLightBlue)) (Variables|Default|GetPlace1))
          (Variables|/Game/Blueprints/Character/Player/BP_Controller2.BP_Controller2_C|SetInventory (Variables|Default|GetBP_Controller_Ref) (Variables|Default|GetSlot1))
          (Variables|Default|SetSlot1 0)
          (Rendering|SetVisibility (Variables|Default|GetLightBlue) false false)
          (bind _asbp_ball (Utilities|Casting|CastToBP_Ball (Variables|/Game/Blueprints/Character/Player/BP_Controller2.BP_Controller2_C|GetInventory (Variables|Default|GetBP_Controller_Ref)) :!label _label))
          (Variables|/Script/Project2016.BaseCollectable|Setaltar _asbp_ball true)
          (Variables|/Game/Blueprints/Quest/QuestObjects/BP_Ball.BP_Ball_C|SetFlower_0 _asbp_ball false)
          (Variables|/Script/Project2016.BaseCollectable|Setbowl _asbp_ball false)
          (elif (and (Variables|/Script/Engine.SceneComponent|GetbVisible (Variables|Default|GetPink)) (Variables|Default|GetPlace2))
            (Variables|/Game/Blueprints/Character/Player/BP_Controller2.BP_Controller2_C|SetInventory (Variables|Default|GetBP_Controller_Ref) (Variables|Default|GetSlot2))
            (Variables|Default|SetSlot2 0)
            (Rendering|SetVisibility (Variables|Default|GetPink) false false)
            (goto _label)
            (elif (and (Variables|/Script/Engine.SceneComponent|GetbVisible (Variables|Default|GetRed)) (Variables|Default|GetPlace3))
              (Variables|/Game/Blueprints/Character/Player/BP_Controller2.BP_Controller2_C|SetInventory (Variables|Default|GetBP_Controller_Ref) (Variables|Default|GetSlot3))
              (Variables|Default|SetSlot3 0)
              (Rendering|SetVisibility (Variables|Default|GetRed) false false)
              (goto _label)))))
      (else
        ;[1 1 1] Place Ball
        (if (== (Utilities|GetClass (Variables|/Game/Blueprints/Character/Player/BP_Controller2.BP_Controller2_C|GetInventory (Variables|Default|GetBP_Controller_Ref))) "/Game/Blueprints/Quest/QuestObjects/BP_Ball.BP_Ball_C")
          (if (Actor|ActorHasTag (Variables|/Game/Blueprints/Character/Player/BP_Controller2.BP_Controller2_C|GetInventory (Variables|Default|GetBP_Controller_Ref)) "LightBlue")
            (Rendering|SetVisibility (Variables|Default|GetLightBlue) true false)
            (Variables|Default|SetSlot1 (Variables|/Game/Blueprints/Character/Player/BP_Controller2.BP_Controller2_C|GetInventory (Variables|Default|GetBP_Controller_Ref)))
            (Variables|/Game/Blueprints/Character/Player/BP_Controller2.BP_Controller2_C|SetInventory (Variables|Default|GetBP_Controller_Ref) 0 :!label _label_2)
            (elif (Actor|ActorHasTag (Variables|/Game/Blueprints/Character/Player/BP_Controller2.BP_Controller2_C|GetInventory (Variables|Default|GetBP_Controller_Ref)) "Pink")
              (Rendering|SetVisibility (Variables|Default|GetPink) true false)
              (Variables|Default|SetSlot2 (Variables|/Game/Blueprints/Character/Player/BP_Controller2.BP_Controller2_C|GetInventory (Variables|Default|GetBP_Controller_Ref)))
              (goto _label_2)
              (elif (Actor|ActorHasTag (Variables|/Game/Blueprints/Character/Player/BP_Controller2.BP_Controller2_C|GetInventory (Variables|Default|GetBP_Controller_Ref)) "Red")
                (Rendering|SetVisibility (Variables|Default|GetRed) true false)
                (Variables|Default|SetSlot3 (Variables|/Game/Blueprints/Character/Player/BP_Controller2.BP_Controller2_C|GetInventory (Variables|Default|GetBP_Controller_Ref)))
                (goto _label_2)))))))))

(fn ConstructionScript)

(fn Enable
  (params (Actor :type Actor%20Object%20Reference))
  (Utilities|Casting|CastToBP_Character Actor)
  (Input|EnableInput (Game|GetPlayerController 0)))

(fn Disable
  (params (Actor :type Actor%20Object%20Reference))
  (Utilities|Casting|CastToBP_Character Actor)
  (Input|DisableInput (Game|GetPlayerController 0)))
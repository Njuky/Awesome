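; BP_Tree is a quest object tree whose nest, eggs and ball toggle visibility with the player controller's CurrentTime state.
; BeginPlay caches the BP_Controller2 reference.
; Every Tick shows the nest and eggs only while CurrentTime is false.
; The ball follows the same rule, but stops updating while RedBallRef's Bowl is set or that ball is the controller's CInventory item.
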(event EventBeginPlay
  (bind _asbp_controller_2 (Utilities|Casting|CastToBP_Controller2 (Game|GetPlayerController 0)))
  (Variables|Default|SetPController _asbp_controller_2))

(event EventTick
  (params (DeltaSeconds :type Float%20%28single-precision%29))
  (bind _pcontroller (Variables|Default|GetPController))
  (bind _currenttime (Variables|/Script/Project2016.C_PlayerController|GetcurrentTime _pcontroller))
  (bind _returnvalue (not _currenttime))
  (Rendering|SetVisibility (Variables|Default|GetSM_Nest) _returnvalue false)
  (if (and (not (Variables|/Script/Project2016.BaseCollectable|Getbowl (Variables|Default|GetRedBallRef))) (!= (Variables|/Script/Project2016.C_PlayerController|Getc_Inventory (Variables|Default|GetPController)) (Variables|Default|GetRedBallRef)))
    (Rendering|SetVisibility (Variables|Default|GetSM_Ball) _returnvalue false)))

(fn ConstructionScript)
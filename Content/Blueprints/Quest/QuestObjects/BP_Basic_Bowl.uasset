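; BP_Basic_Bowl is a quest puzzle bowl that holds one collectable and sets Solved when that item's tag matches its expected ball tag.
; Within the sphere overlap, F or gamepad input swaps items with the player controller's single inventory slot, accepting only the expected class.
; A broken bowl first consumes a repair item, with Tick toggling whole and broken meshes.
; The construction script previews preset contents and warns about unset tags.
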(event OnComponentBeginOverlap(Sphere_Collision)
  (params (OtherActor :type Actor%20Object%20Reference) (OtherComp :type Primitive%20Component%20Object%20Reference) (OtherBodyIndex :type Integer) (bFromSweep :type Boolean) (SweepResult :type Hit%20Result%20Structure%20%28by%20ref%29))
  (Utilities|Casting|CastToBP_Character OtherActor)
  (Input|EnableInput (Game|GetPlayerController 0)))

(event OnComponentEndOverlap(Sphere_Collision)
  (params (OtherActor :type Actor%20Object%20Reference) (OtherComp :type Primitive%20Component%20Object%20Reference) (OtherBodyIndex :type Integer))
  (Utilities|Casting|CastToBP_Character OtherActor)
  (Input|DisableInput (Game|GetPlayerController 0)))

(event Custom|DropItem
  (bind _bp_controller_ref (Variables|Default|GetBP_Controller_Ref))
  (bind _inserted_object (Variables|Default|GetInserted_Object))
  (bind _bp_controller_ref_2 (Variables|Default|GetBP_Controller_Ref))
  (if (Variables|Default|GetBowl)
    (if (!= (Variables|/Script/Project2016.C_PlayerController|Getc_Inventory (Variables|Default|GetBP_Controller_Ref)) 0) ; Check Inventory empty
      (if (== (Utilities|GetClass (Variables|/Script/Project2016.C_PlayerController|Getc_Inventory (Variables|Default|GetBP_Controller_Ref))) (Variables|Default|GetSupposedObjectCLASS)) ; Check Inventory supposed Itemclass
        (if (== (Variables|Default|GetSlot) 0) ; Check Slot empty
          (Rendering|SetVisibility (Variables|Default|GetInserted_Object) true false)
          (Components|StaticMesh|SetStaticMesh _inserted_object (Variables|/Script/Engine.StaticMeshComponent|GetStaticMesh (Variables|/Script/Project2016.BaseCollectable|GetStaticMeshComponent (Variables|/Script/Project2016.C_PlayerController|Getc_Inventory (Variables|Default|GetBP_Controller_Ref)))))
          (Rendering|Material|SetMaterial _inserted_object 0 (Rendering|Material|GetMaterial (Variables|/Script/Project2016.BaseCollectable|GetStaticMeshComponent (Variables|/Script/Project2016.C_PlayerController|Getc_Inventory (Variables|Default|GetBP_Controller_Ref))) 0))
          (bind _asbp_base_collectable (Utilities|Casting|CastToBP_BaseCollectable (Variables|/Script/Project2016.C_PlayerController|Getc_Inventory _bp_controller_ref_2)))
          (Variables|Default|SetSlot _asbp_base_collectable)
          (Variables|/Script/Project2016.C_PlayerController|Setc_Inventory _bp_controller_ref_2 0)
          (if (Utilities|Name|Equal(Name) (Variables|/Script/Project2016.BaseCollectable|GetsupposedBowlTag (Variables|Default|GetSlot)) (Variables|Default|GetSupposedBallTag))
            (Variables|Default|SetSolved true))))
      (elif (!= (Variables|Default|GetSlot) 0)
        (Variables|/Script/Project2016.C_PlayerController|Setc_Inventory (Variables|Default|GetBP_Controller_Ref) (Variables|Default|GetSlot))
        (Variables|Default|SetSlot 0)
        (Rendering|SetVisibility (Variables|Default|GetInserted_Object) false false)
        (Variables|/Script/Project2016.BaseCollectable|Setbowl (Variables|/Script/Project2016.C_PlayerController|Getc_Inventory (Variables|Default|GetBP_Controller_Ref)) true)
        (bind _asbp_base_collectable_2 (Utilities|Casting|CastToBP_BaseCollectable (Variables|/Script/Project2016.C_PlayerController|Getc_Inventory (Variables|Default|GetBP_Controller_Ref))))
        (Variables|/Game/Blueprints/Objects/BP_BaseCollectable.BP_BaseCollectable_C|SetLastPlace _asbp_base_collectable_2 self)
        (Variables|Default|SetSolved false)))
    (elif (== (Variables|Default|GetSupposedRepairObject) (Utilities|GetClass (Variables|/Script/Project2016.C_PlayerController|Getc_Inventory _bp_controller_ref)))
      (Variables|Default|SetBowl true)
      (Variables|/Script/Project2016.C_PlayerController|Setc_Inventory _bp_controller_ref 0))))

(event EventTick
  (params (DeltaSeconds :type Float%20%28single-precision%29))
  (bind _decorative_mesh_whole (Variables|Default|GetDecorative_Mesh_Whole))
  (bind _decorative_mesh_kaputto (Variables|Default|GetDecorative_Mesh_Kaputto))
  (if (Variables|Default|GetBowl)
    (Rendering|SetVisibility _decorative_mesh_whole true false)
    (Rendering|SetVisibility _decorative_mesh_kaputto false false)
    (else
      (Rendering|SetVisibility _decorative_mesh_whole false false)
      (Rendering|SetVisibility _decorative_mesh_kaputto true false))))

(event EventBeginPlay
  (bind _asbp_controller_2 (Utilities|Casting|CastToBP_Controller2 (Game|GetPlayerController 0)))
  (Variables|Default|SetBP_Controller_Ref _asbp_controller_2)
  (Utilities|IsValid (Variables|Default|GetBP_Controller_Ref)
    (:Is%20Not%20Valid
      (Development|PrintString "Controller_Ref in BP_Basic_Bowl not valid"))))

(event Input|KeyboardEvents|F
  (params (Key :type Key%20Structure :default "AnyKey"))
  (bind _bp_controller_ref (Variables|Default|GetBP_Controller_Ref))
  (bind _inserted_object (Variables|Default|GetInserted_Object))
  (bind _bp_controller_ref_2 (Variables|Default|GetBP_Controller_Ref))
  (:Pressed
    (if (Variables|Default|GetBowl)
      (if (!= (Variables|/Script/Project2016.C_PlayerController|Getc_Inventory (Variables|Default|GetBP_Controller_Ref)) 0) ; Check Inventory empty
        (if (== (Utilities|GetClass (Variables|/Script/Project2016.C_PlayerController|Getc_Inventory (Variables|Default|GetBP_Controller_Ref))) (Variables|Default|GetSupposedObjectCLASS)) ; Check Inventory supposed Itemclass
          (if (== (Variables|Default|GetSlot) 0) ; Check Slot empty
            (Rendering|SetVisibility (Variables|Default|GetInserted_Object) true false)
            (Components|StaticMesh|SetStaticMesh _inserted_object (Variables|/Script/Engine.StaticMeshComponent|GetStaticMesh (Variables|/Script/Project2016.BaseCollectable|GetStaticMeshComponent (Variables|/Script/Project2016.C_PlayerController|Getc_Inventory (Variables|Default|GetBP_Controller_Ref)))))
            (Rendering|Material|SetMaterial _inserted_object 0 (Rendering|Material|GetMaterial (Variables|/Script/Project2016.BaseCollectable|GetStaticMeshComponent (Variables|/Script/Project2016.C_PlayerController|Getc_Inventory (Variables|Default|GetBP_Controller_Ref))) 0))
            (bind _asbp_base_collectable (Utilities|Casting|CastToBP_BaseCollectable (Variables|/Script/Project2016.C_PlayerController|Getc_Inventory _bp_controller_ref_2)))
            (Variables|Default|SetSlot _asbp_base_collectable)
            (Variables|/Script/Project2016.C_PlayerController|Setc_Inventory _bp_controller_ref_2 0)
            (if (Utilities|Name|Equal(Name) (Variables|/Script/Project2016.BaseCollectable|GetsupposedBowlTag (Variables|Default|GetSlot)) (Variables|Default|GetSupposedBallTag))
              (Variables|Default|SetSolved true))))
        (elif (!= (Variables|Default|GetSlot) 0)
          (Variables|/Script/Project2016.C_PlayerController|Setc_Inventory (Variables|Default|GetBP_Controller_Ref) (Variables|Default|GetSlot))
          (Variables|Default|SetSlot 0)
          (Rendering|SetVisibility (Variables|Default|GetInserted_Object) false false)
          (Variables|/Script/Project2016.BaseCollectable|Setbowl (Variables|/Script/Project2016.C_PlayerController|Getc_Inventory (Variables|Default|GetBP_Controller_Ref)) true)
          (bind _asbp_base_collectable_2 (Utilities|Casting|CastToBP_BaseCollectable (Variables|/Script/Project2016.C_PlayerController|Getc_Inventory (Variables|Default|GetBP_Controller_Ref))))
          (Variables|/Game/Blueprints/Objects/BP_BaseCollectable.BP_BaseCollectable_C|SetLastPlace _asbp_base_collectable_2 self)
          (Variables|Default|SetSolved false)))
      (elif (== (Variables|Default|GetSupposedRepairObject) (Utilities|GetClass (Variables|/Script/Project2016.C_PlayerController|Getc_Inventory _bp_controller_ref)))
        (Variables|Default|SetBowl true)
        (Variables|/Script/Project2016.C_PlayerController|Setc_Inventory _bp_controller_ref 0)))))

(event Input|GamepadEvents|GamepadFaceButtonRight
  (params (Key :type Key%20Structure :default "AnyKey"))
  (bind _bp_controller_ref (Variables|Default|GetBP_Controller_Ref))
  (bind _inserted_object (Variables|Default|GetInserted_Object))
  (bind _bp_controller_ref_2 (Variables|Default|GetBP_Controller_Ref))
  (:Pressed
    (if (Variables|Default|GetBowl)
      (if (!= (Variables|/Script/Project2016.C_PlayerController|Getc_Inventory (Variables|Default|GetBP_Controller_Ref)) 0) ; Check Inventory empty
        (if (== (Utilities|GetClass (Variables|/Script/Project2016.C_PlayerController|Getc_Inventory (Variables|Default|GetBP_Controller_Ref))) (Variables|Default|GetSupposedObjectCLASS)) ; Check Inventory supposed Itemclass
          (if (== (Variables|Default|GetSlot) 0) ; Check Slot empty
            (Rendering|SetVisibility (Variables|Default|GetInserted_Object) true false)
            (Components|StaticMesh|SetStaticMesh _inserted_object (Variables|/Script/Engine.StaticMeshComponent|GetStaticMesh (Variables|/Script/Project2016.BaseCollectable|GetStaticMeshComponent (Variables|/Script/Project2016.C_PlayerController|Getc_Inventory (Variables|Default|GetBP_Controller_Ref)))))
            (Rendering|Material|SetMaterial _inserted_object 0 (Rendering|Material|GetMaterial (Variables|/Script/Project2016.BaseCollectable|GetStaticMeshComponent (Variables|/Script/Project2016.C_PlayerController|Getc_Inventory (Variables|Default|GetBP_Controller_Ref))) 0))
            (bind _asbp_base_collectable (Utilities|Casting|CastToBP_BaseCollectable (Variables|/Script/Project2016.C_PlayerController|Getc_Inventory _bp_controller_ref_2)))
            (Variables|Default|SetSlot _asbp_base_collectable)
            (Variables|/Script/Project2016.C_PlayerController|Setc_Inventory _bp_controller_ref_2 0)
            (if (Utilities|Name|Equal(Name) (Variables|/Script/Project2016.BaseCollectable|GetsupposedBowlTag (Variables|Default|GetSlot)) (Variables|Default|GetSupposedBallTag))
              (Variables|Default|SetSolved true))))
        (elif (!= (Variables|Default|GetSlot) 0)
          (Variables|/Script/Project2016.C_PlayerController|Setc_Inventory (Variables|Default|GetBP_Controller_Ref) (Variables|Default|GetSlot))
          (Variables|Default|SetSlot 0)
          (Rendering|SetVisibility (Variables|Default|GetInserted_Object) false false)
          (Variables|/Script/Project2016.BaseCollectable|Setbowl (Variables|/Script/Project2016.C_PlayerController|Getc_Inventory (Variables|Default|GetBP_Controller_Ref)) true)
          (bind _asbp_base_collectable_2 (Utilities|Casting|CastToBP_BaseCollectable (Variables|/Script/Project2016.C_PlayerController|Getc_Inventory (Variables|Default|GetBP_Controller_Ref))))
          (Variables|/Game/Blueprints/Objects/BP_BaseCollectable.BP_BaseCollectable_C|SetLastPlace _asbp_base_collectable_2 self)
          (Variables|Default|SetSolved false)))
      (elif (== (Variables|Default|GetSupposedRepairObject) (Utilities|GetClass (Variables|/Script/Project2016.C_PlayerController|Getc_Inventory _bp_controller_ref)))
        (Variables|Default|SetBowl true)
        (Variables|/Script/Project2016.C_PlayerController|Setc_Inventory _bp_controller_ref 0)))))

(fn ConstructionScript
  (bind _inserted_object (Variables|Default|GetInserted_Object))
  (bind _slot (Variables|Default|GetSlot))
  (bind _staticmeshcomponent (Variables|/Script/Project2016.BaseCollectable|GetStaticMeshComponent _slot))
  (if (!= (Variables|Default|GetSlot) 0)
    (Rendering|SetVisibility (Variables|Default|GetInserted_Object) true false)
    (Components|StaticMesh|SetStaticMesh _inserted_object (Variables|/Script/Engine.StaticMeshComponent|GetStaticMesh _staticmeshcomponent))
    (Rendering|Material|SetMaterial _inserted_object 0 (Rendering|Material|GetMaterial _staticmeshcomponent 0)))
  (if (Utilities|Name|Equal(Name) (Variables|Default|GetSupposedBallTag) "None")
    (Development|PrintString (Utilities|String|Append "Please set \"Supposed Ball Tag\" in: " (Utilities|GetDisplayName self)))))
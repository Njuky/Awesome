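; BP_Ball is a quest pickup that can appear intact or broken, optionally depending on the controller's current time matching its supposed time.
; Tick swaps the meshes and sphere overlap events to reflect that state.
; Interact input either stores an intact ball in BP_Controller2's single inventory slot or repairs a broken one by consuming a held BP_Schnecke, if eligible.
; DropItem delegates to altars, flower or bowl places, otherwise re-shows the ball, then clears the slot.
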(event Custom|DropItem
  (bind _returnvalue (Game|GetPlayerController 0))
  (if (Variables|Default|Getaltar)
    (bind _outactors (Actor|GetAllActorsOfClass "/Game/Blueprints/Quest/QuestObjects/Quest2/BP_Altar.BP_Altar_C"))
    (for _array_element _outactors
      (Default|DropItem _array_element)
      (bind _asbp_controller_2 (Utilities|Casting|CastToBP_Controller2 _returnvalue))
      (Variables|/Script/Project2016.C_PlayerController|Setc_Inventory _asbp_controller_2 0)
      (Input|DisableInput _returnvalue)
      (Collision|SetActorEnableCollision true))
    (else
      (if (Variables|Default|GetFlower_0)
        (Default|DropItem (Variables|Default|GetlastFlower))
        (elif (Variables|Default|GetBowl)
          (Default|DropItem (Variables|Default|GetLastPlace))
          (else
            (Rendering|SetVisibility (Variables|Default|GetStaticMeshComponent) true true)
            (Variables|Default|SetEnabled true))))
      (bind _asbp_controller_2_2 (Utilities|Casting|CastToBP_Controller2 _returnvalue))
      (Variables|/Script/Project2016.C_PlayerController|Setc_Inventory _asbp_controller_2_2 0)
      (Input|DisableInput _returnvalue)
      (Collision|SetActorEnableCollision true))))

(event EventTick
  (params (DeltaSeconds :type Float%20%28single-precision%29))
  (bind _brokenmesh (Variables|Default|GetBrokenMesh))
  (bind _staticmeshcomponent (Variables|Default|GetStaticMeshComponent))
  (bind _sphere1 (Variables|Default|GetSphere1))
  (if (Variables|Default|GetEnabled)
    (if (Variables|Default|GetTimeRelevant)
      (bind _asbp_controller_2 (Utilities|Casting|CastToBP_Controller2 (Game|GetPlayerController 0)))
      (if (Math|Boolean|Equal(Boolean) (Variables|/Script/Project2016.C_PlayerController|GetcurrentTime _asbp_controller_2) (Variables|Default|GetSupposedTime))
        (Variables|Default|Setbroken false)
        (else
          (Variables|Default|Setbroken true))))
    (if (Variables|Default|Getbroken)
      (Rendering|SetVisibility _brokenmesh true false)
      (Rendering|SetVisibility _staticmeshcomponent false false)
      (Variables|/Script/Engine.PrimitiveComponent|SetbGenerateOverlapEvents _sphere1 false)
      (else
        (Rendering|SetVisibility _brokenmesh false false)
        (Rendering|SetVisibility _staticmeshcomponent true false)
        (Variables|/Script/Engine.PrimitiveComponent|SetbGenerateOverlapEvents _sphere1 true)))))

(event Input|KeyboardEvents|F
  (params (Key :type Key%20Structure :default "AnyKey"))
  (:Pressed
    (if (Variables|Default|GetEnabled)
      (bind _asbp_controller_2 (Utilities|Casting|CastToBP_Controller2 (Game|GetPlayerController 0)))
      (if (Variables|Default|Getbroken)
        (if (and (== (Utilities|GetClass (Variables|/Script/Project2016.C_PlayerController|Getc_Inventory _asbp_controller_2)) "/Game/Blueprints/Quest/QuestObjects/Quest2/BP_Schnecke.BP_Schnecke_C") (or (Actor|ActorHasTag "Verzweiflung") (Variables|Default|GetSnail_0)))
          (Variables|Default|Setbroken false)
          (Actor|DestroyActor (Variables|/Script/Project2016.C_PlayerController|Getc_Inventory _asbp_controller_2))
          (Variables|/Script/Project2016.C_PlayerController|Setc_Inventory _asbp_controller_2 0))
        (elif (== (Variables|/Script/Project2016.C_PlayerController|Getc_Inventory _asbp_controller_2) 0)
          (Rendering|SetVisibility (Variables|Default|GetStaticMeshComponent) false true)
          (Variables|/Script/Project2016.C_PlayerController|Setc_Inventory _asbp_controller_2 self)
          (Variables|Default|SetEnabled false)
          (Collision|SetActorEnableCollision false))))))

(event Input|GamepadEvents|GamepadFaceButtonRight
  (params (Key :type Key%20Structure :default "AnyKey"))
  (:Pressed
    (if (Variables|Default|GetEnabled)
      (bind _asbp_controller_2 (Utilities|Casting|CastToBP_Controller2 (Game|GetPlayerController 0)))
      (if (Variables|Default|Getbroken)
        (if (and (== (Utilities|GetClass (Variables|/Script/Project2016.C_PlayerController|Getc_Inventory _asbp_controller_2)) "/Game/Blueprints/Quest/QuestObjects/Quest2/BP_Schnecke.BP_Schnecke_C") (or (Actor|ActorHasTag "Verzweiflung") (Variables|Default|GetSnail_0)))
          (Variables|Default|Setbroken false)
          (Actor|DestroyActor (Variables|/Script/Project2016.C_PlayerController|Getc_Inventory _asbp_controller_2))
          (Variables|/Script/Project2016.C_PlayerController|Setc_Inventory _asbp_controller_2 0))
        (elif (== (Variables|/Script/Project2016.C_PlayerController|Getc_Inventory _asbp_controller_2) 0)
          (Rendering|SetVisibility (Variables|Default|GetStaticMeshComponent) false true)
          (Variables|/Script/Project2016.C_PlayerController|Setc_Inventory _asbp_controller_2 self)
          (Variables|Default|SetEnabled false)
          (Collision|SetActorEnableCollision false))))))

(fn ConstructionScript
  (if (not (Variables|Default|GetEnabled))
    (Rendering|SetVisibility (Variables|Default|GetStaticMeshComponent) false true)))
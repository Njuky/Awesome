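; BP_Bowl is a quest bowl that the player can interact with while inside its collision sphere.
; Sphere overlaps register the bowl on BP_Controller and switch off the controller's general interaction flag until exit.
; Tick spawns an optional one-shot particle above the inserted object when solved, re-arming if unsolved, and can tie BowlExist to the controller's current time.
; A distance-based custom-depth highlight is present but never runs.
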(event OnComponentBeginOverlap(c_CollisionSphere)
  (params (OverlappedComponent :type Primitive%20Component%20Object%20Reference) (OtherActor :type Actor%20Object%20Reference) (OtherComp :type Primitive%20Component%20Object%20Reference) (OtherBodyIndex :type Integer) (bFromSweep :type Boolean) (SweepResult :type Hit%20Result%20Structure%20%28by%20ref%29))
  (Utilities|Casting|CastToBP_Character OtherActor)
  (Variables|Default|Setc_CanInteract true)
  (bind _asbp_controller (Utilities|Casting|CastToBP_Controller (Game|GetPlayerController 0)))
  (Variables|/Script/Project2016.C_PlayerController|SetbCanInteract _asbp_controller false)
  (Variables|/Script/Project2016.C_PlayerController|Setc_BowlRef _asbp_controller self))

(event OnComponentEndOverlap(c_CollisionSphere)
  (params (OverlappedComponent :type Primitive%20Component%20Object%20Reference) (OtherActor :type Actor%20Object%20Reference) (OtherComp :type Primitive%20Component%20Object%20Reference) (OtherBodyIndex :type Integer))
  (Utilities|Casting|CastToBP_Character OtherActor)
  (Variables|Default|Setc_CanInteract false)
  (bind _asbp_controller (Utilities|Casting|CastToBP_Controller (Game|GetPlayerController 0)))
  (Variables|/Script/Project2016.C_PlayerController|SetbCanInteract _asbp_controller true)
  (Variables|/Script/Project2016.C_PlayerController|Setc_BowlRef _asbp_controller 0))

(event EventTick
  (params (DeltaSeconds :type Float%20%28single-precision%29))
  (bind _c_insertedobject (Variables|Default|Getc_InsertedObject))
  (bind _returnvalue (Transformation|GetWorldLocation _c_insertedobject))
  (bind (_x _y _z) (Math|Vector|BreakVector _returnvalue))
  (|CallParentFunction DeltaSeconds)
  (Utilities|FlowControl|Sequence
    (:then_0
      (if (Variables|Default|GetUseParticle)
        (if (Variables|Default|Getc_solved)
          (if (not (Variables|Default|Getdidparticle))
            (Variables|Default|Setdidparticle true)
            (bind _returnvalue_2 (Effects|SpawnEmitteratLocation (Variables|Default|GetParticle) (Math|Vector|MakeVector _x _y (+ _z (* (.Z (Math|Vector|BreakVector (Transformation|GetWorldScale (Variables|Default|Getc_InsertedObject)))) 5.0)))))
            (Transformation|SetWorldScale3D _returnvalue_2 "2.000000,2.000000,2.000000"))
          (elif (Variables|Default|Getdidparticle)
            (Variables|Default|Setdidparticle false)))))
    (:then_1
      (if (Variables|Default|GetTimeRevelant)
        (if (Math|Boolean|Equal(Boolean) (Variables|/Script/Project2016.C_PlayerController|GetcurrentTime (Variables|Default|GetpController_Ref)) (Variables|Default|GetSupposedTime))
          (Variables|Default|SetbowlExist true)
          (else
            (Variables|Default|SetbowlExist false)))))))

(fn ConstructionScript)
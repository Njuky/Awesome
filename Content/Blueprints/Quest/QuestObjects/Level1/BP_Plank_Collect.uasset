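; BP_Plank_Collect is the collectible plank quest object for Level 1, extending a parent collectable Blueprint.
; It finds BP_QuestoverviewLevel1 and only allows collection, button display and overlap highlighting while its TimeObject flag is set.
; Collecting sets the overview's Plank flag before calling the parent logic.
; Overlap turns on custom depth and Outline; ending overlap clears custom depth but leaves Outline enabled.
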(event Collision|EventActorBeginOverlap
  (params (OtherActor :type Actor%20Object%20Reference))
  ;[1 1 1] Outline
  (bind _outactors (Actor|GetAllActorsOfClass "/Game/Blueprints/Quest/BP_QuestoverviewLevel1.BP_QuestoverviewLevel1_C"))
  (for _array_element _outactors
    (if (Variables|/Game/Blueprints/Quest/BP_QuestoverviewLevel1.BP_QuestoverviewLevel1_C|GetTimeObject _array_element)
      (Rendering|SetRenderCustomDepth (Variables|Default|GetStaticMesh) true)
      (Variables|/Script/Engine.PostProcessComponent|SetbEnabled (Variables|Default|GetOutline) true))))

(event Collision|EventActorEndOverlap
  (params (OtherActor :type Actor%20Object%20Reference))
  ;[1 1 1] Outline
  (Rendering|SetRenderCustomDepth (Variables|Default|GetStaticMesh) false)
  (Variables|/Script/Engine.PostProcessComponent|SetbEnabled (Variables|Default|GetOutline) true))

(event EventCollectObject
  (bind _outactors (Actor|GetAllActorsOfClass "/Game/Blueprints/Quest/BP_QuestoverviewLevel1.BP_QuestoverviewLevel1_C"))
  (for _array_element _outactors
    (if (Variables|/Game/Blueprints/Quest/BP_QuestoverviewLevel1.BP_QuestoverviewLevel1_C|GetTimeObject _array_element)
      (Variables|/Game/Blueprints/Quest/BP_QuestoverviewLevel1.BP_QuestoverviewLevel1_C|SetPlank _array_element true)
      (|CallParentFunction))))

(event EventShowButton
  (bind _outactors (Actor|GetAllActorsOfClass "/Game/Blueprints/Quest/BP_QuestoverviewLevel1.BP_QuestoverviewLevel1_C"))
  (for _array_element _outactors
    (if (Variables|/Game/Blueprints/Quest/BP_QuestoverviewLevel1.BP_QuestoverviewLevel1_C|GetTimeObject _array_element)
      (|CallParentFunction))))

(fn ConstructionScript
  (|CallParentFunction))
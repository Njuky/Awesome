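; BP_TimeObject is a Level 1 quest object that is collected when both gamepad triggers are held, or when T is pressed.
; Tick watches both trigger flags and, through a DoOnce, calls FirstTimeWalk on BP_Controller, sets TimeObject on each BP_QuestoverviewLevel1 and calls the parent CollectObject.
; Actor overlap toggles custom depth for an outline, while ShowButton only prints a placeholder for an unfinished widget.
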(event EventShowButton
  (Development|PrintString "Create Widget for BP_TimeObject"))

(event Collision|EventActorBeginOverlap
  (params (OtherActor :type Actor%20Object%20Reference))
  ;[1 1 1] Outline
  (Rendering|SetRenderCustomDepth (Variables|Default|GetStaticMesh) true)
  (Variables|/Script/Engine.PostProcessComponent|SetbEnabled (Variables|Default|GetOutline) true))

(event Collision|EventActorEndOverlap
  (params (OtherActor :type Actor%20Object%20Reference))
  ;[1 1 1] Outline
  (Rendering|SetRenderCustomDepth (Variables|Default|GetStaticMesh) false)
  (Variables|/Script/Engine.PostProcessComponent|SetbEnabled (Variables|Default|GetOutline) true))

(event EventTick
  (params (DeltaSeconds :type Float%20%28single-precision%29))
  (if (and (Variables|Default|GetTrigger1) (Variables|Default|GetTrigger2))
    (Utilities|FlowControl|DoOnce false
      (:Completed
        (bind _asbp_controller (Utilities|Casting|CastToBP_Controller (Game|GetPlayerController 0)))
        (Default|FirstTimeWalk _asbp_controller)
        (bind _outactors (Actor|GetAllActorsOfClass "/Game/Blueprints/Quest/BP_QuestoverviewLevel1.BP_QuestoverviewLevel1_C"))
        (for _array_element _outactors
          (Variables|/Game/Blueprints/Quest/BP_QuestoverviewLevel1.BP_QuestoverviewLevel1_C|SetTimeObject _array_element true)
          (|CallParentFunction))))))

(event EventCollectObject)

(event Input|GamepadEvents|GamepadLeftTrigger
  (params (Key :type Key%20Structure :default "AnyKey"))
  (:Pressed
    (Variables|Default|SetTrigger1 true))
  (:Released
    (Variables|Default|SetTrigger1 false)))

(event Input|GamepadEvents|GamepadRightTrigger
  (params (Key :type Key%20Structure :default "AnyKey"))
  (:Pressed
    (Variables|Default|SetTrigger2 true))
  (:Released
    (Variables|Default|SetTrigger2 false)))

(event Input|KeyboardEvents|T
  (params (Key :type Key%20Structure :default "AnyKey"))
  (:Pressed
    (Variables|Default|SetTrigger1 true)
    (Variables|Default|SetTrigger2 true)))

(fn ConstructionScript
  (|CallParentFunction))
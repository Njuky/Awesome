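; BP_TimeObject is a Quest1 collectible that the player collects by holding both gamepad triggers at once, or by pressing T.
; Tick watches both trigger flags and, once only, sets TimeObject on BP_Questoverview actors and calls the parent's CollectObject.
; Leaving the Box as BP_Character disables input, while actor overlaps toggle custom depth on the mesh for an outline highlight.
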(event OnComponentEndOverlap(Box)
  (params (OtherActor :type Actor%20Object%20Reference) (OtherComp :type Primitive%20Component%20Object%20Reference) (OtherBodyIndex :type Integer))
  (Utilities|Casting|CastToBP_Character OtherActor)
  (Input|DisableInput (Game|GetPlayerController 0))
  (if (!= (Variables|Default|GetRT_LT%20Widget) 0)
    _))

(event Collision|EventActorBeginOverlap
  (params (OtherActor :type Actor%20Object%20Reference))
  ;[1 1 1] Outline
  (Rendering|SetRenderCustomDepth (Variables|Default|GetObject_Mesh) true)
  (Variables|/Script/Engine.PostProcessComponent|SetbEnabled (Variables|Default|GetOutline) true))

(event Collision|EventActorEndOverlap
  (params (OtherActor :type Actor%20Object%20Reference))
  ;[1 1 1] Outline
  (Rendering|SetRenderCustomDepth (Variables|Default|GetObject_Mesh) false)
  (Variables|/Script/Engine.PostProcessComponent|SetbEnabled (Variables|Default|GetOutline) true))

(event EventTick
  (params (DeltaSeconds :type Float%20%28single-precision%29))
  (if (and (Variables|Default|GetTrigger1) (Variables|Default|GetTrigger2))
    (Utilities|FlowControl|DoOnce false
      (:Completed
        (bind _outactors (Actor|GetAllActorsOfClass "/Game/Blueprints/Quest/BP_Questoverview.BP_Questoverview_C"))
        (for _array_element _outactors
          (Variables|/Game/Blueprints/Quest/BP_Questoverview.BP_Questoverview_C|SetTimeObject _array_element true)
          (|CallParentFunction))))))

(event EventCollectObject)

(event Input|GamepadEvents|GamepadLeftTrigger
  (params (Key :type Key%20Structure :default "AnyKey"))
  (:Pressed
    (Variables|Default|SetTrigger1 true))
  (:Released
    (Variables|Default|SetTrigger1 false)))

(event Input|GamepadEvents|GamepadRightTrigger
  (params (Key :type Key%20Structure :default "AnyKey"))
  (:Pressed
    (Variables|Default|SetTrigger2 true))
  (:Released
    (Variables|Default|SetTrigger2 false)))

(event Input|KeyboardEvents|T
  (params (Key :type Key%20Structure :default "AnyKey"))
  (:Pressed
    (Variables|Default|SetTrigger1 true)
    (Variables|Default|SetTrigger2 true)))

(fn ConstructionScript
  (|CallParentFunction))
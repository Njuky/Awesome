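; BP_Plank_Collect is a collectable plank for Quest 1, built on a parent collect-object Blueprint.
; When collected while a BP_Questoverview has TimeObject set, it flags Plank there and runs the parent's collect logic.
; Overlap start enables custom depth and Outline under the same condition; overlap end disables custom depth but leaves Outline enabled.
; ShowButton checks TimeObject but takes no action.
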(event Custom|ShowButton
  (bind _outactors (Actor|GetAllActorsOfClass "/Game/Blueprints/Quest/BP_Questoverview.BP_Questoverview_C"))
  (for _array_element _outactors
    (if (Variables|/Game/Blueprints/Quest/BP_Questoverview.BP_Questoverview_C|GetTimeObject _array_element)
      _)))

(event Collision|EventActorBeginOverlap
  (params (OtherActor :type Actor%20Object%20Reference))
  ;[1 1 1] Outline
  (bind _outactors (Actor|GetAllActorsOfClass "/Game/Blueprints/Quest/BP_Questoverview.BP_Questoverview_C"))
  (for _array_element _outactors
    (if (Variables|/Game/Blueprints/Quest/BP_Questoverview.BP_Questoverview_C|GetTimeObject _array_element)
      (Rendering|SetRenderCustomDepth (Variables|Default|GetObject_Mesh) true)
      (Variables|/Script/Engine.PostProcessComponent|SetbEnabled (Variables|Default|GetOutline) true))))

(event Collision|EventActorEndOverlap
  (params (OtherActor :type Actor%20Object%20Reference))
  ;[1 1 1] Outline
  (Rendering|SetRenderCustomDepth (Variables|Default|GetObject_Mesh) false)
  (Variables|/Script/Engine.PostProcessComponent|SetbEnabled (Variables|Default|GetOutline) true))

(event EventCollectObject
  (bind _outactors (Actor|GetAllActorsOfClass "/Game/Blueprints/Quest/BP_Questoverview.BP_Questoverview_C"))
  (for _array_element _outactors
    (if (Variables|/Game/Blueprints/Quest/BP_Questoverview.BP_Questoverview_C|GetTimeObject _array_element)
      (Variables|/Game/Blueprints/Quest/BP_Questoverview.BP_Questoverview_C|SetPlank _array_element true)
      (|CallParentFunction))))

(fn ConstructionScript
  (|CallParentFunction))
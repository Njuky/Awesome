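; BP_Plank_placed is a Quest 1 object that lets the player place a plank.
; Entering its TriggerBox enables input and shows a button prompt if BP_Questoverview's Plank flag is set and the controller's CurrentTime is false.
; Pressing F or the gamepad right face button then destroys the blocking volume and makes the plank mesh visible.
; Leaving the trigger removes any shown prompt and disables that input.
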(event OnActorBeginOverlap(TriggerBox)
  (params (OtherActor :type Actor%20Object%20Reference))
  (bind _returnvalue (Game|GetPlayerController 0))
  (bind _outactors (Actor|GetAllActorsOfClass "/Game/Blueprints/Quest/BP_Questoverview.BP_Questoverview_C"))
  (for _array_element _outactors
    (if (Variables|/Game/Blueprints/Quest/BP_Questoverview.BP_Questoverview_C|GetPlank _array_element)
      (bind _asbp_controller (Utilities|Casting|CastToBP_Controller _returnvalue))
      (if (not (Variables|/Game/Blueprints/Character/Player/BP_Controller.BP_Controller_C|GetCurrentTime _asbp_controller))
        (Input|EnableInput _returnvalue)
        (bind _returnvalue_2 (UserInterface|CreateWidget "/Game/Blueprints/TalkToObjects/BButtonWidget.BButtonWidget_C"))
        (bind _output_get (Variables|Default|SetBButtonWidget _returnvalue_2))
        (UserInterface|Viewport|AddtoViewport _output_get 0)
        (Variables|Default|SetCanBePlaced true)))))

(event OnActorEndOverlap(TriggerBox)
  (params (OtherActor :type Actor%20Object%20Reference))
  (if (!= (Variables|Default|GetBButtonWidget) 0)
    (Widget|RemovefromParent (Variables|Default|GetBButtonWidget))
    (Variables|Default|SetCanBePlaced false)
    (Input|DisableInput (Game|GetPlayerController 0))))

(event Input|GamepadEvents|GamepadFaceButtonRight
  (params (Key :type Key%20Structure :default "AnyKey"))
  (:Pressed
    (if (Variables|Default|GetCanBePlaced)
      (Actor|DestroyActor (Variables|Default|GetBlockingVolumePlank))
      (Rendering|SetVisibility (Variables|Default|GetStaticMesh) true false))))

(event Input|KeyboardEvents|F
  (params (Key :type Key%20Structure :default "AnyKey"))
  (:Pressed
    (if (Variables|Default|GetCanBePlaced)
      (Actor|DestroyActor (Variables|Default|GetBlockingVolumePlank))
      (Rendering|SetVisibility (Variables|Default|GetStaticMesh) true false))))

(fn ConstructionScript)
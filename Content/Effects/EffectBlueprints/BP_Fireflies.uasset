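; Firefly effect actor that wraps a particle system with configurable spawn radius and spawn amount.
; The construction script passes both values into the particle parameters and draws a debug sphere showing the radius in the editor.
; Each tick it measures distance to the player character, hiding the particles beyond a fixed range and showing them when closer, as a simple distance cull.
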(event EventBeginPlay)

(event Collision|EventActorBeginOverlap
  (params (OtherActor :type Actor%20Object%20Reference)))

(event EventTick
  (params (DeltaSeconds :type Float%20%28single-precision%29))
  (Math|Float|CompareFloat (Transformation|GetDistanceTo self (Game|GetPlayerCharacter 0)) 1.3e+04
    (:>
      (Rendering|SetVisibility (Variables|Default|GetParticleSystem) false false))
    (:<
      (Rendering|SetVisibility (Variables|Default|GetParticleSystem) true false))))

(fn ConstructionScript
  (bind _particlesystem (Variables|Default|GetParticleSystem))
  (bind _spawnradius (Variables|Default|GetSpawnRadius))
  (Rendering|Debug|DrawDebugSphere (Transformation|GetWorldLocation _particlesystem) _spawnradius 10 "(R=1.000000,G=1.000000,B=1.000000,A=1.000000)" 0.0)
  (Effects|Components|ParticleSystem|SetFloatParameter _particlesystem "SphereRadius" _spawnradius)
  (Effects|Components|ParticleSystem|SetFloatParameter _particlesystem "Spawn" (Variables|Default|GetSpawn)))
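; BP_LowPolyWater is an effect actor that presents a configurable low-poly water surface on a static mesh.
; Its construction script copies the actor's wave, tessellation, noise and dark/bright color variables into parameters on the mesh's materials.
; The Blueprint has no active runtime logic, so any animation is left to the material.
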(event EventActorBeginOverlap
  (params (OtherActor :type Actor%20Object%20Reference)))

(event EventTick
  (params (DeltaSeconds :type Float%20%28single-precision%29)))

(event EventBeginPlay)

(fn ConstructionScript
  (bind _staticmeshcomponent (Variables|Debug|GetStaticMeshComponent))
  (Rendering|Material|SetScalarParameterValueonMaterials _staticmeshcomponent "WaveHeight" (Variables|Default|GetWave%20Height))
  (Rendering|Material|SetScalarParameterValueonMaterials _staticmeshcomponent "TesselationMultiplier" (Variables|Default|GetTesselation%20Multiplier))
  (Rendering|Material|SetScalarParameterValueonMaterials _staticmeshcomponent "Noise Animation Speed" (Variables|Default|GetNoise%20Animation%20Speed))
  (Rendering|Material|SetScalarParameterValueonMaterials _staticmeshcomponent "NoiseScale" (Variables|Default|GetNoiseScale))
  (Rendering|Material|SetVectorParameterValueonMaterials _staticmeshcomponent "Color1" (Math|Conversions|ToVector(LinearColor) (Variables|Default|GetWave%20Color%20Dark)))
  (Rendering|Material|SetVectorParameterValueonMaterials _staticmeshcomponent "Color2" (Math|Conversions|ToVector(LinearColor) (Variables|Default|GetWave%20Color%20Bright))))
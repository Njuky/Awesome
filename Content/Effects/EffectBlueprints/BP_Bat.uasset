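; BP_Bat is an effect trigger actor that spawns a particle emitter when BP_Character enters its sphere.
; The construction script applies a configurable sphere radius and offsets the particle component by ParticleLocation.
; On overlap it prints a debug "Hello" and, while First is false, spawns the emitter using that same vector as world location.
; Nothing in these graphs sets First, so the effect can repeat on each overlap.
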(event OnComponentBeginOverlap(Sphere)
  (params (OverlappedComponent :type Primitive%20Component%20Object%20Reference) (OtherActor :type Actor%20Object%20Reference) (OtherComp :type Primitive%20Component%20Object%20Reference) (OtherBodyIndex :type Integer) (bFromSweep :type Boolean) (SweepResult :type Hit%20Result%20Structure%20%28by%20ref%29))
  (Utilities|Casting|CastToBP_Character OtherActor)
  (Development|PrintString "Hello")
  (if (not (Variables|Default|GetFirst))
    (Effects|SpawnEmitteratLocation 0 (Variables|Default|GetParticleLocation))))

(event EventBeginPlay)

(event Collision|EventActorBeginOverlap
  (params (OtherActor :type Actor%20Object%20Reference)))

(event EventTick
  (params (DeltaSeconds :type Float%20%28single-precision%29)))

(fn ConstructionScript
  (Components|Sphere|SetSphereRadius (Variables|Default|GetSphere) (Variables|Default|GetSphereRadius) true)
  (Transformation|AddLocalOffset (Variables|Default|GetParticleSystem) (Variables|Default|GetParticleLocation) false false))
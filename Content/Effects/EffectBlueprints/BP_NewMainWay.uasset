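; Particle effect actor that travels along the FlowAwayWay spline once a BP_Character enters its trigger sphere.
; Tick accumulates interpolated steps to move the particle system along the spline and continually shifts its Orbit parameter.
; On reaching the last point it stops following and sets FlowAway to an upward vector.
; The construction script sets the sphere radius and starting orbit, and caches spline point distances.
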(event OnComponentBeginOverlap(Sphere)
  (params (OverlappedComponent :type Primitive%20Component%20Object%20Reference) (OtherActor :type Actor%20Object%20Reference) (OtherComp :type Primitive%20Component%20Object%20Reference) (OtherBodyIndex :type Integer) (bFromSweep :type Boolean) (SweepResult :type Hit%20Result%20Structure%20%28by%20ref%29))
  (Utilities|Casting|CastToBP_Character OtherActor)
  (if (not (Variables|Default|GetActive))
    (Variables|Default|SetActive true)))

(event EventTick
  (params (DeltaSeconds :type Float%20%28single-precision%29))
  (if (Variables|Default|GetActive)
    (Utilities|FlowControl|Sequence
      (:then_0
        (if (Variables|Default|GetEnd)
          (Effects|Components|ParticleSystem|SetVectorParameter (Variables|Default|GetParticleSystem) "FlowAway" "0, 0,500.000000")
          (else
            (bind _output_get (Variables|Default|SetDistance (+ (Math|Interpolation|FInterpTo 0.0 (Spline|GetSplineLength (Variables|Default|GetFlowAwayWay)) DeltaSeconds (Variables|Default|GetSpeed)) (stale _output_get))))
            (Transformation|SetWorldLocationAndRotation (Variables|Default|GetParticleSystem) (Spline|GetLocationatDistanceAlongSpline (Variables|Default|GetFlowAwayWay) _output_get "World") (Spline|GetRotationatDistanceAlongSpline (Variables|Default|GetFlowAwayWay) _output_get "World") false false)
            (if (Math|Vector|Equal(Vector) (Transformation|GetWorldLocation (Variables|Default|GetParticleSystem)) (Spline|GetLocationatSplinePoint (Variables|Default|GetFlowAwayWay) (Spline|GetNumberOfSplinePoints (Variables|Default|GetFlowAwayWay)) "World") 0.0001)
              (Variables|Default|SetEnd true)))))
      (:then_1
        (bind _output_get_2 (Variables|Default|SetOrbitSize (+ (Math|Interpolation|VInterpTo (Variables|Default|GetOrbitStart) (Variables|Default|GetOrbitFlowAway) 0.05 0.005) (stale _output_get_2))))
        (Effects|Components|ParticleSystem|SetVectorParameter (Variables|Default|GetParticleSystem) "Orbit" _output_get_2)))))

(fn ConstructionScript
  (bind _flowawayway (Variables|Default|GetFlowAwayWay))
  (bind _segmentlocations (Variables|Default|GetSegmentLocations))
  (Utilities|Array|Clear _segmentlocations)
  (for _index (range 0 (Spline|GetNumberOfSplinePoints _flowawayway))
    (Utilities|Array|Add _segmentlocations (Spline|GetDistanceAlongSplineatSplinePoint _flowawayway _index))
    (Components|Sphere|SetSphereRadius (Variables|Default|GetSphere) (Variables|Default|GetCollisionRadius) true)
    (Effects|Components|ParticleSystem|SetVectorParameter (Variables|Default|GetParticleSystem) "Orbit" (Variables|Default|GetOrbitStart))))
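; BP_Butterfly2 is a butterfly effect actor whose particle system reacts to day and night changes.
; Each tick it reads the CurrentTime flag on BP_Controller: true fires a TurnNight particle event and false fires StartDay, both at the particle system's location.
; Two cross-resetting DoOnce gates make each event fire once per transition instead of every frame.
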(event EventBeginPlay)

(event Collision|EventActorBeginOverlap
  (params (OtherActor :type Actor%20Object%20Reference)))

(event EventTick
  (params (DeltaSeconds :type Float%20%28single-precision%29))
  (bind _asbp_controller (Utilities|Casting|CastToBP_Controller (Game|GetPlayerController 0)))
  (if (Variables|/Script/Project2016.C_PlayerController|GetcurrentTime _asbp_controller)
    (Utilities|FlowControl|DoOnce false :!label _label
      (:Completed
        (Class|ParticleSystemComponent|GenerateParticleEvent (Variables|Default|GetParticleSystem) "TurnNight" 0.0 (Transformation|GetWorldLocation (Variables|Default|GetParticleSystem)) "0, 0, 0" "0, 0, 0")
        (goto _label_2 Reset)))
    (else
      (Utilities|FlowControl|DoOnce false :!label _label_2
        (:Completed
          (Class|ParticleSystemComponent|GenerateParticleEvent (Variables|Default|GetParticleSystem) "StartDay" 0.0 (Transformation|GetWorldLocation (Variables|Default|GetParticleSystem)) "0, 0, 0" "0, 0, 0")
          (goto _label Reset))))))

(fn ConstructionScript)
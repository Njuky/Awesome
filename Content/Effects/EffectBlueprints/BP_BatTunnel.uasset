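; BP_BatTunnel is an effect actor that spawns a one-time bat particle burst when the player character approaches.
; On sphere overlap with BP_Character, it checks BP_Controller's CurrentTime flag, then spawns P_Bat1 at SpawnPoint.
; A First flag, set only when the effect fires, prevents repeats.
; The construction script applies the configurable trigger radius and offsets the ParticleSystem component by ParticleLocation.
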(event OnComponentBeginOverlap(Sphere)
  (params (OverlappedComponent :type Primitive%20Component%20Object%20Reference) (OtherActor :type Actor%20Object%20Reference) (OtherComp :type Primitive%20Component%20Object%20Reference) (OtherBodyIndex :type Integer) (bFromSweep :type Boolean) (SweepResult :type Hit%20Result%20Structure%20%28by%20ref%29))
  (Utilities|Casting|CastToBP_Character OtherActor)
  (bind _asbp_controller (Utilities|Casting|CastToBP_Controller (Game|GetPlayerController 0)))
  (if (Variables|/Script/Project2016.C_PlayerController|GetcurrentTime _asbp_controller)
    (if (not (Variables|Default|GetFirst))
      (Variables|Default|SetFirst true)
      (Effects|SpawnEmitteratLocation "/Game/Effects/ParticleEffects/P_Bat1.P_Bat1" (Transformation|GetWorldLocation (Variables|Default|GetSpawnPoint))))))

(event EventBeginPlay)

(event Collision|EventActorBeginOverlap
  (params (OtherActor :type Actor%20Object%20Reference)))

(event EventTick
  (params (DeltaSeconds :type Float%20%28single-precision%29)))

(fn ConstructionScript
  (Components|Sphere|SetSphereRadius (Variables|Default|GetSphere) (Variables|Default|GetSphereRadius) true)
  (Transformation|AddLocalOffset (Variables|Default|GetParticleSystem) (Variables|Default|GetParticleLocation) false false))